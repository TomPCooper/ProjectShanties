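; Trigger volume that starts a cinematic camera moment introducing the boss when the player ship enters it.
; BeginPlay caches the first BaseBoss actor in the level.
; The first box overlap, gated by a DoOnce, switches an overlapping Pawn_Ship to its cinematic cam, then calls the boss's ShowOff after a short delay.
; The construction script shows the cube only when Debug is set.
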(event OnComponentBeginOverlap(Box)
  (params (OverlappedComponent :type Primitive%20Component%20Object%20Reference) (OtherActor :type Actor%20Object%20Reference) (OtherComp :type Primitive%20Component%20Object%20Reference) (OtherBodyIndex :type Integer) (bFromSweep :type Boolean) (SweepResult :type Hit%20Result%20Structure%20%28by%20ref%29))
  (Utilities|FlowControl|DoOnce false
    (:Completed
      (bind _aspawn_ship (Utilities|Casting|CastToPawn_Ship OtherActor))
      (Default|EnterCinematicCam _aspawn_ship)
      (Utilities|FlowControl|Delay 2.0)
      (Default|ShowOff (Variables|Default|GetBoss)))))

(event EventBeginPlay
  (bind _returnvalue (Actor|GetActorOfClass "/Game/Bosses/BaseBoss.BaseBoss_C"))
  (Variables|Default|SetBoss _returnvalue))

(fn ConstructionScript
  (bind _cube (Variables|Default|GetCube))
  (if (Variables|Default|GetDebug)
    (Rendering|SetVisibility _cube true false)
    (else
      (Rendering|SetVisibility _cube false false))))