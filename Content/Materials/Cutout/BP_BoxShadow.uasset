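; Box shadow actor that publishes its Cube component's oriented box to materials through the MPC_Box_Data parameter collection.
; It writes the cube's world location, world scale and forward, right and up vectors as vector parameters.
; The same writes run in the construction script and once on BeginPlay, with no per-tick update.
; The shared collection and fixed parameter names mean it describes only one box at a time.
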(event EventBeginPlay
  (bind _cube (Variables|Default|GetCube))
  (Rendering|Material|SetVectorParameterValue "/Game/Materials/Cutout/MPC_Box_Data.MPC_Box_Data" "sLocation" (Math|Conversions|ToLinearColor(Vector) (Transformation|GetWorldLocation _cube)) :!class /Script/Engine.KismetMaterialLibrary)
  (Rendering|Material|SetVectorParameterValue "/Game/Materials/Cutout/MPC_Box_Data.MPC_Box_Data" "sBounds" (Math|Conversions|ToLinearColor(Vector) (Transformation|GetWorldScale _cube)) :!class /Script/Engine.KismetMaterialLibrary)
  (Rendering|Material|SetVectorParameterValue "/Game/Materials/Cutout/MPC_Box_Data.MPC_Box_Data" "sX" (Math|Conversions|ToLinearColor(Vector) (Math|Vector|GetForwardVector _cube)) :!class /Script/Engine.KismetMaterialLibrary)
  (Rendering|Material|SetVectorParameterValue "/Game/Materials/Cutout/MPC_Box_Data.MPC_Box_Data" "sY" (Math|Conversions|ToLinearColor(Vector) (Math|Vector|GetRightVector _cube)) :!class /Script/Engine.KismetMaterialLibrary)
  (Rendering|Material|SetVectorParameterValue "/Game/Materials/Cutout/MPC_Box_Data.MPC_Box_Data" "sZ" (Math|Conversions|ToLinearColor(Vector) (Math|Vector|GetUpVector _cube)) :!class /Script/Engine.KismetMaterialLibrary))

(event Collision|EventActorBeginOverlap
  (params (OtherActor :type Actor%20Object%20Reference)))

(fn ConstructionScript
  (bind _cube (Variables|Default|GetCube))
  (Rendering|Material|SetVectorParameterValue "/Game/Materials/Cutout/MPC_Box_Data.MPC_Box_Data" "sLocation" (Math|Conversions|ToLinearColor(Vector) (Transformation|GetWorldLocation _cube)) :!class /Script/Engine.KismetMaterialLibrary)
  (Rendering|Material|SetVectorParameterValue "/Game/Materials/Cutout/MPC_Box_Data.MPC_Box_Data" "sBounds" (Math|Conversions|ToLinearColor(Vector) (Transformation|GetWorldScale _cube)) :!class /Script/Engine.KismetMaterialLibrary)
  (Rendering|Material|SetVectorParameterValue "/Game/Materials/Cutout/MPC_Box_Data.MPC_Box_Data" "sX" (Math|Conversions|ToLinearColor(Vector) (Math|Vector|GetForwardVector _cube)) :!class /Script/Engine.KismetMaterialLibrary)
  (Rendering|Material|SetVectorParameterValue "/Game/Materials/Cutout/MPC_Box_Data.MPC_Box_Data" "sY" (Math|Conversions|ToLinearColor(Vector) (Math|Vector|GetRightVector _cube)) :!class /Script/Engine.KismetMaterialLibrary)
  (Rendering|Material|SetVectorParameterValue "/Game/Materials/Cutout/MPC_Box_Data.MPC_Box_Data" "sZ" (Math|Conversions|ToLinearColor(Vector) (Math|Vector|GetUpVector _cube)) :!class /Script/Engine.KismetMaterialLibrary))