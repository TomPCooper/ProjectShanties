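; BP_FloatVolume is a box volume that marks a body of fluid in which overlapping actors can float.
; On begin and end overlap it messages the actor's first BPI_FloatInterface component with the submerged state and fluid density, which is zero on exit.
; The message also passes the volume's box and the actor's box components, leaving the float response to that component.
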(event Custom|SetInWater
  (params (InWater :type Boolean) (FluidDensity :type Float%20%28double-precision%29) (OverlappingActor :type Actor%20Object%20Reference))
  (bind _returnvalue (Class|Actor|GetComponentsbyInterface OverlappingActor "/Game/Water/WaterFloat/BPI_FloatInterface.BPI_FloatInterface_C"))
  (if (Utilities|Array|IsNotEmpty _returnvalue)
    (Class|BPIFloatInterface|ISetFloating(Message) (Utilities|Array|Get(acopy) _returnvalue) InWater FluidDensity (Variables|Default|GetBox) (Actor|GetComponentsByClass OverlappingActor "/Script/Engine.BoxComponent"))))

(event Collision|EventActorBeginOverlap
  (params (OtherActor :type Actor%20Object%20Reference))
  (CallFunction|SetinWater true (Variables|Default|GetFluidDensity) OtherActor))

(event Collision|EventActorEndOverlap
  (params (OtherActor :type Actor%20Object%20Reference))
  (CallFunction|SetinWater false 0.0 OtherActor))

(fn ConstructionScript)