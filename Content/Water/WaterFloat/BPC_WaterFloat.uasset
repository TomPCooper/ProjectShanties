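; BPC_WaterFloat is an actor component that applies buoyancy to its owner while submerged in a fluid volume.
; The ISetFloating interface event supplies the submerged state, fluid density, float volume and the prop's box colliders.
; Each tick, it scales every box's extent product by its axis-aligned depth below the float volume's top.
; The summed volume, fluid density and gravity become an upward force on the owner's primitive component.
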(event EventBeginPlay)

(event EventTick
  (params (DeltaSeconds :type Float%20%28single-precision%29))
  (if (Variables|Default|GetSubmerged)
    (CallFunction|IApplyBuoyantForce)))

(event EventISetFloating
  (params (SubmergedState :type Boolean) (FluidDensity :type Float%20%28double-precision%29) (FloatVolume :type Box%20Component%20Object%20Reference) (PropVolume :type Array%20of%20Box%20Component%20Object%20References))
  (Variables|Default|SetSubmerged SubmergedState)
  (Variables|Default|SetCurrentFluidDensity FluidDensity)
  (Variables|Default|SetFloatVolume FloatVolume)
  (Variables|Default|SetPropVolumes PropVolume))

(event EventIApplyBuoyantForce
  (bind _floatvolume (Variables|Default|GetFloatVolume))
  (bind _propvolumes (Variables|Default|GetPropVolumes))
  (bind (_origin _boxextent) (Collision|GetComponentBounds _floatvolume))
  ;[1 1 1] Scale collider volumes by how much they are submerged (Axis aligned)
  (Variables|Default|SetNewCalculatedPropVol 0.0)
  (if (Utilities|Array|IsNotEmpty _propvolumes)
    (for _array_element _propvolumes
      (Variables|Default|SetNewCalculatedPropVol (+ (Variables|Default|GetNewCalculatedPropVol) (* (Math|Float|Clamp(Float) (/ (- (.z (+ _origin _boxextent)) (- (.z (Transformation|GetWorldLocation _array_element)) (.z (Components|Box|GetScaledBoxExtent _array_element)))) (* (.z (Components|Box|GetScaledBoxExtent _array_element)) 2.0))) (* (.x (Components|Box|GetScaledBoxExtent _array_element)) (.y (Components|Box|GetScaledBoxExtent _array_element)) (.z (Components|Box|GetScaledBoxExtent _array_element)))))))
    (Physics|AddForce (Actor|GetComponentbyClass (Components|GetOwner) "/Script/Engine.PrimitiveComponent") (/ (* (Variables|Default|GetCurrentFluidDensity) (Variables|Default|GetNewCalculatedPropVol) (Math|Vector|MakeVector 0.0 0.0 9.81)) 1e+02) "None" false)))