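; Boss music controller that plays a MetaSound in time with a Quartz clock and switches it between numbered phases.
; A music data table supplies time signature, BPM, phase index and intro timing.
; Requested phases are clamped and applied on bar boundaries by setting tempo, triggering MetaSound parameters and resetting transport.
; BeginPlay starts phase one and advances twice on hardcoded delays; the intro flag is tracked but never gates changes.
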(event Custom|StartPhase
  (params (phaseToUse :type Integer))
  (bind _audiosource (Variables|Default|GetAudioSource))
  ;[1 1 1] Handles changing between the phases
  (bind _returnvalue (Utilities|GetDataTableRow (Variables|Default|GetmusicDataTable) (Utilities|String|StringToName (Utilities|String|ToString(Integer) phaseToUse)))
    (:then
      (bind _output_get (Variables|Default|SetisPlayingIntro (.includesIntro (Utilities|Struct|BreakSTR_MusicPhaseInfo _returnvalue))))
      (if _output_get
        (bind _returnvalue_2 (Utilities|Time|SetTimerbyEvent (EventDispatchers|CreateEvent :!event Custom|IntroEnd) (.introLength (Utilities|Struct|BreakSTR_MusicPhaseInfo _returnvalue))))
        (Variables|Default|SetintroTimer _returnvalue_2))
      (Class|QuartzClockHandle|SetBeatsPerMinute :self (Variables|Default|GetquartzClockHandle) :BeatsPerMinute (.BPM (Utilities|Struct|BreakSTR_MusicPhaseInfo _returnvalue)))
      (Effects|Components|ParticleSystem|SetIntParameter _audiosource "newPhase" (.phaseIndex (Utilities|Struct|BreakSTR_MusicPhaseInfo _returnvalue)))
      (Class|AudioParameterControllerInterface|SetTriggerParameter _audiosource "Updatephase")
      (Class|QuartzClockHandle|ResetTransportQuantized (Variables|Default|GetquartzClockHandle) (Utilities|Struct|MakeQuartzQuantizationBoundary "Bar" 1.0 "BarRelative"))
      (bind _output_get_2 (Variables|Default|SetcurrentPhase (Variables|Default|GetupcomingPhase)))
      (Development|PrintString (Utilities|String|ToString(Integer) _output_get_2)))
    (:RowNotFound
      (Development|PrintString "ROW NOT FOUND"))))

(event Custom|OnBar
  (params (ClockName :type Name) (QuantizationType :type EQuartzCommandQuantization%20Enum :default "Bar") (NumBars :type Integer) (Beat :type Integer) (BeatFraction :type Float%20%28single-precision%29))
  (if (not (== (Variables|Default|GetcurrentPhase) (Variables|Default|GetupcomingPhase)))
    (CallFunction|StartPhase (Variables|Default|GetupcomingPhase))))

(event Custom|IntroEnd
  (Variables|Default|SetisPlayingIntro false))

(event Custom|SetNewPhase
  (params (newPhase :type Integer))
  (Variables|Default|SetupcomingPhase (Math|Integer|Clamp(Integer) newPhase 1 (Variables|Default|GetmaxPhase))))

(event Custom|IncrementPhase
  (CallFunction|SetNewPhase (+ (Variables|Default|GetcurrentPhase) 1)))

(event EventBeginPlay
  (bind _musicdatatable (Variables|Default|GetmusicDataTable))
  (bind _returnvalue (Utilities|GetDataTableRow _musicdatatable "1")
    (:then
      (bind _outrownames (DataTable|GetDataTableRowNames _musicdatatable))
      (Variables|Default|SetmaxPhase (Utilities|Array|Length _outrownames))
      ;[1 1 1] Initialises the quartz clock
      (Audio|Components|Audio|SetSound (Variables|Default|GetAudioSource) (Variables|Default|GetmetaSound))
      (bind _returnvalue_2 (Class|QuartzSubsystem|CreateNewClock (WorldSubsystems|GetQuartzSubsystem) "BossClock" (Utilities|Struct|MakeQuartzClockSettings (Utilities|Struct|MakeQuartzTimeSignature (.timeSIgTop (Utilities|Struct|BreakSTR_MusicPhaseInfo _returnvalue)) (Utilities|Select :Index (/ (.timeSigBottom (Utilities|Struct|BreakSTR_MusicPhaseInfo _returnvalue)) 4) :Option%200 "HalfNote" :Option%201 "QuarterNote" :Option%202 "EighthNote" :Option%203 "SixteenthNote")) false) false))
      (bind _output_get (Variables|Default|SetquartzClockHandle _returnvalue_2))
      (Class|QuartzClockHandle|SubscribetoQuantizationEvent _output_get "Bar" (EventDispatchers|CreateEvent :!event Custom|OnBar))
      (Audio|Components|Audio|PlayQuantized (Variables|Default|GetAudioSource) (Variables|Default|GetquartzClockHandle) (Utilities|Struct|MakeQuartzQuantizationBoundary "Bar" 1.0 "CurrentTimeRelative") 0)
      (CallFunction|StartPhase 1)
      (Class|QuartzClockHandle|StartClock (Variables|Default|GetquartzClockHandle))
      (Utilities|FlowControl|Delay 12.0)
      (CallFunction|IncrementPhase)
      (Utilities|FlowControl|Delay 2e+01)
      (CallFunction|IncrementPhase))))

(fn ConstructionScript)