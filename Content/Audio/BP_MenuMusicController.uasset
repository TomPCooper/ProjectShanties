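; Menu music controller that plays the MS_Menu sound as a 2D audio component on BeginPlay and adapts it to the open menu screen.
; Opening or closing Credits and Options sets the matching gain parameter on the playing sound to full or zero.
; This layers the music per screen through parameters instead of switching tracks.
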(event Custom|OpenCredits
  (Audio|Parameter|SetFloatParameter (Variables|Default|GetmenuMusic) "CreditsGain" 1.0 :!class /Script/AudioExtensions.AudioParameterControllerInterface))

(event Custom|CloseCredits
  (Audio|Parameter|SetFloatParameter (Variables|Default|GetmenuMusic) "CreditsGain" 0.0 :!class /Script/AudioExtensions.AudioParameterControllerInterface))

(event Custom|OpenOptions
  (Audio|Parameter|SetFloatParameter (Variables|Default|GetmenuMusic) "OptionsGain" 1.0 :!class /Script/AudioExtensions.AudioParameterControllerInterface))

(event Custom|CloseOptions
  (Audio|Parameter|SetFloatParameter (Variables|Default|GetmenuMusic) "OptionsGain" 0.0 :!class /Script/AudioExtensions.AudioParameterControllerInterface))

(event EventBeginPlay
  (bind _returnvalue (Audio|CreateSound2D "/Game/Audio/MS_Menu.MS_Menu" 1.0 1.0 0.0 0))
  (bind _output_get (Variables|Default|SetmenuMusic _returnvalue))
  (Audio|Components|Audio|Play _output_get 0.0))

(fn ConstructionScript)