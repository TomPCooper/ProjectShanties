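; Base boss music Blueprint that plays a MetaSound as phased, layered boss-fight music driven through interface events.
; A data table supplies each phase's tempo, index and optional intro, plus the time signature for a Quartz clock.
; Phase changes and track endings are queued until a bar boundary, with phase changes held during intros.
; Player aiming, harpoon and low-health layers toggle through MetaSound gain parameters.
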(event Custom|StartPhase
  (params (phaseToUse :type Integer))
  (bind _audiosource (Variables|Default|GetAudioSource))
  ;[1 1 1] Handles changing between the phases
  (bind _returnvalue (Utilities|GetDataTableRow (Variables|Default|GetmusicDataTable) (Utilities|String|StringToName (Utilities|String|ToString(Integer) phaseToUse)))
    (:then
      (bind _output_get (Variables|Default|SetisPlayingIntro (.includesIntro (Utilities|Struct|BreakSTR_MusicPhaseInfo _returnvalue))))
      (if _output_get
        (bind _returnvalue_2 (Utilities|Time|SetTimerbyEvent (EventDispatchers|CreateEvent :!event Custom|IntroEnd) (.introLength (Utilities|Struct|BreakSTR_MusicPhaseInfo _returnvalue))))
        (Variables|Default|SetintroTimer _returnvalue_2))
      (Class|QuartzClockHandle|SetBeatsPerMinute :self (Variables|Default|GetquartzClockHandle) :BeatsPerMinute (.BPM (Utilities|Struct|BreakSTR_MusicPhaseInfo _returnvalue)))
      (Effects|Components|ParticleSystem|SetIntParameter _audiosource "newPhase" (.phaseIndex (Utilities|Struct|BreakSTR_MusicPhaseInfo _returnvalue)))
      (Class|AudioParameterControllerInterface|SetTriggerParameter _audiosource "Updatephase")
      (Class|QuartzClockHandle|ResetTransportQuantized (Variables|Default|GetquartzClockHandle) (Utilities|Struct|MakeQuartzQuantizationBoundary "Bar" 1.0 "BarRelative"))
      (Variables|Default|SetcurrentPhase (Variables|Default|GetupcomingPhase)))))

(event Custom|OnBar
  (params (ClockName :type Name) (QuantizationType :type EQuartzCommandQuantization%20Enum :default "Bar") (NumBars :type Integer) (Beat :type Integer) (BeatFraction :type Float%20%28single-precision%29))
  ;[1 1 1] Fires on every bar change
  (if (Variables|Default|GettrackEndQueued) ; Checks if track needs to end first
    (Class|AudioParameterControllerInterface|SetTriggerParameter (Variables|Default|GetAudioSource) "EndTrack")
    (Variables|Default|SettrackEndQueued false)
    (Class|QuartzClockHandle|StopClock (Variables|Default|GetquartzClockHandle) true)
    (elif (not (Variables|Default|GetisPlayingIntro))
      (if (not (== (Variables|Default|GetcurrentPhase) (Variables|Default|GetupcomingPhase)))
        (CallFunction|StartPhase (Variables|Default|GetupcomingPhase))))))

(event Custom|IntroEnd
  ;[1 1 1] Handles ending the intro and resetting the quartz clock
  (Variables|Default|SetisPlayingIntro false)
  (Class|QuartzClockHandle|ResetTransportQuantized (Variables|Default|GetquartzClockHandle) (Utilities|Struct|MakeQuartzQuantizationBoundary "None" 1.0 "CurrentTimeRelative")))

(event Custom|SetNewPhase
  (params (newPhase :type Integer))
  ;[1 1 1] Music phase changing
  (Variables|Default|SetupcomingPhase (Math|Integer|Clamp(Integer) newPhase 1 (Variables|Default|GetmaxPhase))))

(event Custom|IncrementPhase
  ;[1 1 1] Music phase changing
  (CallFunction|SetNewPhase (+ (Variables|Default|GetcurrentPhase) 1)))

(event EventIChangeLayerState
  (params (layerToUpdate :type E_BossMusicLayers%20Enum :default "NewEnumerator0") (newState :type Boolean))
  ;[1 1 1] Music layer updating
  (CallFunction|ChangeLayerState layerToUpdate newState))

(event EventIStartPlaying
  (bind _musicdatatable (Variables|Default|GetmusicDataTable))
  (bind _returnvalue (Utilities|GetDataTableRow _musicdatatable "1")
    (:then
      (bind _outrownames (DataTable|GetDataTableRowNames _musicdatatable))
      (Variables|Default|SetmaxPhase (Utilities|Array|Length _outrownames))
      ;[1 1 1] Initialises the quartz clock
      (Audio|Components|Audio|SetSound (Variables|Default|GetAudioSource) (Variables|Default|GetmetaSound))
      (bind _returnvalue_2 (Class|QuartzSubsystem|CreateNewClock (WorldSubsystems|GetQuartzSubsystem) "BossClock" (Utilities|Struct|MakeQuartzClockSettings (Utilities|Struct|MakeQuartzTimeSignature (.timeSIgTop (Utilities|Struct|BreakSTR_MusicPhaseInfo _returnvalue)) (Utilities|Select :Index (/ (.timeSigBottom (Utilities|Struct|BreakSTR_MusicPhaseInfo _returnvalue)) 4) :Option%200 "HalfNote" :Option%201 "QuarterNote" :Option%202 "EighthNote" :Option%203 "SixteenthNote")) false) false))
      (bind _output_get (Variables|Default|SetquartzClockHandle _returnvalue_2))
      (Class|QuartzClockHandle|SubscribetoQuantizationEvent _output_get "Bar" (EventDispatchers|CreateEvent :!event Custom|OnBar))
      (Audio|Components|Audio|PlayQuantized (Variables|Default|GetAudioSource) (Variables|Default|GetquartzClockHandle) (Utilities|Struct|MakeQuartzQuantizationBoundary "Tick" 1.0 "CurrentTimeRelative") 0)
      (CallFunction|StartPhase 1)
      (Class|QuartzClockHandle|StartClock (Variables|Default|GetquartzClockHandle)))))

(event EventIChangePhase
  (params (newPhase :type Integer))
  ;[1 1 1] Music phase changing
  (CallFunction|SetNewPhase newPhase))

(event EventBeginPlay)

(event EventIIncrementPhase
  ;[1 1 1] Music phase changing
  (CallFunction|IncrementPhase))

(event EventIEndTrack
  ;[1 1 1] Music phase changing
  (Variables|Default|SettrackEndQueued true))

(fn ConstructionScript)

(fn ChangeLayerState
  (params (layerToChange :type E_BossMusicLayers%20Enum :default "NewEnumerator0") (newState :type Boolean))
  (Utilities|FlowControl|Sequence
    (:then_0
      ;[1 1 1] Sets the gain that needs to be used on an individual channel
      (if newState
        (LocalVariables|SetgainToSet 1.0)
        (else
          (LocalVariables|SetgainToSet 0.0))))
    (:then_1
      ;[1 1 1] Sets the correct parameter for the layer
      (switch Utilities|FlowControl|Switch|SwitchonE_BossMusicLayers layerToChange
        (:NewEnumerator0
          (Audio|Parameter|SetFloatParameter (Variables|Default|GetAudioSource) "AimingLayerGain" (LocalVariables|GetgainToSet) :!class /Script/Engine.AudioComponent))
        (:NewEnumerator1
          (Audio|Parameter|SetFloatParameter (Variables|Default|GetAudioSource) "HarpoonLayerGain" (LocalVariables|GetgainToSet) :!class /Script/Engine.AudioComponent))
        (:NewEnumerator2
          (Audio|Parameter|SetFloatParameter (Variables|Default|GetAudioSource) "PlayerLowHealthGain" (LocalVariables|GetgainToSet) :!class /Script/Engine.AudioComponent))))))