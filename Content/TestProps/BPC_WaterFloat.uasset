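; Actor component that makes its owning actor float by applying buoyant force while submerged.
; ISetFloating stores the submerged state, fluid density and volume supplied by callers.
; Each Tick prints that state and, when submerged, pushes the owner's primitive component upward via AddForce.
; The force is density times volume times gravity, divided by 100 as a unit conversion, with no acceleration change.
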(event EventBeginPlay)

(event EventTick
  (params (DeltaSeconds :type Float%20%28single-precision%29))
  (if (Variables|Default|GetSubmerged)
    (Development|PrintString "Submerged")
    (CallFunction|IApplyBuoyantForce)
    (else
      (Development|PrintString "Not Submerged"))))

(event EventISetFloating
  (params (SubmergedState :type Boolean) (FluidDensity :type Float%20%28double-precision%29) (Volume :type Float%20%28double-precision%29))
  (Variables|Default|SetSubmerged SubmergedState)
  (Variables|Default|SetCurrentFluidDensity FluidDensity)
  (Variables|Default|SetCurrentVolume Volume))

(event EventIApplyBuoyantForce
  (Physics|AddForce (Actor|GetComponentbyClass (Components|GetOwner) "/Script/Engine.PrimitiveComponent") (/ (* (Variables|Default|GetCurrentFluidDensity) (Variables|Default|GetCurrentVolume) (Math|Vector|MakeVector 0.0 0.0 9.81)) "100.000000,100.000000,100.000000") "None" false))