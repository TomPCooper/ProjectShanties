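; BP_FloatVolume is a fluid volume actor in TestProps that notifies overlapping actors when they enter or leave it.
; Begin overlap passes a submerged state with its FluidDensity and Volume variables, and end overlap passes false with zeros.
; SetInWater forwards these values to the actor's first component implementing BPI_FloatInterface, leaving any floating response to that component.
; Unconnected draft nodes for calculating collider volumes never run.
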(event Custom|SetInWater
  (params (InWater :type Boolean) (FluidDensity :type Float%20%28double-precision%29) (Volume :type Float%20%28double-precision%29))
  (bind _overlappingactor (Variables|Default|GetOverlappingActor))
  (bind _returnvalue (Class|Actor|GetComponentsbyInterface _overlappingactor "/Game/TestProps/BPI_FloatInterface.BPI_FloatInterface_C"))
  (if (Utilities|Array|IsNotEmpty _returnvalue)
    (Class|BPIFloatInterface|ISetFloating(Message) (Utilities|Array|Get(acopy) _returnvalue) InWater FluidDensity Volume)))

(event Collision|EventActorBeginOverlap
  (params (OtherActor :type Actor%20Object%20Reference))
  (Variables|Default|SetOverlappingActor OtherActor)
  (CallFunction|SetinWater true (Variables|Default|GetFluidDensity) (Variables|Default|GetVolume)))

(event Collision|EventActorEndOverlap
  (params (OtherActor :type Actor%20Object%20Reference))
  (Variables|Default|SetOverlappingActor OtherActor)
  (CallFunction|SetinWater false 0.0 0.0))

(fn ConstructionScript)