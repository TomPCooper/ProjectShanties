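; BP_SplinePlacer is a level-building tool that lays a mesh and rail pillars along a spline, such as for railings.
; When Build is set, the construction script splits the spline by LengthOfSegment and bends a spline mesh over each segment, with tangents scaled by TangentSmooth.
; RailPillar meshes, also spline mesh components, follow spline position and rotation at every segment boundary if Constant, otherwise only at the first and last segment index.
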(fn ConstructionScript
  (bind _lengthofsegment (Variables|Default|GetLengthOfSegment))
  (bind _spline (Variables|Default|GetSpline))
  (bind _spline_2 (Variables|Default|GetSpline))
  (bind _lengthofsegment_2 (Variables|Default|GetLengthOfSegment))
  (bind _spline_3 (Variables|Default|GetSpline))
  (bind _spline_4 (Variables|Default|GetSpline))
  (bind _returnvalue (Spline|GetSplineLength _spline_2))
  (bind _returnvalue_2 (Math|Float|Division(WholeandRemainder) _returnvalue _lengthofsegment_2))
  (if (Variables|Default|GetBuild?)
    (for _index (range 0 (.ReturnValue (Math|Float|Division(WholeandRemainder) (Spline|GetSplineLength (Variables|Default|GetSpline)) (Variables|Default|GetLengthOfSegment))))
      (bind _returnvalue_3 (AddComponent|AddSplineMeshComponent false))
      (Components|StaticMesh|SetStaticMesh _returnvalue_3 (Variables|Default|GetMesh))
      (SplineMesh|SetStartandEnd _returnvalue_3 (Spline|GetLocationatDistanceAlongSpline _spline (* _index _lengthofsegment) "Local") (* (Spline|GetDirectionatDistanceAlongSpline _spline (* _index _lengthofsegment) "Local") (Variables|Default|GetTangentSmooth)) (Spline|GetLocationatDistanceAlongSpline _spline (+ (* _index _lengthofsegment) _lengthofsegment) "Local") (* (Variables|Default|GetTangentSmooth) (Spline|GetDirectionatDistanceAlongSpline _spline (+ (* _index _lengthofsegment) _lengthofsegment) "Local")) true :!class /Script/Engine.SplineMeshComponent))
    (if (Variables|Default|GetConstant?)
      (for _index_2 (range 0 (.ReturnValue (Math|Float|Division(WholeandRemainder) (Spline|GetSplineLength (Variables|Default|GetSpline)) (Variables|Default|GetLengthOfSegment))))
        (bind _returnvalue_4 (AddComponent|AddSplineMeshComponent false (Math|Transform|MakeTransform (Spline|GetLocationatDistanceAlongSpline _spline_4 (* _index_2 (Variables|Default|GetLengthOfSegment)) "Local") (Spline|GetRotationatDistanceAlongSpline _spline_4 (* _index_2 (Variables|Default|GetLengthOfSegment)) "Local"))))
        (Components|StaticMesh|SetStaticMesh _returnvalue_4 (Variables|Default|GetRailPillar)))
      (else
        (for _index_3 (range 0 _returnvalue_2)
          (if (== _index_3 0)
            (bind _returnvalue_5 (AddComponent|AddSplineMeshComponent false (Math|Transform|MakeTransform (Spline|GetLocationatDistanceAlongSpline _spline_3 (* _index_3 (Variables|Default|GetLengthOfSegment)) "Local") (Spline|GetRotationatDistanceAlongSpline _spline_3 (* _index_3 (Variables|Default|GetLengthOfSegment)) "Local"))))
            (Components|StaticMesh|SetStaticMesh _returnvalue_5 (Variables|Default|GetRailPillar))
            (elif (== _index_3 _returnvalue_2)
              (bind _returnvalue_6 (AddComponent|AddSplineMeshComponent false (Math|Transform|MakeTransform (Spline|GetLocationatDistanceAlongSpline _spline_3 (* _index_3 (Variables|Default|GetLengthOfSegment)) "Local") (Spline|GetRotationatDistanceAlongSpline _spline_3 (* _index_3 (Variables|Default|GetLengthOfSegment)) "Local"))))
              (Components|StaticMesh|SetStaticMesh _returnvalue_6 (Variables|Default|GetRailPillar)))))))))