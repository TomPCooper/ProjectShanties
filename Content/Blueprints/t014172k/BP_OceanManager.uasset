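; BP_OceanManager controls the ocean's wave look through displacement and normal tiling and strength.
; Setter events write each value to both the MPC_WaterParameters material collection and the NPC_WaterParameters Niagara collection.
; LerpToValues reads current MPC values and blends toward targets on a timeline scaled by LerpLength, skipping zero targets.
; The NormalStrength blend calls the NormalTiling setter, so that lerp never changes normal strength.
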(event Custom|DisplacementTiling
  (params (newDisplacementTiling :type Float%20%28double-precision%29))
  ;[1 1 1] Functrions that change the parameters of the material
  (Rendering|Material|SetScalarParameterValue "/Game/Blueprints/t014172k/MPC_WaterParameters.MPC_WaterParameters" (Utilities|Name|MakeLiteralName "DisplacementTiling") newDisplacementTiling :!class /Script/Engine.KismetMaterialLibrary)
  (bind _returnvalue (Class|NiagaraFunctionLibrary|GetNiagaraParameterCollection "/Game/Blueprints/t014172k/NPC_WaterParameters.NPC_WaterParameters"))
  (Effects|Components|ParticleSystem|SetFloatParameter _returnvalue "DisplacementTiling" newDisplacementTiling))

(event Custom|VertexDisplacementStrength
  (params (NewVertexDisplacementStrength :type Float%20%28double-precision%29))
  ;[1 1 1] Functrions that change the parameters of the material
  (Rendering|Material|SetScalarParameterValue "/Game/Blueprints/t014172k/MPC_WaterParameters.MPC_WaterParameters" (Utilities|Name|MakeLiteralName "VertexDisplacementStrength") NewVertexDisplacementStrength :!class /Script/Engine.KismetMaterialLibrary)
  (bind _returnvalue (Class|NiagaraFunctionLibrary|GetNiagaraParameterCollection "/Game/Blueprints/t014172k/NPC_WaterParameters.NPC_WaterParameters"))
  (Effects|Components|ParticleSystem|SetFloatParameter _returnvalue "VertexDisplacementStrength" NewVertexDisplacementStrength))

(event Custom|NormalTiling
  (params (NewNormalTiling :type Float%20%28double-precision%29))
  ;[1 1 1] Functrions that change the parameters of the material
  (Rendering|Material|SetScalarParameterValue "/Game/Blueprints/t014172k/MPC_WaterParameters.MPC_WaterParameters" (Utilities|Name|MakeLiteralName "NormalTiling") NewNormalTiling :!class /Script/Engine.KismetMaterialLibrary)
  (bind _returnvalue (Class|NiagaraFunctionLibrary|GetNiagaraParameterCollection "/Game/Blueprints/t014172k/NPC_WaterParameters.NPC_WaterParameters"))
  (Effects|Components|ParticleSystem|SetFloatParameter _returnvalue "NormalTiling" NewNormalTiling))

(event Custom|NormalStrength
  (params (NewNormalStrength :type Float%20%28double-precision%29))
  ;[1 1 1] Functrions that change the parameters of the material
  (Rendering|Material|SetScalarParameterValue "/Game/Blueprints/t014172k/MPC_WaterParameters.MPC_WaterParameters" (Utilities|Name|MakeLiteralName "NormalStrength") NewNormalStrength :!class /Script/Engine.KismetMaterialLibrary)
  (bind _returnvalue (Class|NiagaraFunctionLibrary|GetNiagaraParameterCollection "/Game/Blueprints/t014172k/NPC_WaterParameters.NPC_WaterParameters"))
  (Effects|Components|ParticleSystem|SetFloatParameter _returnvalue "NormalStrength" NewNormalStrength))

(event Custom|LerpToValues
  (params (lerpLength :type Float%20%28double-precision%29) (DisplacementTiling :type Float%20%28double-precision%29) (VertexDisplacement :type Float%20%28double-precision%29) (NormalTiling :type Float%20%28double-precision%29) (NormalStrength :type Float%20%28double-precision%29))
  ;[1 1 1] Timeline to control the wave change variables via lerping
  (Components|Timeline|SetPlayRate (Variables|Default|GetLerpTimeline) (/ 1.0 lerpLength))
  (CallFunction|CheckLerpValues DisplacementTiling VertexDisplacement NormalTiling NormalStrength)
  (Utilities|FlowControl|Sequence
    (:then_0
      ;;[1 1 1] Assigns the initial variables used in the lerp
      (bind _displacementtiling (CallFunction|GetDisplacementTiling))
      (Variables|EventLocalVar|SetoldDisplacementTiling _displacementtiling)
      (bind _vertexdisplacementstrength (CallFunction|GetVertexDisplacementStrength))
      (Variables|EventLocalVar|SetoldVertexDisplacementStrength _vertexdisplacementstrength)
      (bind _normaltiling (CallFunction|GetNormalTiling))
      (Variables|EventLocalVar|SetoldNormalTiling _normaltiling)
      (bind _normalstrength (CallFunction|GetNormalStrength))
      (Variables|EventLocalVar|SetoldNormalStrength _normalstrength))
    (:then_1
      ;;[1 1 1] Changes the wave values over time
      (bind _alpha (Timeline|LerpTimeline PlayFromStart)
        (:Update
          (if (Variables|EventLocalVar|GetupdateDisplacementTiling)
            (CallFunction|DisplacementTiling (Math|Float|Lerp (Variables|EventLocalVar|GetoldDisplacementTiling) DisplacementTiling _alpha)))
          (if (Variables|EventLocalVar|GetupdateVDS)
            (CallFunction|VertexDisplacementStrength (Math|Float|Lerp (Variables|EventLocalVar|GetoldVertexDisplacementStrength) VertexDisplacement _alpha)))
          (if (Variables|EventLocalVar|GetupdateNormalTiling)
            (CallFunction|NormalTiling (Math|Float|Lerp (Variables|EventLocalVar|GetoldNormalTiling) NormalTiling _alpha)))
          (if (Variables|EventLocalVar|GetupdateNormalStrength)
            (CallFunction|NormalTiling (Math|Float|Lerp (Variables|EventLocalVar|GetoldNormalStrength) NormalStrength _alpha))))))))

(fn ConstructionScript)

(fn GetNormalTiling
  (bind _returnvalue (Rendering|Material|GetScalarParameterValue "/Game/Blueprints/t014172k/MPC_WaterParameters.MPC_WaterParameters" "NormalTiling" :!class /Script/Engine.KismetMaterialLibrary))
  (return _returnvalue))

(fn GetNormalStrength
  (bind _returnvalue (Rendering|Material|GetScalarParameterValue "/Game/Blueprints/t014172k/MPC_WaterParameters.MPC_WaterParameters" "NormalStrength" :!class /Script/Engine.KismetMaterialLibrary))
  (return _returnvalue))

(fn GetVertexDisplacementStrength
  (bind _returnvalue (Rendering|Material|GetScalarParameterValue "/Game/Blueprints/t014172k/MPC_WaterParameters.MPC_WaterParameters" "VertexDisplacementStrength" :!class /Script/Engine.KismetMaterialLibrary))
  (return _returnvalue))

(fn GetDisplacementTiling
  (bind _returnvalue (Rendering|Material|GetScalarParameterValue "/Game/Blueprints/t014172k/MPC_WaterParameters.MPC_WaterParameters" "DisplacementTiling" :!class /Script/Engine.KismetMaterialLibrary))
  (return _returnvalue))

(fn CheckLerpValues
  (params (displacementTiling :type Float%20%28double-precision%29) (VDS :type Float%20%28double-precision%29) (normalTiling :type Float%20%28double-precision%29) (normalStrength :type Float%20%28double-precision%29))
  ;[1 1 1] Checks whether each of the values need to be updated for the lerp
  (Variables|EventLocalVar|SetupdateDisplacementTiling (!= displacementTiling 0.0))
  (Variables|EventLocalVar|SetupdateVDS (!= VDS 0.0))
  (Variables|EventLocalVar|SetupdateNormalTiling (!= normalTiling 0.0))
  (Variables|EventLocalVar|SetupdateNormalStrength (!= normalStrength 0.0)))