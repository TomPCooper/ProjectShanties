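; Player ship pawn with physics-based buoyancy, impulse-driven steering and an orbit/zoom spring-arm camera.
; A Niagara system receives the pontoon positions and exports GPU wave heights back through ParticleData.
; While buoyancy simulates, Tick turns each pontoon's depth into spherical-cap submerged volume, applied as local force on the Boat.
; Interface events drive movement, camera and external forces; starting movement eases the camera back to default, and attack input only prints radial-menu placeholders.
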(event Custom|AddForceAtPoint
  (params (force :type Vector) (location :type Vector))
  ;[1 1 1] Functions for adding extra forces to ship
  (Class|PrimitiveComponent|AddForceatLocation (Variables|Default|GetBoat) force location "None"))

(event Custom|ResetCameraRotation
  ;[1 1 1] Resets camera position
  (Variables|LocalEvent|SetpreResetCameraRot (Variables|/Script/Engine.SceneComponent|GetRelativeRotation (Variables|Default|GetSpringArm)))
  (bind _alpha (Timeline|CameraReset PlayFromStart)
    (:Update
      (Transformation|SetRelativeRotation (Variables|Default|GetSpringArm) (Math|Rotator|Lerp(Rotator) (Variables|LocalEvent|GetpreResetCameraRot) (Variables|Camera|GetdefaultRotation) _alpha true) false false))))

(event Custom|AddTurn
  (params (turnInput :type Float%20%28double-precision%29))
  ;[1 1 1] Adds turning force
  (Class|PrimitiveComponent|AddAngularImpulseinDegrees (Variables|Default|GetBoat) (* turnInput (Variables|Movement|GetturnForce) (Math|Vector|GetUpVector (Variables|Default|GetBoat))) "None" true))

(event Custom|AddForward
  (params (forwardInput :type Float%20%28double-precision%29))
  ;[1 1 1] Adds forward force
  (Physics|AddImpulse (Variables|Default|GetBoat) (* forwardInput (Transformation|GetActorForwardVector) (Variables|Movement|GetmoveForce)) "None" true))

(event EventILookInput
  (params (AxisX :type Float%20%28double-precision%29) (AxisY :type Float%20%28double-precision%29))
  (bind _springarm (Variables|Default|GetSpringArm))
  (bind _relativerotation (Variables|/Script/Engine.SceneComponent|GetRelativeRotation _springarm))
  ;[1 1 1] Camera look input
  (Transformation|SetRelativeRotation (Variables|Default|GetSpringArm) (Math|Rotator|MakeRotator (.roll _relativerotation) (+ (* AxisY (Variables|Default|GetcameraSensitivity) -1.0) (.pitch _relativerotation)) (+ (* AxisX (Variables|Default|GetcameraSensitivity)) (.yaw _relativerotation))) false false))

(event EventICameraMovementToggle
  (params (CanMove :type Boolean))
  ;[1 1 1] Toggles whether the camera can move
  (Variables|Camera|SetisCameraMovable CanMove))

(event EventBeginPlay
  (bind _fx_systreadback (Variables|Default|GetFX_SystReadback))
  ;[1 1 1] Ship initialisation
  (Transformation|SetRelativeRotation (Variables|Default|GetSpringArm) (Variables|Camera|GetdefaultRotation) false false)
  ;[1 1 1] Niagara buoyancy system setup
  (Class|NiagaraComponent|SetVariableObject _fx_systreadback "Actor" self)
  (Class|NiagaraComponent|SetVariableBool _fx_systreadback "bExport" true)
  (Class|NiagaraDataInterfaceArrayFunctionLibrary|SetNiagaraArrayVector _fx_systreadback "Pontoons" (Variables|Default|Getpontoons))
  (Niagara|ReinitializeSystem _fx_systreadback))

(event EventIInit
  (bind _fx_systreadback (Variables|Default|GetFX_SystReadback))
  ;[1 1 1] Ship initialisation
  (Transformation|SetRelativeRotation (Variables|Default|GetSpringArm) (Variables|Camera|GetdefaultRotation) false false)
  ;[1 1 1] Niagara buoyancy system setup
  (Class|NiagaraComponent|SetVariableObject _fx_systreadback "Actor" self)
  (Class|NiagaraComponent|SetVariableBool _fx_systreadback "bExport" true)
  (Class|NiagaraDataInterfaceArrayFunctionLibrary|SetNiagaraArrayVector _fx_systreadback "Pontoons" (Variables|Default|Getpontoons))
  (Niagara|ReinitializeSystem _fx_systreadback))

(event EventTick
  (params (DeltaSeconds :type Float%20%28single-precision%29))
  (bind _pontoons (Variables|Default|Getpontoons))
  (bind _boat (Variables|Default|GetBoat))
  ;[1 1 1] Calculate the submerged depth
  (if (Variables|Buoyancy|GetsimulateBuoyancy)
    (for (_array_element _array_index) (Variables|Default|GetData)
      (if (Utilities|Array|IsValidIndex _pontoons _array_index) ; If pontoon index is a valid position
        ;[1 1 1] Calculates submerged volume for each pontoon
        (if (> (* (Math|Float|MultiplybyPi 0.333333) (Math|Float|Square (Math|Float|Clamp(Float) (Utilities|Operators|Subtract (.Size (Utilities|Struct|BreakBasicParticleData _array_element)) (* (.Z (Class|KismetMathLibrary|BreakVector3f (Transformation|GetWorldLocation (Variables|Default|GetwaterPlane)))) -1.0) (.Z (Class|KismetMathLibrary|BreakVector3f (Math|Transform|TransformLocation (Transformation|GetWorldTransform _boat) (/ (Utilities|Array|Get(acopy) _pontoons _array_index) (Transformation|GetWorldScale _boat)))))) 0.0 6e+01)) (- (* 3e+01 3.0) (Math|Float|Clamp(Float) (Utilities|Operators|Subtract (.Size (Utilities|Struct|BreakBasicParticleData _array_element)) (* (.Z (Class|KismetMathLibrary|BreakVector3f (Transformation|GetWorldLocation (Variables|Default|GetwaterPlane)))) -1.0) (.Z (Class|KismetMathLibrary|BreakVector3f (Math|Transform|TransformLocation (Transformation|GetWorldTransform _boat) (/ (Utilities|Array|Get(acopy) _pontoons _array_index) (Transformation|GetWorldScale _boat)))))) 0.0 6e+01))) 0.0)
          (Class|PrimitiveComponent|AddForceatLocationLocal (Variables|Default|GetBoat) (* (* (Math|Float|MultiplybyPi 0.333333) (Math|Float|Square (Math|Float|Clamp(Float) (Utilities|Operators|Subtract (.Size (Utilities|Struct|BreakBasicParticleData _array_element)) (* (.Z (Class|KismetMathLibrary|BreakVector3f (Transformation|GetWorldLocation (Variables|Default|GetwaterPlane)))) -1.0) (.Z (Class|KismetMathLibrary|BreakVector3f (Math|Transform|TransformLocation (Transformation|GetWorldTransform _boat) (/ (Utilities|Array|Get(acopy) _pontoons _array_index) (Transformation|GetWorldScale _boat)))))) 0.0 6e+01)) (- (* 3e+01 3.0) (Math|Float|Clamp(Float) (Utilities|Operators|Subtract (.Size (Utilities|Struct|BreakBasicParticleData _array_element)) (* (.Z (Class|KismetMathLibrary|BreakVector3f (Transformation|GetWorldLocation (Variables|Default|GetwaterPlane)))) -1.0) (.Z (Class|KismetMathLibrary|BreakVector3f (Math|Transform|TransformLocation (Transformation|GetWorldTransform _boat) (/ (Utilities|Array|Get(acopy) _pontoons _array_index) (Transformation|GetWorldScale _boat)))))) 0.0 6e+01))) (Math|Vector|VectorUp)) (Utilities|Array|Get(acopy) _pontoons _array_index) "None"))))))

(event EventIAttackReleased
  ;[1 1 1] Used to control radial menu
  (Development|PrintString "Close radial menu"))

(event EventIAttackPressed
  ;[1 1 1] Used to control radial menu
  (Development|PrintString "Open radial menu"))

(event EventIMoveInputStarted
  ;[1 1 1] Resets camera when the boat starts to move again
  (if (Variables|Camera|GetisCameraMovable)
    (CallFunction|ResetCameraRotation)))

(event EventIMoveInputTriggered
  (params (AxisX :type Float%20%28double-precision%29) (AxisY :type Float%20%28double-precision%29))
  ;[1 1 1] Checks player input to see whether forces need to be added to ship
  (Utilities|FlowControl|Sequence ; Handles x and y components separately
    (:then_0
      (if (> (Math|Float|Absolute(Float) AxisX) 0.0)
        (CallFunction|AddTurn AxisX)))
    (:then_1
      (if (> (Math|Float|Absolute(Float) AxisY) 0.0)
        (CallFunction|AddForward AxisY)))))

(event EventIZoomInput
  (params (InputAxis :type Float%20%28double-precision%29))
  ;[1 1 1] Camera zoom input
  (Variables|/Script/Engine.SpringArmComponent|SetTargetArmLength (Variables|Default|GetSpringArm) (Math|Float|Clamp(Float) (- (Variables|/Script/Engine.SpringArmComponent|GetTargetArmLength (Variables|Default|GetSpringArm)) (* InputAxis (Variables|Camera|GetcameraZoomSpeed))) (Variables|Camera|GetminCameraDistance) (Variables|Camera|GetmaxCameraDistance))))

(event EventIAddForcetoShip
  (params (forceToAdd :type Vector :default "0, 0, 0"))
  ;[1 1 1] Functions for adding extra forces to ship
  (Physics|AddForce (Variables|Default|GetBoat) forceToAdd "None" true))

(event EventIGetMovingWaterPlane
  (params (mesh :type Static%20Mesh%20Component%20Object%20Reference))
  ;[1 1 1] Updates positioning to be used in ship rotations
  (Variables|Default|SetwaterPlane mesh))

(event EventParticleData
  (params (Data :type Array%20of%20Basic%20Particle%20Data%20Structures) (NiagaraSystem :type Niagara%20System%20Object%20Reference) (SimulationPositionOffset :type Vector%20%28by%20ref%29 :default "0, 0, 0"))
  ;[1 1 1] Stores wave height data sent over from GPU
  (Variables|Default|SetData Data))

(fn ConstructionScript)