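; Ship pawn with unfinished groundwork for rotating the boat relative to a moving water plane.
; An interface event stores the water plane mesh and caches the static mesh's Y bounds extent as the boat width.
; GetRotation only reads the plane's world location; two unconnected vector calculations offset the ship by that width to build sample points, and no rotation is computed or applied.
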(event EventIGetMovingWaterPlane
  (params (mesh :type Static%20Mesh%20Component%20Object%20Reference))
  ;[1 1 1] Updates positioning to be used in ship rotations
  (Variables|Default|SetwaterPlane mesh)
  (Variables|Default|SetboatWidth (.Y (Class|KismetMathLibrary|BreakVector3f (.BoxExtent (Collision|GetComponentBounds (Variables|Default|GetStaticMesh)))))))

(fn ConstructionScript)

(fn GetRotation
  (LocalVariables|Setwater_World_Position (Transformation|GetWorldLocation (Variables|Default|GetwaterPlane))))