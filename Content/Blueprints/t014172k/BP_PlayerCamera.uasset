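; Spring-arm player camera that follows the ship and switches between free-roam and combat views on game state changes.
; Free roam allows clamped orbit and zoom, then eases back behind the moving ship after a retriggerable delay.
; Combat locks input, aims toward the midpoint between ship and a BP_TargetTest actor, and lengthens the arm with their separation.
; Timelines blend state transitions and rotation resets; Docked only records the state.
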(event Custom|isCamMovable
  ;[1 1 1] Delay between cam movement input and resetting rotation
  (CallFunction|StopReset)
  (Variables|Default|SetisCameraMovable false)
  (Utilities|FlowControl|RetriggerableDelay 3.0)
  (Variables|Default|SetisCameraMovable true)
  (if (Variables|Default|GetisCamFree)
    (if (Variables|Default|GetisMoving)
      (CallFunction|ResetCameraRotation))))

(event Custom|StopReset
  ;[1 1 1] Reset camera position
  (bind _alpha (Timeline|CameraReset Stop)
    (:Update
      (Transformation|SetActorRotation (Math|Rotator|MakeRotator 0.0 (.pitch (Math|Rotator|Lerp(Rotator) (Variables|Default|GetpreResetCameraRot) (Variables|Default|GetdefaultRotation) _alpha true)) (.yaw (Math|Rotator|Lerp(Rotator) (Variables|Default|GetpreResetCameraRot) (Variables|Default|GetdefaultRotation) _alpha true)))))
    (:Finished
      (Variables|Default|SetisFollowing true))))

(event Custom|TransitionGameState
  (Variables|Default|SetisTransitioning true)
  (Variables|Default|SetisCamFree false)
  (Variables|Default|SetpreTransitionPos (Transformation|GetActorLocation))
  (Variables|Default|SetpreTransitionRot (Transformation|GetActorRotation))
  (bind _transition (Timeline|Transition PlayFromStart)
    (:Update
      (switch Utilities|FlowControl|Switch|SwitchonE_GameState (Variables|Default|GetCurrentGameState)
        (:NewEnumerator0
          (Transformation|SetActorLocation (Math|Vector|Lerp(Vector) (Variables|Default|GetpreTransitionPos) (+ (Transformation|GetActorLocation (Variables|Default|Getship)) (Variables|Default|GetcameraPositionOffset)) _transition) false false)
          (Utilities|FlowControl|DoOnce false
            (:Completed
              (CallFunction|ResetCameraCompRotation))))
        (:NewEnumerator1
          (Variables|/Script/Engine.SpringArmComponent|SetTargetArmLength (Variables|Default|GetSpringArm) (Math|Float|Lerp (Variables|/Script/Engine.SpringArmComponent|GetTargetArmLength (Variables|Default|GetSpringArm)) (Variables|Default|GetCombatCameraMinimunArmLength) _transition)))))
    (:Finished
      (Variables|Default|SetisTransitioning false)
      (switch Utilities|FlowControl|Switch|SwitchonE_GameState (Variables|Default|GetCurrentGameState)))))

(event Custom|FreeRoamCamReset
  (Utilities|FlowControl|DoOnce false) ; enters at Reset
)

(event Custom|ResetCameraCompRotation
  ;[1 1 1] Transitions the camera to freeplay
  (Variables|Default|SetpreResetCameraCompRot (Variables|/Script/Engine.SceneComponent|GetRelativeRotation (Variables|Default|GetCamera)))
  (Variables|Default|SetpreResetCameraRot (Transformation|GetActorRotation))
  (CallFunction|ResetCameraRotation)
  (Variables|Default|SetisCamFree false)
  (bind _transition (Timeline|Timeline PlayFromStart)
    (:Update
      (Transformation|SetRelativeRotation (Variables|Default|GetCamera) (Math|Rotator|MakeRotator 0.0 (.pitch (Math|Rotator|Lerp(Rotator) (Variables|Default|GetpreResetCameraCompRot) "0, 0, 0" _transition)) (.yaw (Math|Rotator|Lerp(Rotator) (Variables|Default|GetpreResetCameraCompRot) "0, 0, 0" _transition))) false false))
    (:Finished
      (Variables|Default|SetisCamFree true))))

(event Custom|Init
  ;[1 1 1] Camera initialisation
  (Variables|Default|Setship (Game|Player|GetPlayerPawn 0))
  (Transformation|SetActorLocation (+ (Transformation|GetActorLocation (Variables|Default|Getship)) (Variables|Default|GetcameraPositionOffset)) false false)
  (bind _output_get (Variables|Default|SetdefaultRotation (Math|Rotator|CombineRotators (Transformation|GetActorRotation (Variables|Default|Getship)) "-15.000000,0.000000,0.000000")))
  (Transformation|SetActorRotation _output_get)
  (Game|Player|SetViewTargetwithBlend (Game|GetPlayerController 0) self 0.0 "VTBlend_Linear" 0.0 false)
  (bind _aspirate_game_state (Utilities|Casting|CastToPirate_GameState (Game|GetGameState)))
  (EventDispatchers|BindEventtoGameStateChanged _aspirate_game_state (EventDispatchers|CreateEvent :!event Custom|SwitchCam))
  (bind _returnvalue (Actor|GetActorOfClass "/Game/Blueprints/t014172k/BP_TargetTest.BP_TargetTest_C"))
  (Variables|Default|SetTarget _returnvalue))

(event Custom|LookInput
  (params (axisX :type Float%20%28double-precision%29) (axisY :type Float%20%28double-precision%29))
  (bind _returnvalue (Transformation|GetActorRotation))
  ;[1 1 1] Camera look input
  (if (Variables|Default|GetisCamFree)
    (Variables|Default|SetisFollowing false)
    (Transformation|SetActorRotation (Math|Rotator|MakeRotator (.roll _returnvalue) (Math|Float|Clamp(Float) (+ (* axisY (Variables|Default|GetcameraSensitivity) -1.0) (.pitch _returnvalue)) -85.0 -5.0) (+ (* axisX (Variables|Default|GetcameraSensitivity)) (.yaw _returnvalue))))
    (CallFunction|IsCamMovable)))

(event Custom|MoveInputStarted
  (Variables|Default|SetisMoving true)
  (if (and (Variables|Default|GetisCameraMovable) (Variables|Default|GetisCamFree))
    (CallFunction|ResetCameraRotation)))

(event Custom|ZoomInput
  (params (inputAxis :type Float%20%28double-precision%29))
  ;[1 1 1] Camera zoom input
  (if (Variables|Default|GetisCamFree)
    (Variables|/Script/Engine.SpringArmComponent|SetTargetArmLength (Variables|Default|GetSpringArm) (Math|Float|Clamp(Float) (- (Variables|/Script/Engine.SpringArmComponent|GetTargetArmLength (Variables|Default|GetSpringArm)) (* inputAxis (Variables|Default|GetcameraZoomSpeed))) (Variables|Default|GetminCameraDistance) (Variables|Default|GetmaxCameraDistance)))))

(event Custom|ResetCameraRotation
  ;[1 1 1] Reset camera position
  (Variables|Default|SetpreResetCameraRot (Transformation|GetActorRotation))
  (bind _alpha (Timeline|CameraReset PlayFromStart)
    (:Update
      (Transformation|SetActorRotation (Math|Rotator|MakeRotator 0.0 (.pitch (Math|Rotator|Lerp(Rotator) (Variables|Default|GetpreResetCameraRot) (Variables|Default|GetdefaultRotation) _alpha true)) (.yaw (Math|Rotator|Lerp(Rotator) (Variables|Default|GetpreResetCameraRot) (Variables|Default|GetdefaultRotation) _alpha true)))))
    (:Finished
      (Variables|Default|SetisFollowing true))))

(event Custom|MoveInputStopped
  (Variables|Default|SetisMoving false))

(event Custom|CameraMovementToggle
  (params (CanMove :type Boolean))
  (Variables|Default|SetisCameraMovable CanMove))

(event Custom|SwitchCam
  (params (CurrentGameState :type E_GameState%20Enum :default "NewEnumerator0"))
  ;[1 1 1] Switches Cam State
  (switch Utilities|FlowControl|Switch|SwitchonE_GameState CurrentGameState
    (:NewEnumerator0
      (Variables|Default|SetCurrentGameState "NewEnumerator0")
      (CallFunction|TransitionGameState))
    (:NewEnumerator1
      (Variables|Default|SetCurrentGameState "NewEnumerator1")
      (Variables|Default|SetisCamFree false)
      (CallFunction|StopReset)
      (CallFunction|TransitionGameState))
    (:NewEnumerator2
      (Variables|Default|SetCurrentGameState "NewEnumerator2"))))

(event EventTick
  (params (DeltaSeconds :type Float%20%28single-precision%29))
  (bind _target (Variables|Default|GetTarget))
  (bind _camera (Variables|Default|GetCamera))
  (bind _ship (Variables|Default|Getship))
  (bind _ship_2 (Variables|Default|Getship))
  (bind _camerapositionoffset (Variables|Default|GetcameraPositionOffset))
  (bind _camera_2 (Variables|Default|GetCamera))
  (bind _returnvalue (Transformation|GetActorLocation _ship))
  (bind _returnvalue_2 (Transformation|GetActorLocation _target))
  (bind _returnvalue_3 (Transformation|GetActorLocation _ship_2))
  (bind _relativerotation (Variables|/Script/Engine.SceneComponent|GetRelativeRotation _camera_2))
  (bind _returnvalue_4 (- _returnvalue_2 _returnvalue))
  (bind _returnvalue_5 (+ _returnvalue_3 _camerapositionoffset))
  (switch Utilities|FlowControl|Switch|SwitchonE_GameState (Variables|Default|GetCurrentGameState)
    (:NewEnumerator0
      ;[1 1 1] Updates position
      (if (Variables|Default|GetisTransitioning)
        ;[1 1 1] If is transitioning back to default rotation, this updates the default rotation Z
        (Variables|Default|SetdefaultRotation (Math|Rotator|MakeRotator 0.0 -15.0 (.yaw (Transformation|GetActorRotation (Variables|Default|Getship)))) :!label _label)
        (else
          (Transformation|SetActorLocation (+ (Transformation|GetActorLocation (Variables|Default|Getship)) (Variables|Default|GetcameraPositionOffset)) false false)
          ;[1 1 1] Makes the cam follow the ship rotation
          (if (Variables|Default|GetisFollowing)
            (Transformation|SetActorRotation (Math|Rotator|MakeRotator 0.0 (.pitch (Transformation|GetActorRotation)) (.yaw (Transformation|GetActorRotation (Variables|Default|Getship)))))
            (elif (Variables|Default|GetisCameraMovable)
              (goto _label))))))
    (:NewEnumerator1
      ;[1 1 1] Spring Arm Location
      (Transformation|SetActorLocation (Math|Vector|MakeVector (.x (+ (/ (- (Transformation|GetActorLocation (Variables|Default|GetTarget)) (Transformation|GetActorLocation (Variables|Default|Getship))) 2) (Transformation|GetActorLocation (Variables|Default|Getship)))) (.y _returnvalue_5) (.z _returnvalue_5)) false false)
      ;[1 1 1] Spring arm rotation
      (Transformation|SetActorRotation (Math|Rotator|MakeRotator 0.0 (- 3.6e+02 (Variables|Default|GetCameraViewAngle)) 0.0))
      ;[1 1 1] Camera Rotation
      (Transformation|SetWorldRotation _camera (Math|Rotator|MakeRotator 0.0 (.pitch (Transformation|GetWorldRotation _camera)) (.yaw (Math|Rotator|FindLookatRotation (Transformation|GetWorldLocation _camera) (+ (/ (- (Transformation|GetActorLocation (Variables|Default|GetTarget)) (Transformation|GetActorLocation (Variables|Default|Getship))) 2) (Transformation|GetActorLocation (Variables|Default|Getship)))))) false false)
      (Transformation|SetRelativeRotation _camera_2 (Math|Rotator|MakeRotator 0.0 (.pitch _relativerotation) (.yaw _relativerotation)) false false)
      (if (>= (Math|Vector|VectorLength _returnvalue_4) (Variables|Default|GetCombatCameraZoomCutOff))
        (Variables|/Script/Engine.SpringArmComponent|SetTargetArmLength (Variables|Default|GetSpringArm) (+ (* (Variables|Default|GetCombatCameraZoomMultiplier) (- (Math|Vector|VectorLength _returnvalue_4) (Variables|Default|GetCombatCameraZoomCutOff))) (Variables|Default|GetCombatCameraMinimunArmLength)))
        (else
          (Variables|/Script/Engine.SpringArmComponent|SetTargetArmLength (Variables|Default|GetSpringArm) (Variables|Default|GetCombatCameraMinimunArmLength)))))))

(fn ConstructionScript)