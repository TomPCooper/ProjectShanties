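; Player ship pawn with physics-based sailing, a spawned follow camera and a toggleable combat aiming mode.
; Niagara reads GPU wave heights back to pontoons, whose spherical-cap submerged volumes drive buoyancy forces and scale forward thrust.
; Input applies speed-capped thrust and speed-scaled turning, while look input moves either the camera or a trace-constrained crosshair.
; Data-table-driven attack components supply the range indicator for the selected weapon; radial menu handlers only print.
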(event Custom|AddForceAtPoint
  (params (force :type Vector) (location :type Vector))
  ;[1 1 1] Functions for adding extra forces to ship
  (Class|PrimitiveComponent|AddForceatLocation (Variables|Components|GetBoat) force location "None"))

(event Custom|AddForward
  (params (forwardInput :type Float%20%28double-precision%29))
  (bind _returnvalue (Transformation|GetActorForwardVector))
  (bind _averagesubmergedamount (Variables|Buoyancy|GetaverageSubmergedAmount))
  (bind _moveforce (Variables|Movement|GetmoveForce))
  (bind _returnvalue_2 (* _averagesubmergedamount 2.25))
  (bind _returnvalue_3 (* forwardInput _returnvalue _moveforce _returnvalue_2))
  ;[1 1 1] Adds forward force
  (if (> forwardInput 0.0)
    (Physics|AddImpulse (Variables|Components|GetBoat) _returnvalue_3 "None" true)
    (else
      (Physics|AddImpulse (Variables|Components|GetBoat) (* _returnvalue_3 (Variables|Movement|GetbackwardsMoveMultiplier)) "None" true) ; If moving backwards, force is\nreduced
    )))

(event Custom|AddTurn
  (params (turnInput :type Float%20%28double-precision%29))
  ;[1 1 1] Adds turning force
  (Class|PrimitiveComponent|AddAngularImpulseinDegrees (Variables|Components|GetBoat) (* turnInput (Variables|Movement|GetturnForce) (Math|Float|MapRangeClamped (/ (Variables|Default|GetcurrentSpeed) (Variables|Default|GetmaxSpeed)) 0.0 1.0 0.2 1.0) (Math|Vector|GetUpVector (Variables|Components|GetBoat))) "None" true))

(event Custom|Event%20DoCrosshairMovement
  (params (InputX :type Float%20%28double-precision%29) (InputY :type Float%20%28double-precision%29))
  (bind _child_crosshair (Variables|Components|GetChild_Crosshair))
  (bind _child_crosshair_2 (Variables|Components|GetChild_Crosshair))
  (bind _child_crosshair_3 (Variables|Components|GetChild_Crosshair))
  (bind _crosshair_sensitivity (Variables|Combat|GetCrosshair%20Sensitivity))
  (bind _camera (Variables|Default|Getcamera))
  (bind _returnvalue (Transformation|GetActorRightVector _camera))
  (bind _returnvalue_2 (Transformation|GetActorUpVector _camera))
  (bind _childactor (Variables|/Script/Engine.ChildActorComponent|GetChildActor _child_crosshair_2))
  (bind _childactor_2 (Variables|/Script/Engine.ChildActorComponent|GetChildActor _child_crosshair_3))
  (bind _returnvalue_3 (Transformation|GetActorLocation _childactor))
  (bind _returnvalue_4 (Transformation|GetActorLocation _childactor_2))
  (bind _returnvalue_5 (* _returnvalue_2 _crosshair_sensitivity -1.0 InputY))
  (bind _returnvalue_6 (* _returnvalue _crosshair_sensitivity InputX))
  (bind _returnvalue_7 (+ _returnvalue_6 _returnvalue_5))
  ;[0.125 0.002436 0] Combat
  ;;[1 1 1] Updates
  (bind (_outhit _returnvalue_8) (Collision|LineTraceForObjects _returnvalue_4 (+ _returnvalue_4 (* _returnvalue_7 1e+01)) (Utilities|Array|MakeArray "ObjectTypeQuery8") false 0 "None"))
  (if _returnvalue_8
    (Transformation|SetWorldLocation _child_crosshair (Math|Vector|MakeVector (.x (Math|Vector|Lerp(Vector) _returnvalue_3 (- (.Location (Collision|BreakHitResult _outhit)) (* (Math|Vector|GetUnitDirection(Vector) _returnvalue_3 (.Location (Collision|BreakHitResult _outhit))) 1e+01)) 0.35)) (.y (Math|Vector|Lerp(Vector) _returnvalue_3 (- (.Location (Collision|BreakHitResult _outhit)) (* (Math|Vector|GetUnitDirection(Vector) _returnvalue_3 (.Location (Collision|BreakHitResult _outhit))) 1e+01)) 0.35)) (.z (Transformation|GetWorldLocation _child_crosshair))) false false)
    (else
      (Transformation|AddWorldOffset (Variables|Components|GetChild_Crosshair) _returnvalue_7 false false))))

(event Custom|Event%20EnterCombatMode
  ;[0.125 0.002436 0] Combat
  ;;[1 1 1] Initialisation
  (Variables|Combat|SetInCombatMode true)
  (Input|SetInputModeGameOnly (Game|GetPlayerController 0) false)
  (bind _returnvalue (Utilities|Time|SetTimerbyEvent (EventDispatchers|CreateEvent :!event Custom|Event%20LocationUpdate) 0.01 true))
  (Variables|Combat|SetLocationUpdateTimer _returnvalue))

(event Custom|Event%20InitialiseCrosshair
  ;[0.125 0.002436 0] Combat
  ;;[1 1 1] Initialisation
  (Rendering|SetVisibility (Variables|Components|GetChild_Crosshair) true false)
  (bind _bpc_attack (CallFunction|SetAttackRangeType))
  (bind _output_get (Variables|Components|SetBPC_AttackRef _bpc_attack))
  (ChildActorComponent|SetChildActorClass (Variables|Components|GetChild_AttackRange) (Variables|/Game/Blueprints/Attacks/BPC_Base_Attack.BPC_Base_Attack_C|GetAttackRangeClass _output_get))
  (Rendering|SetVisibility (Variables|Components|GetChild_AttackRange) true false))

(event Custom|Event%20LocationUpdate
  (bind _returnvalue (Transformation|GetActorLocation))
  (bind _child_crosshair (Variables|Components|GetChild_Crosshair))
  (bind _childactor (Variables|/Script/Engine.ChildActorComponent|GetChildActor _child_crosshair))
  (bind _returnvalue_2 (Transformation|GetActorLocation _childactor))
  ;[0.125 0.002436 0] Combat
  ;;[1 1 1] Updates
  (Transformation|SetWorldLocationAndRotation (Variables|Components|GetChild_AttackRange) (Math|Vector|MakeVector (.x _returnvalue) (.y _returnvalue) (+ (.z _returnvalue) (Variables|Combat|GetLocation%20Offset))) (Math|Rotator|MakeRotator 0.0 0.0 (.yaw (Transformation|GetActorRotation))) false false)
  (Transformation|SetWorldRotation (Variables|Components|GetChild_Crosshair) (Math|Rotator|MakeRotator 0.0 0.0 (.yaw (Transformation|GetActorRotation (Variables|Default|Getcamera)))) false false)
  (Transformation|SetWorldLocation (Variables|Components|GetChild_Crosshair) (Math|Vector|MakeVector (.x _returnvalue_2) (.y _returnvalue_2) (+ (Variables|Combat|GetLocation%20Offset) (.z (Transformation|GetActorLocation)))) false false))

(event EventILookInput
  (params (AxisX :type Float%20%28double-precision%29) (AxisY :type Float%20%28double-precision%29))
  ;[1 1 1] Camera look input
  (if (Variables|Combat|GetInCombatMode)
    (CallFunction|EventDoCrosshairMovement AxisX AxisY)
    (else
      (Default|LookInput (Variables|Default|Getcamera) AxisX AxisY))))

(event EventICameraMovementToggle
  (params (CanMove :type Boolean))
  ;[1 1 1] Toggles whether the camera can move
  (Default|CameraMovementToggle (Variables|Default|Getcamera) CanMove))

(event EventBeginPlay
  (bind _returnvalue (Game|GetPlayerController 0))
  (bind _fx_systreadback (Variables|Components|GetFX_SystReadback))
  (bind _returnvalue_2 (Actor|GetComponentbyClass _returnvalue "/Game/Blueprints/Water/Foam/BP_Foam_Controller_Component.BP_Foam_Controller_Component_C"))
  ;[0 1 0] Ship initialisation
  (Utilities|FlowControl|Sequence
    (:then_0
      ;[0 1 0] Niagara buoyancy system setup
      (Class|NiagaraComponent|SetVariableObject _fx_systreadback "Actor" self)
      (Class|NiagaraComponent|SetVariableBool _fx_systreadback "bExport" true)
      (Class|NiagaraDataInterfaceArrayFunctionLibrary|SetNiagaraArrayVector _fx_systreadback "Pontoons" (Variables|Buoyancy|Getpontoons))
      (Niagara|ReinitializeSystem _fx_systreadback)
      (Utilities|Array|Clear (Variables|Buoyancy|GetpontoonSubmergedAmounts))
      ;[0 1 0] Initialises array for pontoon submerged amounts
      (for _array_element (Variables|Buoyancy|Getpontoons)
        (Utilities|Array|Add (Variables|Buoyancy|GetpontoonSubmergedAmounts) 1.0))
      (Variables|Buoyancy|SetaverageSubmergedAmount 1.0)
      (Variables|Buoyancy|SetfullPontoonVolume (* (Math|Float|Power (Variables|Buoyancy|GetpontoonRadius) 3.0) (Math|Trig|GetPI) (/ 4.0 3.0)))
      ;[0 1 0] Spawns player camera
      (bind _returnvalue_3 (Game|SpawnActorfromClass "/Game/Blueprints/t014172k/BP_PlayerCamera.BP_PlayerCamera_C" (Transformation|GetActorTransform) "AlwaysSpawn" "MultiplyWithRoot" 0 0))
      (bind _output_get (Variables|Default|Setcamera _returnvalue_3))
      (Default|Init _output_get)
      ;[0 1 0] Initialises foam controller
      (Utilities|IsValid _returnvalue_2
        (:Is%20Valid
          (Default|AddFoamComponent _returnvalue_2 (Variables|Components|GetBoat)))))
    (:then_1
      (CallFunction|AddNewAttackType "NewEnumerator0"))))

(event EventIInit
  (bind _returnvalue (Game|GetPlayerController 0))
  (bind _fx_systreadback (Variables|Components|GetFX_SystReadback))
  (bind _returnvalue_2 (Actor|GetComponentbyClass _returnvalue "/Game/Blueprints/Water/Foam/BP_Foam_Controller_Component.BP_Foam_Controller_Component_C"))
  ;[0 1 0] Ship initialisation
  (Utilities|FlowControl|Sequence
    (:then_0
      ;[0 1 0] Niagara buoyancy system setup
      (Class|NiagaraComponent|SetVariableObject _fx_systreadback "Actor" self)
      (Class|NiagaraComponent|SetVariableBool _fx_systreadback "bExport" true)
      (Class|NiagaraDataInterfaceArrayFunctionLibrary|SetNiagaraArrayVector _fx_systreadback "Pontoons" (Variables|Buoyancy|Getpontoons))
      (Niagara|ReinitializeSystem _fx_systreadback)
      (Utilities|Array|Clear (Variables|Buoyancy|GetpontoonSubmergedAmounts))
      ;[0 1 0] Initialises array for pontoon submerged amounts
      (for _array_element (Variables|Buoyancy|Getpontoons)
        (Utilities|Array|Add (Variables|Buoyancy|GetpontoonSubmergedAmounts) 1.0))
      (Variables|Buoyancy|SetaverageSubmergedAmount 1.0)
      (Variables|Buoyancy|SetfullPontoonVolume (* (Math|Float|Power (Variables|Buoyancy|GetpontoonRadius) 3.0) (Math|Trig|GetPI) (/ 4.0 3.0)))
      ;[0 1 0] Spawns player camera
      (bind _returnvalue_3 (Game|SpawnActorfromClass "/Game/Blueprints/t014172k/BP_PlayerCamera.BP_PlayerCamera_C" (Transformation|GetActorTransform) "AlwaysSpawn" "MultiplyWithRoot" 0 0))
      (bind _output_get (Variables|Default|Setcamera _returnvalue_3))
      (Default|Init _output_get)
      ;[0 1 0] Initialises foam controller
      (Utilities|IsValid _returnvalue_2
        (:Is%20Valid
          (Default|AddFoamComponent _returnvalue_2 (Variables|Components|GetBoat)))))
    (:then_1
      (CallFunction|AddNewAttackType "NewEnumerator0"))))

(event EventTick
  (params (DeltaSeconds :type Float%20%28single-precision%29))
  (bind _pontoons (Variables|Buoyancy|Getpontoons))
  (bind _boat (Variables|Components|GetBoat))
  ;[0 1 0] Calculate the submerged depth
  (Utilities|FlowControl|Sequence
    (:then_0
      (if (Variables|Buoyancy|GetsimulateBuoyancy)
        (for (_array_element _array_index) (Variables|Buoyancy|GetData)
          (if (Utilities|Array|IsValidIndex _pontoons _array_index) ; If pontoon index is a valid position
            ;[0 1 0] Calculates submerged volume for each pontoon
            (Utilities|Array|SetArrayElem (Variables|Buoyancy|GetpontoonSubmergedAmounts) _array_index (/ (* (Math|Float|MultiplybyPi 0.333333) (Math|Float|Square (Math|Float|Clamp(Float) (Utilities|Operators|Subtract (.Size (Utilities|Struct|BreakBasicParticleData _array_element)) (* (.Z (Class|KismetMathLibrary|BreakVector3f (Transformation|GetWorldLocation (Variables|Components|GetwaterPlane)))) -1.0) (.Z (Class|KismetMathLibrary|BreakVector3f (Math|Transform|TransformLocation (Transformation|GetWorldTransform _boat) (/ (Utilities|Array|Get(acopy) _pontoons _array_index) (Transformation|GetWorldScale _boat)))))) 0.0 (* (Variables|Buoyancy|GetpontoonRadius) 2.0))) (- (* (Variables|Buoyancy|GetpontoonRadius) 3.0) (Math|Float|Clamp(Float) (Utilities|Operators|Subtract (.Size (Utilities|Struct|BreakBasicParticleData _array_element)) (* (.Z (Class|KismetMathLibrary|BreakVector3f (Transformation|GetWorldLocation (Variables|Components|GetwaterPlane)))) -1.0) (.Z (Class|KismetMathLibrary|BreakVector3f (Math|Transform|TransformLocation (Transformation|GetWorldTransform _boat) (/ (Utilities|Array|Get(acopy) _pontoons _array_index) (Transformation|GetWorldScale _boat)))))) 0.0 (* (Variables|Buoyancy|GetpontoonRadius) 2.0)))) (Variables|Buoyancy|GetfullPontoonVolume)))
            (if (> (* (Math|Float|MultiplybyPi 0.333333) (Math|Float|Square (Math|Float|Clamp(Float) (Utilities|Operators|Subtract (.Size (Utilities|Struct|BreakBasicParticleData _array_element)) (* (.Z (Class|KismetMathLibrary|BreakVector3f (Transformation|GetWorldLocation (Variables|Components|GetwaterPlane)))) -1.0) (.Z (Class|KismetMathLibrary|BreakVector3f (Math|Transform|TransformLocation (Transformation|GetWorldTransform _boat) (/ (Utilities|Array|Get(acopy) _pontoons _array_index) (Transformation|GetWorldScale _boat)))))) 0.0 (* (Variables|Buoyancy|GetpontoonRadius) 2.0))) (- (* (Variables|Buoyancy|GetpontoonRadius) 3.0) (Math|Float|Clamp(Float) (Utilities|Operators|Subtract (.Size (Utilities|Struct|BreakBasicParticleData _array_element)) (* (.Z (Class|KismetMathLibrary|BreakVector3f (Transformation|GetWorldLocation (Variables|Components|GetwaterPlane)))) -1.0) (.Z (Class|KismetMathLibrary|BreakVector3f (Math|Transform|TransformLocation (Transformation|GetWorldTransform _boat) (/ (Utilities|Array|Get(acopy) _pontoons _array_index) (Transformation|GetWorldScale _boat)))))) 0.0 (* (Variables|Buoyancy|GetpontoonRadius) 2.0)))) 0.0)
              (Class|PrimitiveComponent|AddForceatLocationLocal (Variables|Components|GetBoat) (* (* (Math|Float|MultiplybyPi 0.333333) (Math|Float|Square (Math|Float|Clamp(Float) (Utilities|Operators|Subtract (.Size (Utilities|Struct|BreakBasicParticleData _array_element)) (* (.Z (Class|KismetMathLibrary|BreakVector3f (Transformation|GetWorldLocation (Variables|Components|GetwaterPlane)))) -1.0) (.Z (Class|KismetMathLibrary|BreakVector3f (Math|Transform|TransformLocation (Transformation|GetWorldTransform _boat) (/ (Utilities|Array|Get(acopy) _pontoons _array_index) (Transformation|GetWorldScale _boat)))))) 0.0 (* (Variables|Buoyancy|GetpontoonRadius) 2.0))) (- (* (Variables|Buoyancy|GetpontoonRadius) 3.0) (Math|Float|Clamp(Float) (Utilities|Operators|Subtract (.Size (Utilities|Struct|BreakBasicParticleData _array_element)) (* (.Z (Class|KismetMathLibrary|BreakVector3f (Transformation|GetWorldLocation (Variables|Components|GetwaterPlane)))) -1.0) (.Z (Class|KismetMathLibrary|BreakVector3f (Math|Transform|TransformLocation (Transformation|GetWorldTransform _boat) (/ (Utilities|Array|Get(acopy) _pontoons _array_index) (Transformation|GetWorldScale _boat)))))) 0.0 (* (Variables|Buoyancy|GetpontoonRadius) 2.0)))) (Math|Vector|VectorUp)) (Utilities|Array|Get(acopy) _pontoons _array_index) "None"))))
        (CallFunction|UpdateAverageSubmerged)))
    (:then_1
      (CallFunction|MaxSpeedClamp))))

(event EventIAttackReleased
  ;[1 1 1] Used to control radial menu
  (Development|PrintString "Close radial menu"))

(event EventIAttackPressed
  ;[1 1 1] Used to control radial menu
  (Development|PrintString "Open radial menu"))

(event EventIMoveInputStarted
  ;[1 1 1] Resets camera when the boat starts to move again
  (Default|MoveInputStarted (Variables|Default|Getcamera)))

(event EventIMoveInputTriggered
  (params (AxisX :type Float%20%28double-precision%29) (AxisY :type Float%20%28double-precision%29))
  ;[1 1 1] Checks player input to see whether forces need to be added to ship
  (Utilities|FlowControl|Sequence ; Handles x and y components separately
    (:then_0
      (if (> (Math|Float|Absolute(Float) AxisX) 0.0)
        (CallFunction|AddTurn AxisX)))
    (:then_1
      (if (> (Math|Float|Absolute(Float) AxisY) 0.0)
        (CallFunction|AddForward AxisY)))))

(event EventIZoomInput
  (params (InputAxis :type Float%20%28double-precision%29))
  ;[1 1 1] Camera zoom input
  (Default|ZoomInput (Variables|Default|Getcamera) InputAxis))

(event EventIAddForcetoShip
  (params (forceToAdd :type Vector :default "0, 0, 0"))
  ;[1 1 1] Functions for adding extra forces to ship
  (Physics|AddForce (Variables|Components|GetBoat) forceToAdd "None" true))

(event EventIGetMovingWaterPlane
  (params (mesh :type Static%20Mesh%20Component%20Object%20Reference))
  ;[1 1 1] Updates positioning to be used in ship rotations
  (Variables|Components|SetwaterPlane mesh))

(event EventParticleData
  (params (Data :type Array%20of%20Basic%20Particle%20Data%20Structures) (NiagaraSystem :type Niagara%20System%20Object%20Reference) (SimulationPositionOffset :type Vector%20%28by%20ref%29 :default "0, 0, 0"))
  ;[1 1 1] Stores wave height data sent over from GPU
  (Variables|Buoyancy|SetData Data))

(event EventIMoveInputStopped
  ;[1 1 1] Resets camera when the boat starts to move again
  (Default|MoveInputStopped (Variables|Default|Getcamera)))

(event Input|KeyboardEvents|Q
  (params (Key :type Key%20Structure))
  ;[0.125 0.002436 0] Combat
  ;;[1 1 1] Initialisation
  (:Pressed
    (Utilities|FlowControl|FlipFlop
      (:A
        (CallFunction|EventEnterCombatMode)
        (CallFunction|EventInitialiseCrosshair)
        (CallFunction|ICameraMovementToggle false))
      (:B
        (Rendering|SetVisibility (Variables|Components|GetChild_Crosshair) false false)
        (Rendering|SetVisibility (Variables|Components|GetChild_AttackRange) false false)
        (Utilities|Time|ClearandInvalidateTimerbyHandle (Variables|Combat|GetLocationUpdateTimer))
        (Variables|Combat|SetInCombatMode false)
        (CallFunction|ICameraMovementToggle true)))))

(event Input|KeyboardEvents|T
  (params (Key :type Key%20Structure))
  (:Pressed
    (Utilities|FlowControl|FlipFlop
      (:A
        (CallFunction|SwitchWeapons "NewEnumerator1"))
      (:B
        (CallFunction|SwitchWeapons "NewEnumerator0")))))

(fn ConstructionScript)

(fn SetAttackRangeType
  (for _array_element (Variables|Combat|GetCurrentAttackComponents)
    (if (Utilities|Enum|Equal(Enum) (Variables|/Game/Blueprints/Attacks/BPC_Base_Attack.BPC_Base_Attack_C|GetAttackType _array_element) (Variables|Combat|GetSelectedAttackType))
      (return _array_element)))
  (return 0))

(fn UpdateAverageSubmerged
  (bind _pontoonsubmergedamounts (Variables|Buoyancy|GetpontoonSubmergedAmounts))
  (for _array_element _pontoonsubmergedamounts
    (LocalVariables|SetworkingAvg (+ (LocalVariables|GetworkingAvg) _array_element)))
  (Variables|Buoyancy|SetaverageSubmergedAmount (/ (LocalVariables|GetworkingAvg) (Utilities|Array|Length _pontoonsubmergedamounts))))

(fn MaxSpeedClamp
  (bind _maxspeed (Variables|Default|GetmaxSpeed))
  ;[1 1 1] Clamps boat speed to the max speed value
  (Utilities|FlowControl|Sequence
    (:then_0
      (bind _returnvalue (Physics|GetPhysicsLinearVelocity (Variables|Components|GetBoat) "None"))
      (bind _output_get (LocalVariables|SetcurrentVelocity _returnvalue))
      (if (> (Class|KismetMathLibrary|VSizeXYSquared _output_get) (Math|Float|Square _maxspeed)) ; Is current speed faster than max speed\n(using squared is faster as it avoids\nsquare rooting)
        (Physics|SetPhysicsLinearVelocity (Variables|Components|GetBoat) (* (LocalVariables|GetcurrentVelocity) (/ _maxspeed (Math|Float|Sqrt (Class|KismetMathLibrary|VSizeXYSquared _output_get)))) false "None")))
    (:then_1
      (bind _returnvalue_2 (Physics|GetPhysicsLinearVelocity (Variables|Components|GetBoat) "None"))
      (Variables|Default|SetcurrentSpeed (Math|Vector|VectorLengthXY _returnvalue_2)))))

(fn UpdateAttackTypes
  ;[0.125 0.002436 0] s014480m
  (for _array_element (Variables|Combat|GetCurrentAttackComponents)
    (Components|DestroyComponent _array_element))
  (for _array_element_2 (Variables|Combat|GetAvailableAttackTypes)
    (if (not (Utilities|Array|ContainsItem (LocalVariables|GetUniqueAttackTypes) _array_element_2))
      (bind _returnvalue (Utilities|GetDataTableRow "/Game/Blueprints/Attacks/DT_AttackTypeToComponent.DT_AttackTypeToComponent" (Utilities|String|StringToName (Utilities|String|EnumtoString _array_element_2)))
        (:then
          (Utilities|Array|Add (LocalVariables|GetUniqueAttackTypes) _array_element_2)
          (bind _returnvalue_2 (Game|AddComponentbyClass (.Value (Utilities|Map|Find (Utilities|Struct|BreakS_AttackType _returnvalue) _array_element_2))))
          (Utilities|Array|Add (Variables|Combat|GetCurrentAttackComponents) _returnvalue_2))
        (:RowNotFound
          (Development|PrintString "Attack Type not found in data table" true true "(R=1.000000,G=0.000000,B=0.000000,A=1.000000)"))))))

(fn AddNewAttackType
  (params (AttackType :type E_AttackType%20Enum :default "NewEnumerator0"))
  (Utilities|Array|AddUnique (Variables|Combat|GetAvailableAttackTypes) AttackType)
  (CallFunction|UpdateAttackTypes))

(fn SwitchWeapons
  (params (NewAttackType :type E_AttackType%20Enum :default "NewEnumerator0"))
  (Variables|Combat|SetSelectedAttackType NewAttackType))

(fn IBossGetLeapPosition
  (return "0, 0, 0"))

(fn IGetShipMesh
  (return 0))