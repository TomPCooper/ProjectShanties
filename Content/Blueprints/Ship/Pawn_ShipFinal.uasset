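; Player ship pawn that handles physics sailing, combat aiming, firing and damage reported to the HUD.
; A Niagara system exports GPU wave data to the buoyancy component, whose pontoon submersion scales forward impulses, while turning scales with speed.
; Combat mode, set by Q or the boss, redirects look input from the spawned camera to a trace-limited crosshair that aims the projectile spawner.
; Data tables map attack types to components and range indicators.
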(event Custom|AddForceAtPoint
  (params (force :type Vector) (location :type Vector))
  ;[1 0.8589 0] Player Movement
  ;;[1 1 1] Functions for adding extra forces to ship
  (Class|PrimitiveComponent|AddForceatLocation (Variables|Default|GetSM_Boat) force location "None"))

(event Custom|AddForward
  (params (forwardInput :type Float%20%28double-precision%29))
  (bind _returnvalue (Transformation|GetActorForwardVector))
  (bind _bpc_ship_buoyancy_component (Variables|Default|GetBPC_Ship_Buoyancy_Component))
  (bind _movementforce (Variables|Movement|GetMovementForce))
  (bind _pontoonsaveragesubmergedamount (Variables|/Game/Blueprints/Ship/Ship_Components/BP_Ship_Buoyancy_Component.BP_Ship_Buoyancy_Component_C|GetPontoonsAverageSubmergedAmount _bpc_ship_buoyancy_component))
  (bind _returnvalue_2 (* _pontoonsaveragesubmergedamount 2.25))
  (bind _returnvalue_3 (* forwardInput _returnvalue _movementforce _returnvalue_2))
  ;[1 0.8589 0] Player Movement
  ;;[1 1 1] Adds forward force
  (if (> forwardInput 0.0)
    (Physics|AddImpulse (Variables|Default|GetSM_Boat) _returnvalue_3 "None" true)
    (else
      (Physics|AddImpulse (Variables|Default|GetSM_Boat) (* _returnvalue_3 (Variables|Movement|GetBackwardsMovementMultiplier)) "None" true) ; If moving backwards, force is\nreduced
    )))

(event Custom|AddTurn
  (params (turnInput :type Float%20%28double-precision%29))
  ;[1 0.8589 0] Player Movement
  ;;[1 1 1] Adds turning force
  (Class|PrimitiveComponent|AddAngularImpulseinDegrees (Variables|Default|GetSM_Boat) (* turnInput (Variables|Movement|GetTurningForce) (Math|Float|MapRangeClamped (/ (Variables|Misc|GetcurrentSpeed) (Variables|Misc|GetmaxSpeed)) 0.0 1.0 0.2 1.0) (Math|Vector|GetUpVector (Variables|Default|GetSM_Boat))) "None" true))

(event Custom|ExitCombatMode
  ;[0.125 0.002436 0] Combat
  ;;[1 1 1] Initialisation
  ;;;[1 1 1] Exit Combat Mode
  (Variables|Combat|SetInCombatMode false)
  (CallFunction|ICameraMovementToggle true))

(event Custom|Event%20DoCrosshairMovement
  (params (InputX :type Float%20%28double-precision%29) (InputY :type Float%20%28double-precision%29))
  (bind _child_crosshair (Variables|Default|GetChild_Crosshair))
  (bind _child_projectilespawner (Variables|Default|GetChild_ProjectileSpawner))
  (bind _child_crosshair_2 (Variables|Default|GetChild_Crosshair))
  (bind _child_crosshair_3 (Variables|Default|GetChild_Crosshair))
  (bind _crosshair_sensitivity (Variables|Combat|GetCrosshair%20Sensitivity))
  (bind _camera (Variables|Misc|Getcamera))
  (bind _returnvalue (Transformation|GetActorRightVector _camera))
  (bind _returnvalue_2 (Transformation|GetActorUpVector _camera))
  (bind _childactor (Variables|/Script/Engine.ChildActorComponent|GetChildActor _child_crosshair_2))
  (bind _childactor_2 (Variables|/Script/Engine.ChildActorComponent|GetChildActor _child_crosshair_3))
  (bind _returnvalue_3 (Transformation|GetActorLocation _childactor))
  (bind _returnvalue_4 (Transformation|GetActorLocation _childactor_2))
  (bind _returnvalue_5 (* _returnvalue_2 _crosshair_sensitivity -1.0 InputY))
  (bind _returnvalue_6 (* _returnvalue _crosshair_sensitivity InputX))
  (bind _returnvalue_7 (+ _returnvalue_6 _returnvalue_5))
  ;[0.125 0.002436 0] Combat
  ;;[1 1 1] Updates
  ;;;[1 1 1] Move Crosshair
  (bind (_outhit _returnvalue_8) (Collision|LineTraceForObjects _returnvalue_4 (+ _returnvalue_4 (* _returnvalue_7 1e+01)) (Utilities|Array|MakeArray "ObjectTypeQuery8") false 0 "None"))
  (if _returnvalue_8
    (Transformation|SetWorldLocation _child_crosshair (Math|Vector|MakeVector (.x (Math|Vector|Lerp(Vector) _returnvalue_3 (- (.Location (Collision|BreakHitResult _outhit)) (* (Math|Vector|GetUnitDirection(Vector) _returnvalue_3 (.Location (Collision|BreakHitResult _outhit))) 1e+01)) 0.35)) (.y (Math|Vector|Lerp(Vector) _returnvalue_3 (- (.Location (Collision|BreakHitResult _outhit)) (* (Math|Vector|GetUnitDirection(Vector) _returnvalue_3 (.Location (Collision|BreakHitResult _outhit))) 1e+01)) 0.35)) (.z (Transformation|GetWorldLocation _child_crosshair))) false false)
    (else
      (Transformation|AddWorldOffset (Variables|Default|GetChild_Crosshair) _returnvalue_7 false false)))
  (Transformation|SetRelativeRotation _child_projectilespawner (Math|Rotator|MakeRotator 0.0 0.0 (.yaw (Math|Rotator|FindLookatRotation (Variables|/Script/Engine.SceneComponent|GetRelativeLocation _child_projectilespawner) (Variables|/Script/Engine.SceneComponent|GetRelativeLocation _child_crosshair)))) false false))

(event Custom|Event%20EnterCombatMode
  ;[0.125 0.002436 0] Combat
  ;;[1 1 1] Initialisation
  ;;;[1 1 1] Enter Combat Mode
  (Variables|Combat|SetInCombatMode true)
  (Input|SetInputModeGameOnly (Game|GetPlayerController 0) false)
  (bind _returnvalue (Utilities|Time|SetTimerbyEvent (EventDispatchers|CreateEvent :!event Custom|Event%20LocationUpdate) 0.01 true))
  (Variables|Combat|SetLocationUpdateTimer _returnvalue))

(event Custom|Event%20InitialiseCrosshair
  (bind _child_attackrange (Variables|Default|GetChild_AttackRange))
  ;[0.125 0.002436 0] Combat
  ;;[1 1 1] Initialisation
  ;;;[1 1 1] Enter Combat Mode
  (Rendering|SetVisibility (Variables|Default|GetChild_Crosshair) true false)
  (bind _bpc_attack (CallFunction|SetAttackRangeType))
  (bind _output_get (Variables|Default|SetBPC_AttackRef _bpc_attack))
  (bind _attackrangeclass (CallFunction|GetAttackRangeClass (Variables|/Game/Blueprints/Attacks/BPC_Base_Attack.BPC_Base_Attack_C|GetAttackType _output_get)))
  (ChildActorComponent|SetChildActorClass _child_attackrange _attackrangeclass)
  (Rendering|SetVisibility _child_attackrange true false)
  (Default|CallAimingActive true) ; Call for music manager to update
)

(event Custom|Event%20LocationUpdate
  (bind _returnvalue (Transformation|GetActorLocation))
  (bind _child_crosshair (Variables|Default|GetChild_Crosshair))
  (bind _childactor (Variables|/Script/Engine.ChildActorComponent|GetChildActor _child_crosshair))
  (bind _returnvalue_2 (Transformation|GetActorLocation _childactor))
  ;[0.125 0.002436 0] Combat
  ;;[1 1 1] Updates
  (Transformation|SetWorldLocationAndRotation (Variables|Default|GetChild_AttackRange) (Math|Vector|MakeVector (.x _returnvalue) (.y _returnvalue) (+ (.z _returnvalue) (Variables|Combat|GetLocation%20Offset))) (Math|Rotator|MakeRotator 0.0 0.0 (.yaw (Transformation|GetActorRotation))) false false)
  (Transformation|SetWorldRotation (Variables|Default|GetChild_Crosshair) (Math|Rotator|MakeRotator 0.0 0.0 (.yaw (Transformation|GetActorRotation (Variables|Misc|Getcamera)))) false false)
  (Transformation|SetWorldLocation (Variables|Default|GetChild_Crosshair) (Math|Vector|MakeVector (.x _returnvalue_2) (.y _returnvalue_2) (+ (Variables|Combat|GetLocation%20Offset) (.z (Transformation|GetActorLocation)))) false false))

(event EventILookInput
  (params (AxisX :type Float%20%28double-precision%29) (AxisY :type Float%20%28double-precision%29))
  ;[1 0.5215 0.127] Camera Controls
  ;;[1 1 1] Camera look input
  (if (Variables|Combat|GetInCombatMode)
    (CallFunction|EventDoCrosshairMovement AxisX AxisY)
    (else
      (Default|LookInput (Variables|Misc|Getcamera) AxisX AxisY))))

(event EventICameraMovementToggle
  (params (CanMove :type Boolean))
  ;[1 0.5215 0.127] Camera Controls
  ;;[1 1 1] Toggles whether the camera can move
  (Default|CameraMovementToggle (Variables|Misc|Getcamera) CanMove))

(event EventIDamageShip
  (params (Damage :type Float%20%28double-precision%29))
  (bind _bpc_health (Variables|Default|GetBPC_Health))
  ;[1 1 1] Damage Ship & Update HUD
  (Utilities|IsValid _bpc_health
    (:Is%20Valid
      (Class|BPIHealth|IDamage(Message) _bpc_health Damage)
      (bind _hudreference (Class|BPIPlayerController|GetHUDReference(Message) (Game|GetPlayerController 0)))
      (Utilities|IsValid _hudreference
        (:Is%20Valid
          (Class|BPIUI|SetHealthPercent(Message) _hudreference (/ (Variables|/Game/Blueprints/Health/BPC_Health.BPC_Health_C|GetCurrentHealth _bpc_health) (Variables|/Game/Blueprints/Health/BPC_Health.BPC_Health_C|GetHealthMax _bpc_health))))))))

(event EventBeginPlay
  (bind _returnvalue (Game|GetPlayerController 0))
  (bind _niagara (Variables|Default|GetNiagara))
  (bind _returnvalue_2 (Actor|GetComponentbyClass _returnvalue "/Game/Blueprints/Water/Foam/BP_Foam_Controller_Component.BP_Foam_Controller_Component_C"))
  ;[1 1 1] Start
  ;;[1 1 1] Ship initialisation
  ;;[1 1 1] Initialise buoyancy
  (Class|NiagaraComponent|SetVariableObject _niagara "Actor" self)
  (Class|NiagaraComponent|SetVariableBool _niagara "bExport" true)
  (Class|NiagaraDataInterfaceArrayFunctionLibrary|SetNiagaraArrayVector _niagara "Pontoons" (Variables|/Game/Blueprints/Ship/Ship_Components/BP_Ship_Buoyancy_Component.BP_Ship_Buoyancy_Component_C|GetPontoons (Variables|Default|GetBPC_Ship_Buoyancy_Component)))
  (Niagara|ReinitializeSystem _niagara)
  (Default|InitiateBuoyancy (Variables|Default|GetBPC_Ship_Buoyancy_Component))
  ;;[1 1 1] Spawns player camera
  (bind _returnvalue_3 (Game|SpawnActorfromClass "/Game/Blueprints/t014172k/BP_PlayerCamera.BP_PlayerCamera_C" (Transformation|GetActorTransform) "AlwaysSpawn" "MultiplyWithRoot" 0 0))
  (bind _output_get (Variables|Misc|Setcamera _returnvalue_3))
  (Default|Init _output_get)
  ;;[1 1 1] Initialises foam controller
  (Utilities|IsValid _returnvalue_2
    (:Is%20Valid
      (Default|AddFoamComponent _returnvalue_2 (Variables|Default|GetSM_Boat))
      ;;[1 1 1] Adds cannon attacks
      (CallFunction|AddNewAttackType "NewEnumerator0")
      ;[1 1 1] Initialises the health component
      (Default|InitHealthComponent (Variables|Default|GetBPC_Health)))))

(event EventISetCombatMode
  (params (inCombatMode :type Boolean))
  ;[0.125 0.002436 0] Combat
  ;;[1 1 1] Initialisation
  ;;;[1 1 1] Interface function called by the boss to force combat mode
  (if inCombatMode
    (CallFunction|EventEnterCombatMode)
    (else
      (CallFunction|ExitCombatMode))))

(event EventTick
  (params (DeltaSeconds :type Float%20%28single-precision%29))
  ;[1 1 1] Start
  ;;[1 1 1] Initialise buoyancy
  (Default|TickBuoyancy (Variables|Default|GetBPC_Ship_Buoyancy_Component)))

(event EventIAttackReleased
  ;[1 0.5215 0.127] Camera Controls
  ;;[0.8235 0 1] Control Radial Menu (DEBUG)
  (Development|PrintString "Close radial menu"))

(event EventIAttackPressed
  ;[1 0.5215 0.127] Camera Controls
  ;;[0.8235 0 1] Control Radial Menu (DEBUG)
  (Development|PrintString "Open radial menu"))

(event EventIMoveInputStarted
  ;[1 0.5215 0.127] Camera Controls
  ;;[1 1 1] Resets camera when the boat starts to move again
  (Default|MoveInputStarted (Variables|Misc|Getcamera)))

(event EventIMoveInputTriggered
  (params (AxisX :type Float%20%28double-precision%29) (AxisY :type Float%20%28double-precision%29))
  ;[1 0.8589 0] Player Movement
  ;;[1 1 1] Checks player input to see whether forces need to be added to ship
  (Utilities|FlowControl|Sequence ; Handles x and y components separately
    (:then_0
      (if (> (Math|Float|Absolute(Float) AxisX) 0.0)
        (CallFunction|AddTurn AxisX)))
    (:then_1
      (if (> (Math|Float|Absolute(Float) AxisY) 0.0)
        (CallFunction|AddForward AxisY)))))

(event EventIZoomInput
  (params (InputAxis :type Float%20%28double-precision%29))
  ;[1 0.5215 0.127] Camera Controls
  ;;[1 1 1] Camera zoom input
  (Default|ZoomInput (Variables|Misc|Getcamera) InputAxis))

(event EventIAddForcetoShip
  (params (forceToAdd :type Vector :default "0, 0, 0"))
  ;[1 0.8589 0] Player Movement
  ;;[1 1 1] Functions for adding extra forces to ship
  (Physics|AddForce (Variables|Default|GetSM_Boat) forceToAdd "None" true))

(event EventIGetMovingWaterPlane
  (params (mesh :type Static%20Mesh%20Component%20Object%20Reference))
  ;[0 1 0.3243] Wave Data
  ;;[1 1 1] Updates positioning to be used in ship rotations
  (bind _output_get (Variables|Default|SetSM_WaterPlane mesh))
  (Default|SetWaterPlane (Variables|Default|GetBPC_Ship_Buoyancy_Component) _output_get))

(event EventParticleData
  (params (Data :type Array%20of%20Basic%20Particle%20Data%20Structures) (NiagaraSystem :type Niagara%20System%20Object%20Reference) (SimulationPositionOffset :type Vector%20%28by%20ref%29 :default "0, 0, 0"))
  ;[0 1 0.3243] Wave Data
  ;;[1 1 1] Stores wave height data sent over from GPU
  (Variables|/Game/Blueprints/Ship/Ship_Components/BP_Ship_Buoyancy_Component.BP_Ship_Buoyancy_Component_C|SetNiagara%20Data (Variables|Default|GetBPC_Ship_Buoyancy_Component) Data))

(event EventIMoveInputStopped
  ;[1 0.5215 0.127] Camera Controls
  ;;[1 1 1] Resets camera when the boat starts to move again
  (Default|MoveInputStopped (Variables|Misc|Getcamera)))

(event EventIClampMaxSpeed
  ;[1 0.8589 0] Player Movement
  ;;[1 1 1] Clamp Max Speed
  (CallFunction|MaxSpeedClamp))

(event Input|KeyboardEvents|Q
  (params (Key :type Key%20Structure :default "None"))
  ;[0.125 0.002436 0] Combat
  ;;[1 1 1] Initialisation
  (:Pressed
    (Utilities|FlowControl|FlipFlop
      (:A
        ;;;[1 1 1] Enter Combat Mode
        (CallFunction|EventEnterCombatMode)
        (CallFunction|EventInitialiseCrosshair)
        (CallFunction|ICameraMovementToggle false))
      (:B
        ;;;[1 1 1] Exit Combat Mode
        (Rendering|SetVisibility (Variables|Default|GetChild_Crosshair) false false)
        (Rendering|SetVisibility (Variables|Default|GetChild_AttackRange) false false)
        (Utilities|Time|ClearandInvalidateTimerbyHandle (Variables|Combat|GetLocationUpdateTimer))
        (CallFunction|ExitCombatMode)
        (Default|CallAimingActive false) ; Call for music manager to update layering
      ))))

(event Input|MouseEvents|LeftMouseButton
  (params (Key :type Key%20Structure :default "None"))
  ;[0.125 0.002436 0] Combat
  ;;[1 1 1] Updates
  ;;;[1 1 1] Fire Projectiles
  (:Pressed
    (if (Variables|Combat|GetInCombatMode)
      (Development|PrintString "Fired")
      (Class|BPIAttacks|IFireWeapon(Message) (Variables|/Script/Engine.ChildActorComponent|GetChildActor (Variables|Default|GetChild_ProjectileSpawner))))))

(event Input|KeyboardEvents|T
  (params (Key :type Key%20Structure :default "None"))
  ;[1 1 1] Weapon switching
  (:Pressed
    (Utilities|FlowControl|FlipFlop
      (:A
        (CallFunction|SwitchWeapons "NewEnumerator1"))
      (:B
        (CallFunction|SwitchWeapons "NewEnumerator0")))))

(fn ConstructionScript)

(fn SetAttackRangeType
  (for _array_element (Variables|Default|GetCurrentAttackComponents)
    (if (Utilities|Enum|Equal(Enum) (Variables|/Game/Blueprints/Attacks/BPC_Base_Attack.BPC_Base_Attack_C|GetAttackType _array_element) (Variables|Combat|GetSelectedAttackType))
      (return _array_element)))
  (return 0))

(fn MaxSpeedClamp
  (bind _maxspeed (Variables|Misc|GetmaxSpeed))
  ;[1 1 1] Clamps boat speed to the max speed value
  (Utilities|FlowControl|Sequence
    (:then_0
      (bind _returnvalue (Physics|GetPhysicsLinearVelocity (Variables|Default|GetSM_Boat) "None"))
      (bind _output_get (LocalVariables|SetcurrentVelocity _returnvalue))
      (if (> (Class|KismetMathLibrary|VSizeXYSquared _output_get) (Math|Float|Square _maxspeed)) ; Is current speed faster than max speed\n(using squared is faster as it avoids\nsquare rooting)
        (Physics|SetPhysicsLinearVelocity (Variables|Default|GetSM_Boat) (* (LocalVariables|GetcurrentVelocity) (/ _maxspeed (Math|Float|Sqrt (Class|KismetMathLibrary|VSizeXYSquared _output_get)))) false "None")))
    (:then_1
      (bind _returnvalue_2 (Physics|GetPhysicsLinearVelocity (Variables|Default|GetSM_Boat) "None"))
      (Variables|Misc|SetcurrentSpeed (Math|Vector|VectorLengthXY _returnvalue_2)))))

(fn UpdateAttackTypes
  ;[0.125 0.002436 0] s014480m
  (for _array_element (Variables|Default|GetCurrentAttackComponents)
    (Components|DestroyComponent _array_element))
  (for _array_element_2 (Variables|Combat|GetAvailableAttackTypes)
    (if (not (Utilities|Array|ContainsItem (LocalVariables|GetUniqueAttackTypes) _array_element_2))
      (bind _returnvalue (Utilities|GetDataTableRow "/Game/Blueprints/Attacks/DT_AttackTypeToComponent.DT_AttackTypeToComponent" (Utilities|String|StringToName (Utilities|String|EnumtoString _array_element_2)))
        (:then
          (Utilities|Array|Add (LocalVariables|GetUniqueAttackTypes) _array_element_2)
          (bind _returnvalue_2 (Game|AddComponentbyClass (.Value (Utilities|Map|Find (Utilities|Struct|BreakS_AttackType _returnvalue) _array_element_2))))
          (Utilities|Array|Add (Variables|Default|GetCurrentAttackComponents) _returnvalue_2))
        (:RowNotFound
          (Development|PrintString "Attack Type not found in data table" true true "(R=1.000000,G=0.000000,B=0.000000,A=1.000000)"))))))

(fn AddNewAttackType
  (params (AttackType :type E_AttackType%20Enum :default "NewEnumerator0"))
  (Utilities|Array|AddUnique (Variables|Combat|GetAvailableAttackTypes) AttackType)
  (CallFunction|UpdateAttackTypes))

(fn SwitchWeapons
  (params (NewAttackType :type E_AttackType%20Enum :default "NewEnumerator0"))
  (Variables|Combat|SetSelectedAttackType NewAttackType))

(fn GetAttackRangeClass
  (params (attackRangeType :type E_AttackType%20Enum :default "NewEnumerator0"))
  (bind _returnvalue (Utilities|GetDataTableRow "/Game/Blueprints/Attacks/DT_AttackTypeRange.DT_AttackTypeRange" (Utilities|String|StringToName (Utilities|String|EnumtoString attackRangeType)))
    (:then
      (return (.attackRange (Utilities|Struct|BreakS_AttackRange _returnvalue))))
    (:RowNotFound
      (Development|PrintString "[GetAttackRangeClass] COULD NOT FIND RANGE")
      (return "/Game/Blueprints/Attacks/AttackRanges/BP_BaseAttackRange.BP_BaseAttackRange_C"))))

(fn IBossGetLeapPosition
  ;[1 1 1] Sends leap position to the boss
  (return (Transformation|GetWorldLocation (Variables|Default|GetBossLeapLocation))))

(fn IGetShipMesh
  (return (Variables|Default|GetSM_Boat)))

(fn IGetShipVelocity
  (return (Transformation|GetVelocity)))