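; Ship buoyancy component that floats the owning ship's mesh on a water surface using a set of spherical pontoons.
; Niagara wave data supplies a height per pontoon, which with the water plane's Z gives each pontoon's submerged depth and spherical-cap volume.
; That volume becomes a world-up force at the pontoon, applied in mesh-local space.
; Each tick also updates average submersion and messages the owner to clamp max speed.
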(event Custom|Set%20Component%20Wave%20Data
  (params (Wave%20Data :type Array%20of%20Basic%20Particle%20Data%20Structures))
  (Variables|Default|SetNiagara%20Data Wave%20Data)
  (Development|PrintText "Data Set"))

(fn InitiateBuoyancy
  ;[0 0.005816 0.05127] Bouyancy Initialisation
  (bind _shipmesh (Class|BPIShip|IGetShipMesh(Message) (Components|GetOwner)))
  (Variables|Default|SetSM_Boat _shipmesh)
  ;;[1 1 1] Initialises array for pontoon submerged amounts
  (Utilities|Array|Clear (Variables|Default|GetPontoonsSubmergedAmounts))
  (for _array_element (Variables|Default|Getpontoons)
    (Utilities|Array|Add (Variables|Default|GetPontoonsSubmergedAmounts) 1.0))
  (Variables|Default|SetPontoonsAverageSubmergedAmount 1.0)
  (Variables|Default|SetfullPontoonVolume (* (Math|Float|Power (Variables|Default|GetPontoonsRadius) 3.0) (Math|Trig|GetPI) (/ 4.0 3.0))))

(fn TickBuoyancy
  (bind _sm_boat (Variables|Default|GetSM_Boat))
  (bind _pontoons (Variables|Default|Getpontoons))
  (bind _sm_waterplane (Variables|Default|GetSM_WaterPlane))
  ;[0 0.005816 0.05127] Bouyancy
  ;;[1 1 1] Calculate the submerged depth
  (Utilities|FlowControl|Sequence
    (:then_0
      (if (Variables|Default|GetsimulateBuoyancy)
        (for (_array_element _array_index) (Variables|Default|GetNiagara%20Data)
          (if (Utilities|Array|IsValidIndex _pontoons _array_index) ; If pontoon index is a valid position
            (Utilities|IsValid _sm_waterplane
              (:Is%20Valid
                ;;[1 1 1] Calculates submerged volume for each pontoon
                (Utilities|Array|SetArrayElem (Variables|Default|GetPontoonsSubmergedAmounts) _array_index (/ (* (Math|Float|MultiplybyPi 0.333333) (Math|Float|Square (Math|Float|Clamp(Float) (Utilities|Operators|Subtract (.Size (Utilities|Struct|BreakBasicParticleData _array_element)) (* (.Z (Class|KismetMathLibrary|BreakVector3f (Transformation|GetWorldLocation _sm_waterplane))) -1.0) (.Z (Class|KismetMathLibrary|BreakVector3f (Math|Transform|TransformLocation (Transformation|GetWorldTransform _sm_boat) (/ (Utilities|Array|Get(acopy) _pontoons _array_index) (Transformation|GetWorldScale _sm_boat)))))) 0.0 (* (Variables|Default|GetPontoonsRadius) 2.0))) (- (* (Variables|Default|GetPontoonsRadius) 3.0) (Math|Float|Clamp(Float) (Utilities|Operators|Subtract (.Size (Utilities|Struct|BreakBasicParticleData _array_element)) (* (.Z (Class|KismetMathLibrary|BreakVector3f (Transformation|GetWorldLocation _sm_waterplane))) -1.0) (.Z (Class|KismetMathLibrary|BreakVector3f (Math|Transform|TransformLocation (Transformation|GetWorldTransform _sm_boat) (/ (Utilities|Array|Get(acopy) _pontoons _array_index) (Transformation|GetWorldScale _sm_boat)))))) 0.0 (* (Variables|Default|GetPontoonsRadius) 2.0)))) (Variables|Default|GetFullPontoonVolume)))
                (if (> (* (Math|Float|MultiplybyPi 0.333333) (Math|Float|Square (Math|Float|Clamp(Float) (Utilities|Operators|Subtract (.Size (Utilities|Struct|BreakBasicParticleData _array_element)) (* (.Z (Class|KismetMathLibrary|BreakVector3f (Transformation|GetWorldLocation _sm_waterplane))) -1.0) (.Z (Class|KismetMathLibrary|BreakVector3f (Math|Transform|TransformLocation (Transformation|GetWorldTransform _sm_boat) (/ (Utilities|Array|Get(acopy) _pontoons _array_index) (Transformation|GetWorldScale _sm_boat)))))) 0.0 (* (Variables|Default|GetPontoonsRadius) 2.0))) (- (* (Variables|Default|GetPontoonsRadius) 3.0) (Math|Float|Clamp(Float) (Utilities|Operators|Subtract (.Size (Utilities|Struct|BreakBasicParticleData _array_element)) (* (.Z (Class|KismetMathLibrary|BreakVector3f (Transformation|GetWorldLocation _sm_waterplane))) -1.0) (.Z (Class|KismetMathLibrary|BreakVector3f (Math|Transform|TransformLocation (Transformation|GetWorldTransform _sm_boat) (/ (Utilities|Array|Get(acopy) _pontoons _array_index) (Transformation|GetWorldScale _sm_boat)))))) 0.0 (* (Variables|Default|GetPontoonsRadius) 2.0)))) 0.0)
                  (Class|PrimitiveComponent|AddForceatLocationLocal (Variables|Default|GetSM_Boat) (* (* (Math|Float|MultiplybyPi 0.333333) (Math|Float|Square (Math|Float|Clamp(Float) (Utilities|Operators|Subtract (.Size (Utilities|Struct|BreakBasicParticleData _array_element)) (* (.Z (Class|KismetMathLibrary|BreakVector3f (Transformation|GetWorldLocation _sm_waterplane))) -1.0) (.Z (Class|KismetMathLibrary|BreakVector3f (Math|Transform|TransformLocation (Transformation|GetWorldTransform _sm_boat) (/ (Utilities|Array|Get(acopy) _pontoons _array_index) (Transformation|GetWorldScale _sm_boat)))))) 0.0 (* (Variables|Default|GetPontoonsRadius) 2.0))) (- (* (Variables|Default|GetPontoonsRadius) 3.0) (Math|Float|Clamp(Float) (Utilities|Operators|Subtract (.Size (Utilities|Struct|BreakBasicParticleData _array_element)) (* (.Z (Class|KismetMathLibrary|BreakVector3f (Transformation|GetWorldLocation _sm_waterplane))) -1.0) (.Z (Class|KismetMathLibrary|BreakVector3f (Math|Transform|TransformLocation (Transformation|GetWorldTransform _sm_boat) (/ (Utilities|Array|Get(acopy) _pontoons _array_index) (Transformation|GetWorldScale _sm_boat)))))) 0.0 (* (Variables|Default|GetPontoonsRadius) 2.0)))) (Math|Transform|TransformDirection (Transformation|GetWorldTransform (Variables|Default|GetSM_Boat)) (Math|Vector|VectorUp))) (Utilities|Array|Get(acopy) _pontoons _array_index) "None"))))))
        (CallFunction|UpdateAverageSubmerged)))
    (:then_1
      (Class|BPIShip|IClampMaxSpeed(Message) (Components|GetOwner)))))

(fn UpdateAverageSubmerged
  (bind _pontoonssubmergedamounts (Variables|Default|GetPontoonsSubmergedAmounts))
  (for _array_element _pontoonssubmergedamounts
    (LocalVariables|SetWorkingAvg (+ (LocalVariables|GetWorkingAvg) _array_element)))
  (Variables|Default|SetPontoonsAverageSubmergedAmount (/ (LocalVariables|GetWorkingAvg) (Utilities|Array|Length _pontoonssubmergedamounts))))

(fn SetWaterPlane
  (params (SM_WaterPlane :type Static%20Mesh%20Component%20Object%20Reference))
  (Variables|Default|SetSM_WaterPlane SM_WaterPlane))

(fn AddBuoyancyOffsets
  (params (cornerMin :type Float%20%28double-precision%29) (cornerMax :type Float%20%28double-precision%29)))