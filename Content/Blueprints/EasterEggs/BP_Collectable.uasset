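; BP_Collectable is an easter egg pickup that plays a sound, activates an effect and reports to its manager when overlapped.
; On collection it calls OnGet, which only prints text here, hides its mesh, disables trigger collision and destroys itself after a delay.
; GetNewAnimData receives bobbing and spinning values from outside, applying them as Z offset and yaw relative to the transform cached at BeginPlay.
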(event Custom|GetNewAnimData
  (params (Bobbing :type Float%20%28double-precision%29) (Spinning :type Float%20%28double-precision%29))
  (bind _initialrotation (Variables|Default|GetinitialRotation))
  (bind _initialtransform (Variables|Default|GetinitialTransform))
  ;[1 1 1] Animation
  (Transformation|SetActorLocationAndRotation (Math|Vector|MakeVector (.x _initialtransform) (.y _initialtransform) (+ (.z _initialtransform) (* Bobbing (Variables|Default|GetbobbingScale)))) (Math|Rotator|MakeRotator (.roll _initialrotation) (.pitch _initialrotation) (Math|Float|Lerp 0.0 3.6e+02 Spinning))))

(event Custom|Set%20Manager
  (params (Manager :type BP%20Collectable%20Manager%20Object%20Reference))
  (Variables|Default|SetmanagerReference Manager))

(event EventBeginPlay
  ;[1 1 1] Animation
  (Variables|Default|SetinitialTransform (Transformation|GetActorLocation self))
  (Variables|Default|SetinitialRotation (Transformation|GetActorRotation)))

(event Collision|EventActorBeginOverlap
  (params (OtherActor :type Actor%20Object%20Reference))
  (bind _self self)
  (bind _returnvalue (Transformation|GetActorLocation _self))
  ;[1 1 1] Get Collectable
  (Development|PrintText (Utilities|Text|ToText(String) _returnvalue))
  (if true
    (Audio|PlaySoundatLocation (Variables|Default|GetsoundCue) _returnvalue "0, 0, 0" 1.0 1.0 0.0 "/Game/Sounds/SA_Sparkle.SA_Sparkle" 0 0 0))
  (CallFunction|OnGet)
  (Components|Activation|Activate (Variables|Default|GetNS_VFX) false)
  (Default|CollectableCollected (Variables|Default|GetmanagerReference) self)
  (Rendering|SetVisibility (Variables|Default|GetSM_Collectible) false false)
  (Collision|SetCollisionEnabled (Variables|Default|GetSphCol_TriggerArea) "NoCollision")
  (Utilities|FlowControl|Delay (Variables|Default|GetkillDelayOnGet))
  (Actor|DestroyActor))

(fn ConstructionScript)

(fn OnGet
  (Development|PrintText "Get Collectable"))