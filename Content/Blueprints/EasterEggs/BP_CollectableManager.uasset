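; BP_CollectableManager tracks the easter egg collectables in the level and animates them from one central actor.
; On BeginPlay it finds all actors of the configured class, registers itself as their manager and initialises the collected and remaining counts.
; A single Timeline feeds bobbing and rotation values only to collectables within a maximum distance of the player.
; Collection events remove the item from the active list and update both counts.
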(event Custom|CollectableCollected
  (params (Collectible :type BP%20Collectable%20Object%20Reference))
  (Utilities|Array|RemoveItem (Variables|Default|GetactiveCollectables) Collectible)
  (Variables|Default|SetcollectedCollectablesNum (+ (Variables|Default|GetcollectedCollectablesNum) 1))
  (Variables|Default|SettotalCollectablesNum (- (Variables|Default|GettotalCollectablesNum) 1)))

(event EventBeginPlay
  (bind _outactors (Actor|GetAllActorsOfClass (Variables|Default|GetclassToSearch)))
  (bind _output_get (Variables|Default|SetactiveCollectables _outactors))
  (for _array_element _output_get
    (Default|SetManager _array_element self))
  (Variables|Default|SetcollectedCollectablesNum 0)
  (Variables|Default|SettotalCollectablesNum (Utilities|Array|Length (Variables|Default|GetactiveCollectables)))
  (bind (_direction _bobbing _rotation) (Timeline|Timeline PlayFromStart)
    (:Update
      (for _array_element_2 (Variables|Default|GetactiveCollectables)
        (if (<= (Math|Vector|Distance(Vector) (Transformation|GetActorLocation (Game|Player|GetPlayerPawn 0)) (Transformation|GetActorLocation _array_element_2)) (Variables|Default|GetmaxDistanceToUpdate))
          (Default|GetNewAnimData _array_element_2 _bobbing _rotation))))))

(fn ConstructionScript)