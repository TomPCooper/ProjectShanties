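; BP_Water1 is a water plane actor that follows the player's ship horizontally.
; On BeginPlay it finds the Pawn_ShipNew actor, stores it as Boat and passes its static mesh to it through the IGetMovingWaterPlaneMessage interface call.
; Every Tick it moves to the boat's X and Y while keeping its own Z, so the surface stays centered under the ship at a constant height.
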(event EventTick
  (params (DeltaSeconds :type Float%20%28single-precision%29))
  (bind _boat (Variables|Default|GetBoat))
  (bind _returnvalue (Transformation|GetActorLocation _boat))
  (bind (_x _y) (Class|KismetMathLibrary|BreakVector3f _returnvalue))
  (Transformation|SetActorLocation (Math|Vector|MakeVector _x _y (.Z (Class|KismetMathLibrary|BreakVector3f (Transformation|GetActorLocation)))) false false))

(event EventBeginPlay
  (bind _returnvalue (Actor|GetActorOfClass "/Game/Blueprints/t014172k/Pawn_ShipNew.Pawn_ShipNew_C"))
  (bind _output_get (Variables|Default|SetBoat _returnvalue))
  (Class|BPIShip|IGetMovingWaterPlane(Message) _output_get (Variables|Default|GetStaticMesh)))

(fn ConstructionScript)