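; A water current volume that pushes overlapping ships along a set direction and changes their max speed while inside.
; Overlap events on the box filter for BPI_Ship actors, storing a single ship reference and applying or resetting the speed multiplier through interface messages.
; A looping timer applies force along the CurrentDirection forward vector until the ship exits.
; The construction script sizes the box and sets the current's yaw from variables.
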(event OnComponentBeginOverlap(CollisionVolume)
  (params (OverlappedComponent :type Primitive%20Component%20Object%20Reference) (OtherActor :type Actor%20Object%20Reference) (OtherComp :type Primitive%20Component%20Object%20Reference) (OtherBodyIndex :type Integer) (bFromSweep :type Boolean) (SweepResult :type Hit%20Result%20Structure%20%28by%20ref%29))
  (if (Utilities|DoesObjectImplementInterface OtherActor "/Game/Blueprints/Ship/BPI_Ship.BPI_Ship_C")
    (bind _output_get (Variables|Default|SetShipRef OtherActor))
    (Class|BPIShip|IAdjustMaxSpeed(Message) _output_get false (Variables|Default|GetShipMaxSpeedMultiplier))
    (CallFunction|StartCurrentFlow)))

(event OnComponentEndOverlap(CollisionVolume)
  (params (OverlappedComponent :type Primitive%20Component%20Object%20Reference) (OtherActor :type Actor%20Object%20Reference) (OtherComp :type Primitive%20Component%20Object%20Reference) (OtherBodyIndex :type Integer))
  (if (Utilities|DoesObjectImplementInterface OtherActor "/Game/Blueprints/Ship/BPI_Ship.BPI_Ship_C")
    (CallFunction|StopCurrentFlow)))

(event Custom|StartCurrentFlow
  (bind _returnvalue (Utilities|Time|SetTimerbyEvent (delegate Custom|DoCurrentFlow) 0.05 true))
  (Variables|Default|SetCurrentFlowTimer _returnvalue))

(event Custom|DoCurrentFlow
  (Utilities|IsValid (Variables|Default|GetShipRef)
    (:Is%20Valid
      (Class|BPIShip|IAddForcetoShip(Message) (Variables|Default|GetShipRef) (* (Math|Vector|GetForwardVector (Variables|Default|GetCurrentDirection)) (Variables|Default|GetCurrentFlowStrength))))))

(event Custom|StopCurrentFlow
  (Class|BPIShip|IAdjustMaxSpeed(Message) (Variables|Default|GetShipRef) true 0.0)
  (Variables|Default|SetShipRef 0)
  (Utilities|Time|ClearandInvalidateTimerbyHandle (Variables|Default|GetCurrentFlowTimer)))

(fn ConstructionScript
  (Components|Box|SetBoxExtent (Variables|Default|GetCollisionVolume) (Variables|Default|GetBoxVolume) true)
  (Transformation|SetWorldRotation (Variables|Default|GetCurrentDirection) (Math|Rotator|MakeRotator 0.0 0.0 (Variables|Default|GetCurrentZRotation)) false false))