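; BP_Water is a water plane actor that follows the player's boat pawn to keep water beneath it.
; On BeginPlay it caches player pawn 0 as Boat and passes its static mesh to it through an interface message.
; Each tick it moves to the boat's X and Y while keeping its own Z, so the water height stays unchanged.
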(event EventTick
  (params (DeltaSeconds :type Float%20%28single-precision%29))
  (bind _boat (Variables|Default|GetBoat))
  (bind _returnvalue (Transformation|GetActorLocation _boat))
  (bind (_x _y) (Class|KismetMathLibrary|BreakVector3f _returnvalue))
  (Utilities|IsValid _boat
    (:Is%20Valid
      (Transformation|SetActorLocation (Math|Vector|MakeVector _x _y (.Z (Class|KismetMathLibrary|BreakVector3f (Transformation|GetActorLocation)))) false false))))

(event EventBeginPlay
  (bind _output_get (Variables|Default|SetBoat (Game|Player|GetPlayerPawn 0)))
  (Utilities|IsValid _output_get
    (:Is%20Valid
      (Class|BPIShip|IGetMovingWaterPlane(Message) _output_get (Variables|Default|GetStaticMesh)))))

(fn ConstructionScript)