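; BP_Foam_Controller_Component is a controller component that serves as the access point to the water foam capture system.
; GetFoamCaptureActor lazily spawns and caches a BP_Foam_Capture_Actor, passing it the owner, noise, capture, simulation and render target settings.
; Wrapper functions forward foam component registration, pause, unpause, capture initiation and attachment calls to that actor, returning false when its validity check fails.
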(fn AddFoamComponent
  (params (Component :type Primitive%20Component%20Object%20Reference))
  (bind _actor (CallFunction|GetFoamCaptureActor))
  (Utilities|IsValid _actor
    (:Is%20Valid
      (Default|AddFoamComponent _actor Component)
      (return true))
    (:Is%20Not%20Valid
      (return false))))

(fn RemoveFoamComponent
  (params (Component :type Primitive%20Component%20Object%20Reference))
  (bind _actor (CallFunction|GetFoamCaptureActor))
  (Utilities|IsValid _actor
    (:Is%20Valid
      (Default|RemoveFoamComponent _actor Component)
      (return true))
    (:Is%20Not%20Valid
      (return false))))

(fn PauseCapture
  (bind _actor (CallFunction|GetFoamCaptureActor))
  (Utilities|IsValid _actor
    (:Is%20Valid
      (bind _paused (Default|PauseCapture _actor))
      (return _paused))
    (:Is%20Not%20Valid
      (return false))))

(fn UnPauseCapture
  (bind _actor (CallFunction|GetFoamCaptureActor))
  (Utilities|IsValid _actor
    (:Is%20Valid
      (bind _unpaused (Default|UnPauseCapture _actor))
      (return _unpaused))
    (:Is%20Not%20Valid
      (return false))))

(fn InitiateFoamCapture
  (bind _actor (CallFunction|GetFoamCaptureActor))
  (Utilities|IsValid _actor
    (:Is%20Valid
      (bind _instantiated (Default|InitiateFoamCapture _actor))
      (return _instantiated))
    (:Is%20Not%20Valid
      (return false))))

(fn SetCaptureAttachment
  (params (Actor :type Actor%20Object%20Reference))
  (bind _actor (CallFunction|GetFoamCaptureActor))
  (Utilities|IsValid 0
    (:Is%20Valid
      (bind _set (Default|SetCaptureAttachment _actor Actor))
      (return _set))
    (:Is%20Not%20Valid
      (return false))))

(fn GetFoamCaptureActor
  (Utilities|IsValid (Variables|Foam|GetCapture%20Actor)
    (:Is%20Valid
      _)
    (:Is%20Not%20Valid
      (bind _returnvalue (Game|SpawnActorfromClass "/Game/Blueprints/Water/Foam/BP_Foam_Capture_Actor.BP_Foam_Capture_Actor_C" (Math|Transform|MakeTransform "0, 0, 0") "Undefined" "MultiplyWithRoot" (Components|GetOwner) (Variables|Noise|GetNoise%20Amount) (Variables|Noise|GetNoise%20Scale) (Variables|Noise|GetNoise%20Speed) (Variables|Noise|GetUpdate%20Rate) (Variables|Noise|GetCapture%20Width) (Variables|Noise|GetThreshold) (Variables|Noise|GetDecay) (Variables|Noise|GetDiffusion) (Variables|Noise|GetFoam%20Render%20Target) 0 0))
      (bind _output_get (Variables|Foam|SetCapture%20Actor _returnvalue))))
  (return _output_get))