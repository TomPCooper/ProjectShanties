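; Actor that renders aiming-range components top-down into a render target for the water materials, following a set actor snapped to the texel grid.
; On each throttled tick it captures its show-only components, briefly raising a material parameter collection flag when range display is on.
; It copies the previous target into a buffer, then composites the new capture over it using elapsed time.
; Capture position, width and threshold are shared through MPC_WaterParameters.
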(event EventTick
  (params (DeltaSeconds :type Float%20%28single-precision%29))
  (Variables|Capture|SetCapture%20Time (+ DeltaSeconds (Variables|Capture|GetCapture%20Time)))
  (AimingRange|UpdateAimingRangeCapture))

(event EventEndPlay
  (params (EndPlayReason :type EEndPlayReason%20Enum :default "Destroyed"))
  (Rendering|ClearRenderTarget2D "/Game/Blueprints/Water/Foam/AimingRT/RT_AimRange.RT_AimRange"))

(fn ConstructionScript)

(fn AddAimingRangeComponent
  (params (Component :type Primitive%20Component%20Object%20Reference))
  (bind _rangecapture (Variables|Default|GetRangeCapture))
  (Utilities|IsValid _rangecapture
    (:Is%20Valid
      (Rendering|SceneCapture|ShowOnlyComponent _rangecapture Component)
      (return true))
    (:Is%20Not%20Valid
      (return false))))

(fn RemoveAimingRangeComponent
  (params (Component :type Primitive%20Component%20Object%20Reference))
  (bind _rangecapture (Variables|Default|GetRangeCapture))
  (Utilities|IsValid _rangecapture
    (:Is%20Valid
      (Class|SceneCaptureComponent|RemoveShowOnlyComponent _rangecapture Component)
      (return true))
    (:Is%20Not%20Valid
      (return false))))

(fn PauseCapture
  (if (not (Variables|Default|GetPaused))
    (Variables|Default|SetPaused true)
    (Actor|Tick|SetActorTickEnabled false)
    (return false)
    (else
      (return false))))

(fn UnPauseCapture
  (if (Variables|Default|GetPaused)
    (Variables|Default|SetPaused false)
    (Actor|Tick|SetActorTickEnabled (Variables|Default|GetInitiated))
    (return true)
    (else
      (return false))))

(fn InitiateAimingRangeCapture
  (bind _rangecapture (Variables|Default|GetRangeCapture))
  (bind _target_render_target (Variables|AimingRange|GetTarget%20Render%20Target))
  (Utilities|IsValid (Variables|AimingRange|GetTarget%20Render%20Target)
    (:Is%20Valid
      (Utilities|IsValid _rangecapture
        (:Is%20Valid
          (Transformation|SetWorldRotation _rangecapture "-90.000000,-90.000000,0.000000" false false) ; Set to Look Down
          (bind _output_get (Variables|/Script/Engine.SceneCaptureComponent2D|SetOrthoWidth (Variables|Default|GetRangeCapture) (Variables|Capture|GetCapture%20Width)))
          (Rendering|Material|SetScalarParameterValue "/Game/Blueprints/t014172k/MPC_WaterParameters.MPC_WaterParameters" "CaptureTargetWidth" _output_get :!class /Script/Engine.KismetMaterialLibrary) ; Forward Capture Width to a Material Parameter Collection
          (Rendering|Material|SetScalarParameterValue "/Game/Blueprints/t014172k/MPC_WaterParameters.MPC_WaterParameters" "AimingRangeCaptureThreshold" (Variables|Default|GetThreshold) :!class /Script/Engine.KismetMaterialLibrary)
          ;[1 1 1] Create Render Target
          (bind _returnvalue (Rendering|CreateRenderTarget2D (Variables|/Script/Engine.TextureRenderTarget2D|GetSizeX _target_render_target) (Variables|/Script/Engine.TextureRenderTarget2D|GetSizeY _target_render_target) (Variables|/Script/Engine.TextureRenderTarget2D|GetRenderTargetFormat _target_render_target)))
          (bind _output_get_2 (Variables|Capture|SetCapture%20Render%20Target _returnvalue))
          (Variables|/Script/Engine.SceneCaptureComponent2D|SetTextureTarget (Variables|Default|GetRangeCapture) _output_get_2)
          (Variables|Capture|SetCapture%20Texel (/ 1.0 (Math|Float|Max(Float) (Math|Conversions|ToFloat(Integer) (Variables|/Script/Engine.TextureRenderTarget2D|GetSizeX _output_get_2)) (Math|Conversions|ToFloat(Integer) (Variables|/Script/Engine.TextureRenderTarget2D|GetSizeY _output_get_2)))))
          (Rendering|ClearRenderTarget2D (Variables|AimingRange|GetTarget%20Render%20Target))
          ;[1 1 1] Start Rendering Aiming Range/Target
          (Actor|Tick|SetActorTickInterval (Variables|Update|GetUpdate%20Rate))
          (Variables|Default|SetInitiated true)
          (if (Variables|Default|GetPaused)
            _
            (else
              (Actor|Tick|SetActorTickEnabled true)))
          (return true))
        (:Is%20Not%20Valid
          _)))
    (:Is%20Not%20Valid
      _))
  (return false))

(fn SetCaptureAttachment
  (params (Actor :type Actor%20Object%20Reference))
  (bind _output_get (Variables|Capture|SetCapture%20Actor Actor))
  (Development|PrintText "Capture Attachment Set - CAP" true true "(R=0.000000,G=1.000000,B=0.000000,A=1.000000)" 5.0)
  (return (Utilities|IsValid _output_get)))

(fn UpdateAimingRangeCapture
  (bind _rangecapture (Variables|Default|GetRangeCapture))
  (bind _capture_actor (Variables|Capture|GetCapture%20Actor))
  (bind _target_render_target (Variables|AimingRange|GetTarget%20Render%20Target))
  (bind _returnvalue (Transformation|GetActorLocation _capture_actor))
  (bind (_x _y _z) (Math|Vector|BreakVector _returnvalue))
  (Utilities|IsValid _rangecapture
    (:Is%20Valid
      (Utilities|FlowControl|Sequence
        (:then_0
          ;[1 1 1] Snap to Grid
          (Utilities|IsValid _capture_actor
            (:Is%20Valid
              (bind _output_get (Variables|Capture|SetCapture%20Location (+ (Class|KismetMathLibrary|VectorSnappedtoGrid (Math|Vector|MakeVector _x _y 0.0) (* (Variables|/Script/Engine.SceneCaptureComponent2D|GetOrthoWidth _rangecapture) (Variables|Capture|GetCapture%20Texel))) (Math|Vector|MakeVector 0.0 0.0 (+ _z 1e+03)))))
              (Transformation|SetActorLocation _output_get false true)
              (Rendering|Material|SetScalarParameterValue "/Game/Blueprints/t014172k/MPC_WaterParameters.MPC_WaterParameters" "CaptureFoamX" (.X (Math|Vector|BreakVector _output_get)) :!class /Script/Engine.KismetMaterialLibrary)
              (Rendering|Material|SetScalarParameterValue "/Game/Blueprints/t014172k/MPC_WaterParameters.MPC_WaterParameters" "CaptureFoamY" (.Y (Math|Vector|BreakVector _output_get)) :!class /Script/Engine.KismetMaterialLibrary))))
        (:then_1
          (if (Variables|Default|GetdisplayRange)
            ;[1 1 1] Force objects to enter a specific state during capture
            (Rendering|Material|SetScalarParameterValue "/Game/Blueprints/t014172k/MPC_WaterParameters.MPC_WaterParameters" "bShowTargetRange" 1.0 :!class /Script/Engine.KismetMaterialLibrary))
          (Rendering|SceneCapture|CaptureScene (Variables|Default|GetRangeCapture) :!class /Script/Engine.SceneCaptureComponent2D)
          (Rendering|Material|SetScalarParameterValue "/Game/Blueprints/t014172k/MPC_WaterParameters.MPC_WaterParameters" "bShowTargetRange" 0.0 :!class /Script/Engine.KismetMaterialLibrary)
          ;[1 1 1] Create Material Used to Copy Foam RT to Buffer
          (Utilities|IsValid (Variables|Default|GetCopy%20MID)
            (:Is%20Valid
              _)
            (:Is%20Not%20Valid
              (bind _returnvalue_2 (Rendering|Material|CreateDynamicMaterialInstance "/Game/Blueprints/Water/Foam/AimingRT/Materials/M_RenderTarget_AimingRange.M_RenderTarget_AimingRange" "None" "None" :!class /Script/Engine.KismetMaterialLibrary))
              (bind _output_get_2 (Variables|Default|SetCopy%20MID _returnvalue_2))
              (Rendering|Material|SetTextureParameterValue _output_get_2 "Texture" (Variables|AimingRange|GetTarget%20Render%20Target))))
          ;[1 1 1] Create Buffer
          (Utilities|IsValid (Variables|AimingRange|GetTarget%20%20Buffer%20Render%20Target)
            (:Is%20Valid
              _)
            (:Is%20Not%20Valid
              (bind _returnvalue_3 (Rendering|CreateRenderTarget2D (Variables|/Script/Engine.TextureRenderTarget2D|GetSizeX _target_render_target) (Variables|/Script/Engine.TextureRenderTarget2D|GetSizeY _target_render_target) (Variables|/Script/Engine.TextureRenderTarget2D|GetRenderTargetFormat _target_render_target)))
              (Variables|AimingRange|SetTarget%20%20Buffer%20Render%20Target _returnvalue_3)))
          ;[1 1 1] Copy to Buffer
          (Rendering|DrawMaterialtoRenderTarget (Variables|AimingRange|GetTarget%20%20Buffer%20Render%20Target) (Variables|Default|GetCopy%20MID))
          ;[1 1 1] Create Material to Composite New Foam and Previous Foam into Foam Render Target
          (Utilities|IsValid (Variables|Default|GetComp%20MID)
            (:Is%20Valid
              _)
            (:Is%20Not%20Valid
              (bind _returnvalue_4 (Rendering|Material|CreateDynamicMaterialInstance "/Game/Blueprints/Water/Foam/AimingRT/Materials/Instances/Mi_RenderTarget_AimingRange_Composite.Mi_RenderTarget_AimingRange_Composite" "None" "None" :!class /Script/Engine.KismetMaterialLibrary))
              (bind _output_get_3 (Variables|Default|SetComp%20MID _returnvalue_4))
              (Rendering|Material|SetTextureParameterValue _output_get_3 "Capture" (Variables|Capture|GetCapture%20Render%20Target))
              (Rendering|Material|SetTextureParameterValue _output_get_3 "Buffer" (Variables|AimingRange|GetTarget%20%20Buffer%20Render%20Target))))
          (Rendering|Material|SetScalarParameterValue (Variables|Default|GetComp%20MID) "DeltaTime" (- (Variables|Capture|GetCapture%20Time) (Variables|Update|GetUpdate%20Timestamp)) :!class /Script/Engine.MaterialInstanceDynamic)
          ;[1 1 1] Render Foam
          (Rendering|DrawMaterialtoRenderTarget (Variables|AimingRange|GetTarget%20Render%20Target) (Variables|Default|GetComp%20MID))
          (Variables|Update|SetUpdate%20Timestamp (Variables|Capture|GetCapture%20Time))
          (return))))
    (:Is%20Not%20Valid
      (Actor|Tick|SetActorTickEnabled false)
      (return))))

(fn IBossGetLeapPosition
  (return "0, 0, 0"))

(fn IGetCamera
  (return 0))

(fn IGetShipMesh
  (return 0))

(fn IGetShipVelocity
  (return "0, 0, 0"))

(fn ISetRangeVisibility
  (params (True :type Boolean))
  (Variables|Default|SetdisplayRange True))