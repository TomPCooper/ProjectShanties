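; Actor component that serves as the control interface for rendering aiming-range components into a render target.
; Its functions add or remove target components, initiate, pause or unpause capture, and set the capture attachment, forwarding each call to a BP_RenderAimingRange_Capture_Actor.
; A shared getter lazily spawns that actor at the origin, owned by the component's owner and configured with its update rate, width, threshold and render target.
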(fn AddAimTargetComponent
  (params (Component :type Primitive%20Component%20Object%20Reference))
  (bind _actor (AimTarget|GetAimTargetCaptureActor))
  (Utilities|IsValid _actor
    (:Is%20Valid
      (Default|AddAimingRangeComponent _actor Component)
      (return true))
    (:Is%20Not%20Valid
      (return false))))

(fn RemoveAimTargetComponent
  (params (Component :type Primitive%20Component%20Object%20Reference))
  (bind _actor (AimTarget|GetAimTargetCaptureActor))
  (Utilities|IsValid _actor
    (:Is%20Valid
      (Default|RemoveAimingRangeComponent _actor Component)
      (return true))
    (:Is%20Not%20Valid
      (return false))))

(fn PauseCapture
  (bind _actor (AimTarget|GetAimTargetCaptureActor))
  (Utilities|IsValid _actor
    (:Is%20Valid
      (bind _paused (Default|PauseCapture _actor))
      (return _paused))
    (:Is%20Not%20Valid
      (return false))))

(fn UnPauseCapture
  (bind _actor (AimTarget|GetAimTargetCaptureActor))
  (Utilities|IsValid _actor
    (:Is%20Valid
      (bind _unpaused (Default|UnPauseCapture _actor))
      (return _unpaused))
    (:Is%20Not%20Valid
      (return false))))

(fn InitiateAimTargetCapture
  (bind _actor (AimTarget|GetAimTargetCaptureActor))
  (Utilities|IsValid _actor
    (:Is%20Valid
      (bind _instantiated (Default|InitiateAimingRangeCapture _actor))
      (return _instantiated))
    (:Is%20Not%20Valid
      (return false))))

(fn SetCaptureAttachment
  (params (Actor :type Actor%20Object%20Reference))
  (bind _actor (AimTarget|GetAimTargetCaptureActor))
  (Utilities|IsValid _actor
    (:Is%20Valid
      (bind _set (Default|SetCaptureAttachment _actor Actor))
      (Development|PrintText "Capture Attachment Set - CTRLR" true true "(R=0.000000,G=0.984000,B=0.005000,A=1.000000)" 5.0)
      (return _set))
    (:Is%20Not%20Valid
      (Development|PrintText "Capture Attachment Not Set - Range CTRLR" true true "(R=1.000000,G=0.000000,B=0.000000,A=1.000000)" 5.0)
      (return false))))

(fn GetAimTargetCaptureActor
  (Utilities|IsValid (Variables|AimTarget|GetCapture%20Actor)
    (:Is%20Valid
      _)
    (:Is%20Not%20Valid
      (bind _returnvalue (Game|SpawnActorfromClass "/Game/Blueprints/Water/Foam/AimingRT/BP_RenderAimingRange_Capture_Actor.BP_RenderAimingRange_Capture_Actor_C" (Math|Transform|MakeTransform "0, 0, 0") "Undefined" "MultiplyWithRoot" (Components|GetOwner) (Variables|Default|GetUpdate%20Rate) (Variables|Default|GetCapture%20Width) (Variables|Default|GetThreshold) (Variables|Default|GetAimTarget%20Render%20Target) 0 0))
      (bind _output_get (Variables|AimTarget|SetCapture%20Actor _returnvalue))))
  (return _output_get))