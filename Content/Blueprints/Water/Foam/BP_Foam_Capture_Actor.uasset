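; Actor that generates a persistent foam render target around a followed actor wherever registered components intersect water.
; An orthographic top-down capture of show-only components snaps to the texel grid and publishes its position and width to MPC_WaterParameters.
; A bCaptureFoam flag toggles during each capture so materials can test water intersection.
; Each tick, previous foam is copied to a buffer, then composited with the new capture using diffusion, decay and optional noise.
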(event EventTick
  (params (DeltaSeconds :type Float%20%28single-precision%29))
  (Variables|Capture|SetCapture%20Time (+ DeltaSeconds (Variables|Capture|GetCapture%20Time)))
  (CallFunction|UpdateFoamCapture))

(event EventEndPlay
  (params (EndPlayReason :type EEndPlayReason%20Enum :default "Destroyed"))
  (Rendering|ClearRenderTarget2D "/Game/Blueprints/Water/Foam/RT_Foam.RT_Foam"))

(fn ConstructionScript)

(fn AddFoamComponent
  (params (Component :type Primitive%20Component%20Object%20Reference))
  (bind _foamcapture (Variables|Default|GetFoamCapture))
  (Utilities|IsValid _foamcapture
    (:Is%20Valid
      (Rendering|SceneCapture|ShowOnlyComponent _foamcapture Component)
      (return true))
    (:Is%20Not%20Valid
      (return false))))

(fn RemoveFoamComponent
  (params (Component :type Primitive%20Component%20Object%20Reference))
  (bind _foamcapture (Variables|Default|GetFoamCapture))
  (Utilities|IsValid _foamcapture
    (:Is%20Valid
      (Class|SceneCaptureComponent|RemoveShowOnlyComponent _foamcapture Component)
      (return true))
    (:Is%20Not%20Valid
      (return false))))

(fn PauseCapture
  (if (not (Variables|Default|GetPaused))
    (Variables|Default|SetPaused true)
    (Actor|Tick|SetActorTickEnabled false)
    (return false)
    (else
      (return false))))

(fn UnPauseCapture
  (if (Variables|Default|GetPaused)
    (Variables|Default|SetPaused false)
    (Actor|Tick|SetActorTickEnabled (Variables|Default|GetInitiated))
    (return true)
    (else
      (return false))))

(fn InitiateFoamCapture
  (bind _foamcapture (Variables|Default|GetFoamCapture))
  (bind _foam_render_target (Variables|Foam|GetFoam%20Render%20Target))
  (Utilities|IsValid (Variables|Foam|GetFoam%20Render%20Target)
    (:Is%20Valid
      (Utilities|IsValid _foamcapture
        (:Is%20Valid
          (Transformation|SetWorldRotation _foamcapture "-90.000000,-90.000000,0.000000" false false) ; Set to Look Down
          (bind _output_get (Variables|/Script/Engine.SceneCaptureComponent2D|SetOrthoWidth (Variables|Default|GetFoamCapture) (Variables|Capture|GetCapture%20Width)))
          (Rendering|Material|SetScalarParameterValue "/Game/Blueprints/t014172k/MPC_WaterParameters.MPC_WaterParameters" "CaptureFoamWidth" _output_get :!class /Script/Engine.KismetMaterialLibrary) ; Forward Capture Width to a Material Parameter Collection
          (Rendering|Material|SetScalarParameterValue "/Game/Blueprints/t014172k/MPC_WaterParameters.MPC_WaterParameters" "CaptureThreshold" (Variables|Noise|GetThreshold) :!class /Script/Engine.KismetMaterialLibrary)
          ;[1 1 1] Create Render Target
          (bind _returnvalue (Rendering|CreateRenderTarget2D (Variables|/Script/Engine.TextureRenderTarget2D|GetSizeX _foam_render_target) (Variables|/Script/Engine.TextureRenderTarget2D|GetSizeY _foam_render_target) (Variables|/Script/Engine.TextureRenderTarget2D|GetRenderTargetFormat _foam_render_target)))
          (bind _output_get_2 (Variables|Capture|SetCapture%20Render%20Target _returnvalue))
          (Variables|/Script/Engine.SceneCaptureComponent2D|SetTextureTarget (Variables|Default|GetFoamCapture) _output_get_2)
          (Variables|Capture|SetCapture%20Texel (/ 1.0 (Math|Float|Max(Float) (Math|Conversions|ToFloat(Integer) (Variables|/Script/Engine.TextureRenderTarget2D|GetSizeX _output_get_2)) (Math|Conversions|ToFloat(Integer) (Variables|/Script/Engine.TextureRenderTarget2D|GetSizeY _output_get_2)))))
          (Rendering|ClearRenderTarget2D (Variables|Foam|GetFoam%20Render%20Target))
          ;[1 1 1] Start Rendering Foam
          (Actor|Tick|SetActorTickInterval (Variables|Update|GetUpdate%20Rate))
          (Variables|Default|SetInitiated true)
          (if (Variables|Default|GetPaused)
            _
            (else
              (Actor|Tick|SetActorTickEnabled true)))
          (return true))
        (:Is%20Not%20Valid
          _)))
    (:Is%20Not%20Valid
      _))
  (return false))

(fn SetCaptureAttachment
  (params (Actor :type Actor%20Object%20Reference))
  (bind _output_get (Variables|Capture|SetCapture%20Actor Actor))
  (Development|PrintText "Capture Attachment Set - CAP" true true "(R=0.000000,G=1.000000,B=0.000000,A=1.000000)" 5.0)
  (return (Utilities|IsValid _output_get)))

(fn UpdateFoamCapture
  (bind _foamcapture (Variables|Default|GetFoamCapture))
  (bind _capture_actor (Variables|Capture|GetCapture%20Actor))
  (bind _foam_render_target (Variables|Foam|GetFoam%20Render%20Target))
  (bind _returnvalue (Transformation|GetActorLocation _capture_actor))
  (bind (_x _y _z) (Math|Vector|BreakVector _returnvalue))
  (Utilities|IsValid _foamcapture
    (:Is%20Valid
      (Utilities|FlowControl|Sequence
        (:then_0
          ;[1 1 1] Snap to Grid
          (Utilities|IsValid _capture_actor
            (:Is%20Valid
              (bind _output_get (Variables|Capture|SetCapture%20Location (+ (Class|KismetMathLibrary|VectorSnappedtoGrid (Math|Vector|MakeVector _x _y 0.0) (* (Variables|/Script/Engine.SceneCaptureComponent2D|GetOrthoWidth _foamcapture) (Variables|Capture|GetCapture%20Texel))) (Math|Vector|MakeVector 0.0 0.0 (+ _z 1e+03)))))
              (Transformation|SetActorLocation _output_get false true)
              (Rendering|Material|SetScalarParameterValue "/Game/Blueprints/t014172k/MPC_WaterParameters.MPC_WaterParameters" "CaptureFoamX" (.X (Math|Vector|BreakVector _output_get)) :!class /Script/Engine.KismetMaterialLibrary)
              (Rendering|Material|SetScalarParameterValue "/Game/Blueprints/t014172k/MPC_WaterParameters.MPC_WaterParameters" "CaptureFoamY" (.Y (Math|Vector|BreakVector _output_get)) :!class /Script/Engine.KismetMaterialLibrary))))
        (:then_1
          ;[1 1 1] Force objects to enter a specific state during capture to check for water intersection
          (Rendering|Material|SetScalarParameterValue "/Game/Blueprints/t014172k/MPC_WaterParameters.MPC_WaterParameters" "bCaptureFoam" 1.0 :!class /Script/Engine.KismetMaterialLibrary)
          (Rendering|SceneCapture|CaptureScene (Variables|Default|GetFoamCapture) :!class /Script/Engine.SceneCaptureComponent2D)
          (Rendering|Material|SetScalarParameterValue "/Game/Blueprints/t014172k/MPC_WaterParameters.MPC_WaterParameters" "bCaptureFoam" 0.0 :!class /Script/Engine.KismetMaterialLibrary)
          ;[1 1 1] Create Material Used to Copy Foam RT to Buffer
          (Utilities|IsValid (Variables|Default|GetCopy%20MID)
            (:Is%20Valid
              _)
            (:Is%20Not%20Valid
              (bind _returnvalue_2 (Rendering|Material|CreateDynamicMaterialInstance "/Game/Blueprints/Water/Foam/Materials/M_RenderTarget_Foam.M_RenderTarget_Foam" "None" "None" :!class /Script/Engine.KismetMaterialLibrary))
              (bind _output_get_2 (Variables|Default|SetCopy%20MID _returnvalue_2))
              (Rendering|Material|SetTextureParameterValue _output_get_2 "Texture" (Variables|Foam|GetFoam%20Render%20Target))))
          ;[1 1 1] Create Foam Buffer
          (Utilities|IsValid (Variables|Foam|GetFoam%20Buffer%20Render%20Target)
            (:Is%20Valid
              _)
            (:Is%20Not%20Valid
              (bind _returnvalue_3 (Rendering|CreateRenderTarget2D (Variables|/Script/Engine.TextureRenderTarget2D|GetSizeX _foam_render_target) (Variables|/Script/Engine.TextureRenderTarget2D|GetSizeY _foam_render_target) (Variables|/Script/Engine.TextureRenderTarget2D|GetRenderTargetFormat _foam_render_target)))
              (Variables|Foam|SetFoam%20Buffer%20Render%20Target _returnvalue_3)))
          ;[1 1 1] Copy Foam to Buffer
          (Rendering|DrawMaterialtoRenderTarget (Variables|Foam|GetFoam%20Buffer%20Render%20Target) (Variables|Default|GetCopy%20MID))
          ;[1 1 1] Create Material to Composite New Foam and Previous Foam into Foam Render Target
          (Utilities|IsValid (Variables|Default|GetComp%20MID)
            (:Is%20Valid
              _)
            (:Is%20Not%20Valid
              (bind _returnvalue_4 (Rendering|Material|CreateDynamicMaterialInstance (select (> (Variables|Noise|GetNoise%20Amount) 0.0) "/Game/Blueprints/Water/Foam/Materials/Instances/MI_RenderTarget_Foam_Composite_Noise.MI_RenderTarget_Foam_Composite_Noise" "/Game/Blueprints/Water/Foam/Materials/Instances/Mi_RenderTarget_Foam_Composite.Mi_RenderTarget_Foam_Composite") "None" "None" :!class /Script/Engine.KismetMaterialLibrary))
              (bind _output_get_3 (Variables|Default|SetComp%20MID _returnvalue_4))
              (Rendering|Material|SetTextureParameterValue _output_get_3 "Capture" (Variables|Capture|GetCapture%20Render%20Target))
              (Rendering|Material|SetTextureParameterValue _output_get_3 "Buffer" (Variables|Foam|GetFoam%20Buffer%20Render%20Target))
              (Rendering|Material|SetScalarParameterValue _output_get_3 "Diffusion" (Math|Conversions|ToFloat(Integer) (Variables|Noise|GetDiffusion)) :!class /Script/Engine.MaterialInstanceDynamic)
              (Rendering|Material|SetScalarParameterValue _output_get_3 "Decay" (Variables|Noise|GetDecay) :!class /Script/Engine.MaterialInstanceDynamic)
              (if (<= (Variables|Noise|GetNoise%20Amount) 0.0)
                _
                (else
                  (Rendering|Material|SetScalarParameterValue (Variables|Default|GetComp%20MID) "NoiseSpeed" (Variables|Noise|GetNoise%20Speed) :!class /Script/Engine.MaterialInstanceDynamic)
                  (Rendering|Material|SetScalarParameterValue (Variables|Default|GetComp%20MID) "NoiseAmount" (Variables|Noise|GetNoise%20Amount) :!class /Script/Engine.MaterialInstanceDynamic)
                  (Rendering|Material|SetScalarParameterValue (Variables|Default|GetComp%20MID) "NoiseScale" (Variables|Noise|GetNoise%20Scale) :!class /Script/Engine.MaterialInstanceDynamic)))))
          (Rendering|Material|SetScalarParameterValue (Variables|Default|GetComp%20MID) "DeltaTime" (- (Variables|Capture|GetCapture%20Time) (Variables|Update|GetUpdate%20Timestamp)) :!class /Script/Engine.MaterialInstanceDynamic)
          ;[1 1 1] Render Foam
          (Rendering|DrawMaterialtoRenderTarget (Variables|Foam|GetFoam%20Render%20Target) (Variables|Default|GetComp%20MID))
          (Variables|Update|SetUpdate%20Timestamp (Variables|Capture|GetCapture%20Time))
          (return))))
    (:Is%20Not%20Valid
      (Actor|Tick|SetActorTickEnabled false)
      (return))))