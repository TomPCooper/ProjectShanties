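; Buoyancy component that floats its owning actor on the water surface of the first BP_FloatVolume found in the level.
; Each tick, boxes tagged FloatSubmerged act as pontoons, with submerged fraction measured against the volume's top.
; Each pushes the first FloatPhysics-tagged primitive upward at its location, scaled by fluid density, extent product and gravity.
; Only height matters: overlap checks are disconnected and ForceSubmergedCheck is empty.
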(event Custom|ForceSubmergedCheck)

(event EventBeginPlay
  (bind _returnvalue (Actor|GetActorOfClass "/Game/Blueprints/Water/WaterFloat/BP_FloatVolume.BP_FloatVolume_C"))
  (Variables|Default|SetFloatVolume (Variables|/Game/Blueprints/Water/WaterFloat/BP_FloatVolume.BP_FloatVolume_C|GetFloatVolBox _returnvalue)))

(event EventTick
  (params (DeltaSeconds :type Float%20%28single-precision%29))
  (CallFunction|IApplyBuoyantForce))

(event EventIApplyBuoyantForce
  (bind _returnvalue (Components|GetOwner))
  (bind _returnvalue_2 (Components|GetOwner))
  (bind _floatvolume (Variables|Default|GetFloatVolume))
  (bind (_origin _boxextent) (Collision|GetComponentBounds _floatvolume))
  (bind _returnvalue_3 (Actor|GetComponentsbyTag _returnvalue_2 "/Script/Engine.BoxComponent" "FloatSubmerged"))
  (bind _returnvalue_4 (Actor|GetComponentsbyTag _returnvalue "/Script/Engine.PrimitiveComponent" "FloatPhysics"))
  (bind _output (Utilities|Array|Get(acopy) _returnvalue_4))
  ;[1 1 1] Calculate buoyancy
  (if (Utilities|Array|IsNotEmpty _returnvalue_3)
    (for _array_element _returnvalue_3
      (Utilities|IsValid _array_element
        (:Is%20Valid
          (Utilities|IsValid _output
            (:Is%20Valid
              (Class|PrimitiveComponent|AddForceatLocation _output (* (Variables|Default|GetFluidDensity) (* (Math|Float|Clamp(Float) (/ (- (.z (+ _origin _boxextent)) (- (.z (Transformation|GetWorldLocation _array_element)) (.z (Components|Box|GetScaledBoxExtent _array_element)))) (* (.z (Components|Box|GetScaledBoxExtent _array_element)) 2.0))) (* (.x (Components|Box|GetScaledBoxExtent _array_element)) (.y (Components|Box|GetScaledBoxExtent _array_element)) (.z (Components|Box|GetScaledBoxExtent _array_element)))) (Math|Vector|MakeVector 0.0 0.0 981.0)) (Transformation|GetWorldLocation _array_element) "None"))))))))