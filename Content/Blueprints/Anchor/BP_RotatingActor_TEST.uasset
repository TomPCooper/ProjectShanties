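; BP_RotatingActor_TEST is a test actor that orbits a point horizontally at a set radius.
; Each Tick, while rotation is enabled, it accumulates an angle from speed, delta time and direction.
; RotateActorAroundPoint rotates a radius vector about Z from the starting angle and positions the actor around the target actor, or its BeginPlay location if none is valid.
; An optional debug line connects the centre to the actor.
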(event EventBeginPlay
  (Variables|Default|SetInitialLocation (Transformation|GetActorLocation)))

(event EventTick
  (params (DeltaSeconds :type Float%20%28single-precision%29))
  (if (Variables|Default|GetCanRotate)
    (Variables|Default|SetCurrentRotation (+ (Variables|Default|GetCurrentRotation) (* (* DeltaSeconds (Variables|Default|GetRotationSpeed)) (Math|Float|SelectFloat 1.0 -1.0 (Variables|Default|GetClockwise)))))
    (bind _location (CallFunction|RotateActorAroundPoint (Variables|Default|GetTargetActor) (Variables|Default|GetInitialLocation) (Variables|Default|GetRadius) (Variables|Default|GetStartingAngle) (Variables|Default|GetCurrentRotation)))
    (if (Variables|Default|GetDrawDebug)
      (Rendering|Debug|DrawDebugLine _location (Transformation|GetActorLocation) (Variables|Default|GetTraceColour) 1.0 2.0))))

(fn ConstructionScript)

(fn RotateActorAroundPoint
  (params (TargetActor :type Actor%20Object%20Reference) (TargetLocation :type Vector) (Radius :type Float%20%28double-precision%29) (Angle :type Float%20%28double-precision%29) (RotationRate :type Float%20%28double-precision%29))
  (Utilities|FlowControl|Sequence
    (:then_0
      (LocalVariables|SetLTargetActor TargetActor)
      (LocalVariables|SetLLocation TargetLocation)
      (LocalVariables|SetLRadius Radius)
      (LocalVariables|SetLAngle Angle)
      (LocalVariables|SetLRotationRate RotationRate))
    (:then_1
      (Utilities|IsValid (LocalVariables|GetLTargetActor)
        (:Is%20Valid
          (LocalVariables|SetLLocation (Transformation|GetActorLocation (LocalVariables|GetLTargetActor))))
        (:Is%20Not%20Valid
          _))
      (Transformation|SetActorLocation (+ (LocalVariables|GetLLocation) (Math|Vector|RotateVectorAroundAxis (Math|Vector|MakeVector (LocalVariables|GetLRadius) 0.0 0.0) (+ (LocalVariables|GetLAngle) (LocalVariables|GetLRotationRate)) "0.000000,0.000000,1.000000")) false false)
      (return (LocalVariables|GetLLocation)))))