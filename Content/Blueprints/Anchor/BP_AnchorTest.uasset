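; Test anchor actor that simulates physics on BeginPlay, then can be stopped and constrained to a ship for drifting.
; StopAnchor disables physics, resets rotation, constrains the ship mesh at AttachPoint and sets spin direction from whether that point is the right-hand one.
; A Tick-fed gate, open while move input Y is non-zero, yaws the anchor by DriftSpeed in that direction.
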(event Custom|StopAnchor
  (Physics|SetSimulatePhysics (Variables|Default|GetAnchor) false)
  (Transformation|SetRelativeRotation (Variables|Default|GetAnchor) "0, 0, 0" false false)
  (bind _shipmesh (Class|BPIShip|IGetShipMesh(Message) (Variables|Default|GetShipRef)))
  (Variables|Default|SetShipMesh _shipmesh)
  (Class|PhysicsConstraintComponent|SetConstrainedComponents (Variables|Default|GetPhysicsConstraint) 0 "None" (Variables|Default|GetShipMesh) (Variables|Default|GetAttachPoint))
  (Variables|Default|SetClockwise? (== (Variables|Default|GetAttachPoint) "AnchorPointRight")))

(event EventTick
  (params (DeltaSeconds :type Float%20%28single-precision%29))
  (bind _driftspeed (Variables|Default|GetDriftSpeed))
  (Utilities|FlowControl|Sequence
    (:then_0
      (Utilities|FlowControl|Gate true :!label _label
        (:Exit
          (Transformation|AddRelativeRotation (Variables|Default|GetAnchor) (Math|Rotator|MakeRotator 0.0 0.0 (Math|Float|SelectFloat _driftspeed (* _driftspeed -1.0) (Variables|Default|GetClockwise?))) false false))))
    (:then_1
      (if (!= (.y (Input|EnhancedActionValues|GetIA_Move)) 0.0)
        (goto _label Open)
        (else
          (goto _label Close))))))

(event EventAllowDrift
  (bind _driftspeed (Variables|Default|GetDriftSpeed))
  (Utilities|FlowControl|Gate true) ; enters at Open
)

(event EventBeginPlay
  (Physics|SetSimulatePhysics (Variables|Default|GetAnchor) true)
  (Utilities|Time|SetTimerbyEvent (EventDispatchers|CreateEvent :!event Custom|StopAnchor) 1.0))

(fn ConstructionScript)

(fn RotateAnchor
  (Transformation|SetWorldRotation (Variables|Default|GetAnchor) (Math|Rotator|MakeRotator 0.0 0.0 (+ (.yaw (Transformation|GetWorldRotation (Variables|Default|GetAnchor))) 1.0)) false false))