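; Harpoon projectile that sticks to what it hits and pulls it toward its owner, trailing a cable attached to the owner's harpoon socket.
; On overlap it stops, attaches to the hit actor, caches that actor's mesh via interface and starts two timers, apparently for timed removal and repeated pulling.
; Each pull applies the normalized direction to the owner as a local-space offset, scaled by pull speed and frame delta.
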(event OnComponentBeginOverlap(Collider)
  (params (OverlappedComponent :type Primitive%20Component%20Object%20Reference) (OtherActor :type Actor%20Object%20Reference) (OtherComp :type Primitive%20Component%20Object%20Reference) (OtherBodyIndex :type Integer) (bFromSweep :type Boolean) (SweepResult :type Hit%20Result%20Structure%20%28by%20ref%29))
  ;[1 1 1] Activate harpoon once hit
  (Components|Movement|StopMovementImmediately (Variables|Default|GetProjectileMovement))
  (bind _output_get (Variables|Default|SetEnemyHit OtherActor))
  (Transformation|AttachActorToActor _output_get "None" "SnapToTarget" "KeepRelative" "KeepRelative" true)
  (bind _enemymesh (Class|BPIHarpoon|IGetMeshReference(Message) _output_get))
  (Variables|Default|SetEnemy%20Mesh _enemymesh)
  (Utilities|Time|SetTimerbyEvent (EventDispatchers|CreateEvent :!event Custom|RemoveHarpoon) (Variables|Default|GetHarpoonAttachTime))
  (Utilities|Time|SetTimerbyEvent (EventDispatchers|CreateEvent :!event Custom|PullEnemy) 0.1 true))

(event Custom|RemoveHarpoon
  ;[1 1 1] destroy actor
  (Actor|DestroyActor))

(event Custom|PullEnemy
  (bind _enemyhit (Variables|Default|GetEnemyHit))
  ;[1 1 1] Pull enemy towards player
  (Utilities|IsValid _enemyhit
    (:Is%20Valid
      (Transformation|AddActorLocalOffset _enemyhit (* (Math|Vector|Normalize (- (Transformation|GetActorLocation (Variables|Default|GetHarpoonOwner)) (Transformation|GetActorLocation (Variables|Default|GetEnemyHit)))) (Variables|Default|GetPullSpeed) (Utilities|Time|GetWorldDeltaSeconds)) false false))))

(event EventBeginPlay
  ;[1 1 1] Init cable
  (|CallParentFunction)
  (Class|CableComponent|SetAttachEndto (Variables|Default|GetCable) (Variables|Default|GetHarpoonOwner) "None" "HarpoonAttachPoint"))

(fn ConstructionScript
  (|CallParentFunction))