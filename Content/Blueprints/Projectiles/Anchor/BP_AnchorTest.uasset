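; BP_AnchorTest is a test anchor projectile that starts as a physics-simulated body and can be halted and linked to a ship.
; BeginPlay enables physics on the anchor and starts a one-shot timer, presumably for StopAnchor.
; StopAnchor disables physics, fetches the ship mesh through an interface message and constrains the anchor to its AnchorPoint bone.
; It also sets a fast yaw rotation on the RotatingMovement component.
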(event Custom|StopAnchor
  (Physics|SetSimulatePhysics (Variables|Default|GetAnchor) false)
  (bind _shipmesh (Class|BPIShip|IGetShipMesh(Message) (Variables|Default|GetShipRef)))
  (Variables|Default|SetShipMesh _shipmesh)
  (Class|PhysicsConstraintComponent|SetConstrainedComponents (Variables|Default|GetPhysicsConstraint) (Variables|Default|GetAnchor) "None" (Variables|Default|GetShipMesh) "AnchorPoint")
  (Variables|/Script/Engine.RotatingMovementComponent|SetRotationRate (Variables|Default|GetRotatingMovement) "0.000000,720.000000,0.000000"))

(event EventBeginPlay
  (Physics|SetSimulatePhysics (Variables|Default|GetAnchor) true)
  (Utilities|Time|SetTimerbyEvent (EventDispatchers|CreateEvent :!event Custom|StopAnchor) 1.0))

(fn ConstructionScript)