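; Child weapon Blueprint that spawns a projectile when its IFireWeapon event fires.
; It resolves the projectile class by looking up CurrentProjectileType in the EnumToClass map of the DT_ProjectilesConversion "Projectile" row.
; The projectile spawns at the ProjectileSpawnReference transform, receiving this spawner's owner and AimPos.
; Debug strings report each shot and a missing table row.
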(event EventIFireWeapon
  (Development|PrintString "Fired in child")
  (bind _returnvalue (Utilities|GetDataTableRow "/Game/Blueprints/Projectiles/DT_ProjectilesConversion.DT_ProjectilesConversion" "Projectile")
    (:then
      (Game|SpawnActorfromClass (.Value (Utilities|Map|Find (Utilities|Struct|BreakStruct_ProjectileClassToEnum _returnvalue) (Variables|Default|GetCurrentProjectileType))) (Transformation|GetWorldTransform (Variables|Default|GetProjectileSpawnReference)) "Undefined" "MultiplyWithRoot" (Components|GetOwner) (Variables|Default|GetAimPos) 0))
    (:RowNotFound
      (Development|PrintString "Lookup table could not find a projectile class with the requested enum value"))))

(fn ConstructionScript)