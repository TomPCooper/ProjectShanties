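; BP_Projectile is a projectile actor that damages actors with a health component on overlap.
; Its collider ignores the owner and components tagged IgnoreProjectiles, then applies Damage through IDamage on BPC_Health and destroys the projectile.
; BeginPlay sets the lifespan, so projectiles that damage nothing still expire.
; For homing projectiles, the construction script sets AimPos as the movement's homing target, sets the lifespan and detaches the actor.
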(event OnComponentBeginOverlap(Collider)
  (params (OverlappedComponent :type Primitive%20Component%20Object%20Reference) (OtherActor :type Actor%20Object%20Reference) (OtherComp :type Primitive%20Component%20Object%20Reference) (OtherBodyIndex :type Integer) (bFromSweep :type Boolean) (SweepResult :type Hit%20Result%20Structure%20%28by%20ref%29))
  (bind _returnvalue (Actor|GetComponentbyClass OtherActor "/Game/Blueprints/Health/BPC_Health.BPC_Health_C"))
  (if (!= OtherActor (Components|GetOwner))
    (if (not (Components|ComponentHasTag OtherComp "IgnoreProjectiles"))
      (Utilities|IsValid _returnvalue
        (:Is%20Valid
          (Default|IDamage _returnvalue (Variables|Default|Getdamage))
          (Actor|DestroyActor)
          (Development|PrintString "Hello"))))))

(event EventBeginPlay
  (Actor|SetLifeSpan (Variables|Default|GetLifespan)))

(fn ConstructionScript
  (bind _projectilemovement (Variables|Components|GetProjectileMovement))
  (if (Variables|/Script/Engine.ProjectileMovementComponent|GetbIsHomingProjectile _projectilemovement)
    (Variables|/Script/Engine.ProjectileMovementComponent|SetHomingTargetComponent _projectilemovement (Variables|Default|GetAimPos))
    (Actor|SetLifeSpan (Variables|Default|GetLifespan))
    (Transformation|DetachFromActor "KeepRelative" "KeepRelative" "KeepRelative")))