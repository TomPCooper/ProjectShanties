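; Explosive projectile that, on overlapping anything other than its owner or ignore-tagged components, runs a radius sphere trace with debug drawing at its location.
; On a trace hit, if the overlapped actor has a component, it damages the single traced actor through an interface message.
; Damage is scaled by any boss body-part multiplier from the overlapped actor.
; It then calls the projectile-hit event, spawns a Niagara explosion and destroys itself.
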(event OnComponentBeginOverlap(Collider)
  (params (OverlappedComponent :type Primitive%20Component%20Object%20Reference) (OtherActor :type Actor%20Object%20Reference) (OtherComp :type Primitive%20Component%20Object%20Reference) (OtherBodyIndex :type Integer) (bFromSweep :type Boolean) (SweepResult :type Hit%20Result%20Structure%20%28by%20ref%29))
  (bind _returnvalue (Transformation|GetActorLocation))
  (bind _damage (Variables|Default|GetDamage))
  (if (!= OtherActor (Variables|Default|GetprojectileOwner))
    (if (not (Components|ComponentHasTag OtherComp "PROJECTILE_IGNORE"))
      (bind (_outhit _returnvalue_2) (Collision|SphereTraceByChannel _returnvalue _returnvalue (Variables|Default|GetExplosiveRadius) "TraceTypeQuery1" false 0 "ForDuration" true "(R=1.000000,G=0.000000,B=0.000000,A=1.000000)" "(R=0.000000,G=1.000000,B=0.000000,A=1.000000)" 1.0))
      (if _returnvalue_2
        (Utilities|IsValid (Actor|GetComponentbyClass OtherActor "/Script/Engine.ActorComponent")
          (:Is%20Valid
            (bind (_successful _damagemultiplier) (Class|BPIBossBodyPart|GetBossBodyPartDamageMultiplier(Message) OtherActor))
            (if _successful
              (Class|BPIHealth|IDamage(Message) (.HitActor (Collision|BreakHitResult _outhit)) (* _damagemultiplier _damage))
              (else
                (Class|BPIHealth|IDamage(Message) (.HitActor (Collision|BreakHitResult _outhit)) _damage)))
            (Default|CallEProjectileHit)
            (Niagara|SpawnSystematLocation "/Game/VFX/Fire/NS_Explosion.NS_Explosion" (Transformation|GetActorLocation))
            (Actor|DestroyActor)))))))

(event EventBeginPlay
  (|CallParentFunction) ; This node is disabled and will not be called.\nDrag off pins to build functionality.
)

(fn ConstructionScript
  (|CallParentFunction))