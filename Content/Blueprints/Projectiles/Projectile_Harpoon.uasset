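; Harpoon projectile fired from the player's ship that tethers to what it hits with a cable and can yank it loose, apparently enemy scales.
; On first overlap it attaches to the target, sizes the cable and starts timers, including a repeating check.
; Staying beyond the tether length for three seconds detaches the target, notifies it by interface and destroys the harpoon.
; A one-shot pull shortens tether and cable through a timeline.
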(event OnComponentBeginOverlap(Collider)
  (params (OverlappedComponent :type Primitive%20Component%20Object%20Reference) (OtherActor :type Actor%20Object%20Reference) (OtherComp :type Primitive%20Component%20Object%20Reference) (OtherBodyIndex :type Integer) (bFromSweep :type Boolean) (SweepResult :type Hit%20Result%20Structure%20%28by%20ref%29))
  ;[1 1 1] Activate harpoon once hit
  (Utilities|FlowControl|DoOnce false
    (:Completed
      (Actor|SetLifeSpan 0.0)
      (Components|Movement|StopMovementImmediately (Variables|Default|GetProjectileMovement))
      (bind _output_get (Variables|Default|SetEnemyHit OtherActor))
      (Transformation|AttachActorToActor _output_get "None" "SnapToTarget" "KeepRelative" "KeepRelative" true)
      (bind _enemymesh (Class|BPIHarpoon|IGetMeshReference(Message) _output_get))
      (Variables|Default|SetEnemy%20Mesh _enemymesh)
      (Utilities|Time|SetTimerbyEvent (EventDispatchers|CreateEvent :!event Custom|RemoveHarpoon) (Variables|Default|GetHarpoonAttachTime))
      (Utilities|Time|SetTimerbyEvent (EventDispatchers|CreateEvent :!event Custom|CheckDistance) 0.1 true)
      (bind _output_get_2 (Variables|Default|SetStartingDistance (+ (Math|Float|Absolute(Float) (Math|Vector|Distance(Vector) (Transformation|GetActorLocation (Variables|Default|GetprojectileOwner)) (Transformation|GetActorLocation (Variables|Default|GetEnemyHit)))) 2e+02)))
      (bind _output_get_3 (Variables|/Script/CableComponent.CableComponent|SetCableLength (Variables|Default|GetCable) (Math|Float|Absolute(Float) (Math|Vector|Distance(Vector) (Transformation|GetActorLocation (Variables|Default|GetprojectileOwner)) (Transformation|GetActorLocation (Variables|Default|GetEnemyHit))))))
      (Development|PrintString (Utilities|String|ToString(Float) _output_get_2) true true "(R=0.104824,G=1.000000,B=0.000000,A=1.000000)" 5.0)
      (Variables|/Script/CableComponent.CableComponent|SetTileMaterial (Variables|Default|GetCable) (/ _output_get_3 1e+01)))))

(event Custom|RemoveHarpoon
  ;[1 1 1] destroy actor
  (Development|PrintString "Removing Harpoon" true true "(R=1.000000,G=0.516063,B=0.000000,A=1.000000)")
  (Actor|DestroyActor))

(event Custom|CheckDistance
  ;[1 1 1] Check whether to pull scale
  (Utilities|IsValid (Variables|Default|GetEnemyHit)
    (:Is%20Valid
      (if (> (Math|Float|Absolute(Float) (Math|Vector|Distance(Vector) (Transformation|GetActorLocation (Variables|Default|GetprojectileOwner)) (Transformation|GetActorLocation (Variables|Default|GetEnemyHit)))) (Variables|Default|GetStartingDistance))
        (Utilities|FlowControl|DoOnce false :!label _label
          (:Completed
            (bind _returnvalue (Utilities|Time|SetTimerbyEvent (EventDispatchers|CreateEvent :!event Custom|DetachScale) 3.0))
            (Variables|Default|SetScaleDetachHandle _returnvalue)
            (Development|PrintString "Starting Pull!!!!" true true "(R=1.000000,G=0.000000,B=0.483562,A=1.000000)")))
        (else
          (Utilities|FlowControl|Sequence
            (:then_0
              (if (Utilities|Time|IsTimerActivebyHandle (Variables|Default|GetScaleDetachHandle))
                (Utilities|Time|ClearandInvalidateTimerbyHandle (Variables|Default|GetScaleDetachHandle))
                (Development|PrintString "Not far enough" true true "(R=1.000000,G=0.000000,B=0.069579,A=1.000000)")))
            (:then_1
              (goto _label Reset))))))))

(event Custom|DetachScale
  (bind _enemyhit (Variables|Default|GetEnemyHit))
  ;[1 1 1] Detach Scale
  (Development|PrintString "Yank! 
" true true "(R=0.060520,G=0.000000,B=1.000000,A=1.000000)")
  (Utilities|FlowControl|Delay 0.2)
  (Transformation|DetachFromActor _enemyhit "KeepRelative" "KeepRelative" "KeepRelative")
  (Class|BPIHarpoon|IActorPulled(Message) _enemyhit)
  (CallFunction|RemoveHarpoon))

(event Custom|PullHarpoon
  ;[1 1 1] Pull harpoon
  (Utilities|FlowControl|DoOnce false
    (:Completed
      (Variables|Default|SetPullDistance (- (Variables|Default|GetStartingDistance) 2e+02))
      (Development|PrintString "Hello")
      (bind _alpha (Timeline|Timeline Play)
        (:Update
          (bind _output_get (Variables|Default|SetStartingDistance (Math|Float|Lerp (Variables|Default|GetStartingDistance) (Variables|Default|GetPullDistance) _alpha)))
          (bind _output_get_2 (Variables|/Script/CableComponent.CableComponent|SetCableLength (Variables|Default|GetCable) _output_get))
          (Variables|/Script/CableComponent.CableComponent|SetTileMaterial (Variables|Default|GetCable) (/ _output_get_2 1e+01)))))))

(event EventBeginPlay
  (bind _projectileowner (Variables|Default|GetprojectileOwner))
  ;[1 1 1] Init cable
  (|CallParentFunction)
  (Class|CableComponent|SetAttachEndto (Variables|Default|GetCable) _projectileowner "SM_Boat" "HarpoonAttachPoint")
  (EventDispatchers|BindEventtoEDRetriggerWeapon (.AsPawn%20Ship%20Final (Utilities|Casting|CastToPawn_ShipFinal _projectileowner)) (EventDispatchers|CreateEvent :!event Custom|PullHarpoon)))

(fn ConstructionScript
  (|CallParentFunction))