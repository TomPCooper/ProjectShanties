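; BP_ProjectileJavelin is a javelin projectile that damages what it overlaps and can pierce when thrown with enough Strength.
; Its construction script calls Release, which scales Damage and initial speed by Strength as a percentage and applies MaxSpeed to ProjectileMovement.
; On Collider overlap it sends Damage to the other actor's BPC_Health through an interface message, then destroys itself unless Strength reaches PierceMinStrength.
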(event OnComponentBeginOverlap(Collider)
  (params (OverlappedComponent :type Primitive%20Component%20Object%20Reference) (OtherActor :type Actor%20Object%20Reference) (OtherComp :type Primitive%20Component%20Object%20Reference) (OtherBodyIndex :type Integer) (bFromSweep :type Boolean) (SweepResult :type Hit%20Result%20Structure%20%28by%20ref%29))
  ;[0 0 0] Javelin overlap
  (Class|BPIHealth|IDamage(Message) (Actor|GetComponentbyClass OtherActor "/Game/Blueprints/Health/BPC_Health.BPC_Health_C") (Variables|Default|GetDamage))
  (if (not (>= (Variables|Default|GetStrength) (Variables|Default|GetPierceMinStrength)))
    (Actor|DestroyActor)))

(event EventBeginPlay
  (|CallParentFunction) ; This node is disabled and will not be called.\nDrag off pins to build functionality.
)

(fn ConstructionScript
  (|CallParentFunction)
  (CallFunction|Release))

(fn Release
  (bind _strength (Variables|Default|GetStrength))
  (bind _projectilemovement (Variables|Default|GetProjectileMovement))
  (bind _returnvalue (/ _strength 1e+02))
  (Variables|Default|SetDamage (* _returnvalue (Variables|Default|GetDamage)))
  (Variables|/Script/Engine.ProjectileMovementComponent|SetInitialSpeed _projectilemovement (* _returnvalue (Variables|Default|GetMaxSpeed)))
  (Variables|/Script/Engine.ProjectileMovementComponent|SetMaxSpeed _projectilemovement (Variables|Default|GetMaxSpeed)))