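; Trigger volume that ends the prologue, spawning the end boss and moving the game on to the main level.
; When the ship's main component overlaps the cube, it spawns BP_TutorilaEndBossGuy and updates the pirate game state.
; Tick then holds the BP_DockedCamLocation actor above the overlapping ship at a fixed rotation.
; Timed delays show the UI_10YR widget, then open Main_Persistent.
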(event OnComponentBeginOverlap(Cube)
  (params (OverlappedComponent :type Primitive%20Component%20Object%20Reference) (OtherActor :type Actor%20Object%20Reference) (OtherComp :type Primitive%20Component%20Object%20Reference) (OtherBodyIndex :type Integer) (bFromSweep :type Boolean) (SweepResult :type Hit%20Result%20Structure%20%28by%20ref%29))
  (Utilities|IsValid OtherComp
    (:Is%20Valid
      (if (Components|ComponentHasTag OtherComp "SHIP_MAIN")
        (Variables|Default|SetPlayerRef OtherActor)
        (Game|SpawnActorfromClass "/Game/Blueprints/Interactions/BP_TutorilaEndBossGuy.BP_TutorilaEndBossGuy_C" (Math|Transform|MakeTransform "0, 0, 0" "0, 0, 0" "1.000000,1.000000,1.000000") "Undefined" "MultiplyWithRoot" 0 0)
        (bind _aspirate_game_state (Utilities|Casting|CastToPirate_GameState (Game|GetGameState)))
        (Default|UpdateState _aspirate_game_state "NewEnumerator2")
        (bind _returnvalue (Actor|GetActorOfClass "/Game/Blueprints/Interactions/BP_DockedCamLocation.BP_DockedCamLocation_C"))
        (Variables|Default|SetDockedCam _returnvalue)
        (Variables|Default|SetShouldMoveCam true)
        (Utilities|FlowControl|Delay 8.0)
        (bind _returnvalue_2 (UserInterface|CreateWidget "/Game/Blueprints/UI/UI_10YR.UI_10YR_C" (Game|GetPlayerController 0)))
        (UserInterface|Viewport|AddtoViewport _returnvalue_2 0)
        (Utilities|FlowControl|Delay 5.0)
        (Game|OpenLevel(byObjectReference) "/Game/Levels/MainLevel/Main_Persistent.Main_Persistent")))))

(event EventTick
  (params (DeltaSeconds :type Float%20%28single-precision%29))
  (if (Variables|Default|GetShouldMoveCam)
    (Transformation|SetActorTransform (Variables|Default|GetDockedCam) (Math|Transform|MakeTransform (+ (Transformation|GetActorLocation (Variables|Default|GetPlayerRef)) (Math|Vector|MakeVector 0.0 0.0 (Variables|Default|GetNewDockCamHeight))) "-90.000000,180.000000,0.000000" "1.000000,1.000000,1.000000"))))

(fn ConstructionScript)