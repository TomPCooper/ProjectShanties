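; BP_CaveGate is a gate that opens when the cave quest becomes the current quest.
; On BeginPlay it registers a check with Pirate_GameState's new-quest event.
; The check compares the game state's CurrentQuest to QuestCave and, on a match, hides the gate and disables its collision, with no path to close it again.
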(event Custom|CheckShouldOpen
  (bind _aspirate_game_state (Utilities|Casting|CastToPirate_GameState (Game|GetGameState)))
  (if (== (Variables|/Game/Blueprints/GameStates/Pirate_GameState.Pirate_GameState_C|GetCurrentQuest _aspirate_game_state) (Math|Conversions|ToInteger(Byte) (Variables|Default|GetQuestCave)))
    (Rendering|SetActorHiddenInGame true)
    (Collision|SetActorEnableCollision false)))

(event EventBeginPlay
  (bind _aspirate_game_state (Utilities|Casting|CastToPirate_GameState (Game|GetGameState)))
  (EventDispatchers|BindEventtoNewQuest _aspirate_game_state (delegate Custom|CheckShouldOpen)))

(fn ConstructionScript)