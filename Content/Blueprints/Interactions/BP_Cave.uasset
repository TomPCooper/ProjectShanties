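; BP_Cave is a trigger volume that tells the day/night system when the ship enters or leaves a cave.
; Begin and end overlaps on its Cube component filter for other components tagged SHIP_MAIN.
; Matching overlaps call EnterCave or ExitCave on the DayNightManager, which handles the response.
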(event OnComponentBeginOverlap(Cube)
  (params (OverlappedComponent :type Primitive%20Component%20Object%20Reference) (OtherActor :type Actor%20Object%20Reference) (OtherComp :type Primitive%20Component%20Object%20Reference) (OtherBodyIndex :type Integer) (bFromSweep :type Boolean) (SweepResult :type Hit%20Result%20Structure%20%28by%20ref%29))
  (Utilities|IsValid OtherComp
    (:Is%20Valid
      (if (Components|ComponentHasTag OtherComp "SHIP_MAIN")
        (Default|EnterCave (Variables|Default|GetDayNightManager))))))

(event OnComponentEndOverlap(Cube)
  (params (OverlappedComponent :type Primitive%20Component%20Object%20Reference) (OtherActor :type Actor%20Object%20Reference) (OtherComp :type Primitive%20Component%20Object%20Reference) (OtherBodyIndex :type Integer))
  (Utilities|IsValid OtherComp
    (:Is%20Valid
      (if (Components|ComponentHasTag OtherComp "SHIP_MAIN")
        (Default|ExitCave (Variables|Default|GetDayNightManager))))))

(fn ConstructionScript)