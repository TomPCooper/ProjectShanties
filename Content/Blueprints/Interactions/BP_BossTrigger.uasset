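; Boss trigger volume that changes the game state and operates a gate when its box is overlapped.
; Any overlap sends a new state to the game state through BPI_GameState, stopping if that interface is missing.
; It then opens or closes the referenced Gate according to ShouldOpen and destroys every BP_BossTrigger2 actor in the level.
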(event OnComponentBeginOverlap(Box)
  (params (OverlappedComponent :type Primitive%20Component%20Object%20Reference) (OtherActor :type Actor%20Object%20Reference) (OtherComp :type Primitive%20Component%20Object%20Reference) (OtherBodyIndex :type Integer) (bFromSweep :type Boolean) (SweepResult :type Hit%20Result%20Structure%20%28by%20ref%29))
  (bind _gate (Variables|Default|GetGate))
  (bind _asbpi_game_state (Utilities|Casting|CastToBPI_GameState (Game|GetGameState)))
  (Default|INewGameState _asbpi_game_state "NewEnumerator0")
  (if (Variables|Default|GetShouldOpen)
    (Default|OpenGate _gate)
    (else
      (Default|CloseGate _gate)))
  (bind _outactors (Actor|GetAllActorsOfClass "/Game/Blueprints/Interactions/BP_BossTrigger2.BP_BossTrigger2_C"))
  (for _array_element _outactors
    (Actor|DestroyActor _array_element)))

(event EventBeginPlay)

(fn ConstructionScript)