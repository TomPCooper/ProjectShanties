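; Boss gate actor that slides its Cube component between closed and open positions, both offsets from the actor's starting location.
; BeginPlay caches that location and snaps the gate open when StartOpen is set.
; OpenGate plays a Timeline that lerps the position and CloseGate reverses it from the end.
; Each event has its own DoOnce with no reset, so the gate opens and closes only once each.
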(event Custom|CloseGate
  (bind _startposition (Variables|Default|GetStartPosition))
  (Utilities|FlowControl|DoOnce false
    (:Completed
      (bind _door (Timeline|Timeline ReverseFromEnd)
        (:Update
          (Transformation|SetWorldLocation (Variables|Default|GetCube) (Math|Vector|Lerp(Vector) (+ (Variables|Default|GetClosedPosition) _startposition) (+ _startposition (Variables|Default|GetOpenPosition)) _door) false false))))))

(event Custom|OpenGate
  (bind _startposition (Variables|Default|GetStartPosition))
  (Utilities|FlowControl|DoOnce false
    (:Completed
      (bind _door (Timeline|Timeline PlayFromStart)
        (:Update
          (Transformation|SetWorldLocation (Variables|Default|GetCube) (Math|Vector|Lerp(Vector) (+ (Variables|Default|GetClosedPosition) _startposition) (+ _startposition (Variables|Default|GetOpenPosition)) _door) false false))))))

(event EventBeginPlay
  (Variables|Default|SetStartPosition (Transformation|GetActorLocation))
  (if (Variables|Default|GetStartOpen)
    (Transformation|SetWorldLocation (Variables|Default|GetCube) (+ (Variables|Default|GetOpenPosition) (Variables|Default|GetStartPosition)) false false)))

(fn ConstructionScript)