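; BP_BossTrigger2 is a trigger volume that switches the game state and operates a gate when the main ship enters it.
; Overlap of its Cube by a component tagged SHIP_MAIN sends a new state through BPI_GameState, then opens or closes Gate according to ShouldOpen.
; After a ten-second delay it sends a second state and destroys every actor in AllTriggers.
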(event OnComponentBeginOverlap(Cube)
  (params (OverlappedComponent :type Primitive%20Component%20Object%20Reference) (OtherActor :type Actor%20Object%20Reference) (OtherComp :type Primitive%20Component%20Object%20Reference) (OtherBodyIndex :type Integer) (bFromSweep :type Boolean) (SweepResult :type Hit%20Result%20Structure%20%28by%20ref%29))
  (bind _gate (Variables|Default|GetGate))
  (if (Components|ComponentHasTag OtherComp "SHIP_MAIN")
    (bind _asbpi_game_state (Utilities|Casting|CastToBPI_GameState (Game|GetGameState)))
    (Default|INewGameState _asbpi_game_state "NewEnumerator2")
    (if (Variables|Default|GetShouldOpen)
      (Default|OpenGate _gate)
      (else
        (Default|CloseGate _gate)))
    (Utilities|FlowControl|Delay 1e+01)
    (bind _asbpi_game_state_2 (Utilities|Casting|CastToBPI_GameState (Game|GetGameState)))
    (Default|INewGameState _asbpi_game_state_2 "NewEnumerator1")
    (CallFunction|DestroyAll)))

(event Custom|DestroyAll
  (for _array_element (Variables|Default|GetAllTriggers)
    (Actor|DestroyActor _array_element)))

(event EventBeginPlay)

(event Collision|EventActorBeginOverlap
  (params (OtherActor :type Actor%20Object%20Reference)))

(event EventTick
  (params (DeltaSeconds :type Float%20%28single-precision%29)))

(fn ConstructionScript)