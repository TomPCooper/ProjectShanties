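; Sea boss that circles the player and attacks their ship, dealing damage on overlap to actors with a health component.
; Player overlap starts it on a spawned circle spline; AttackCheck picks Ram or Whirlpool at long range, Chomp or Leap up close, limiting repeats.
; Timelines drive movement, using spawned helper splines for Leap and Chomp, then easing back onto a fresh circle.
; Whirlpool currently only returns to circling; its attack logic is disconnected.
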(event OnComponentBeginOverlap(Activation_Range)
  (params (OverlappedComponent :type Primitive%20Component%20Object%20Reference) (OtherActor :type Actor%20Object%20Reference) (OtherComp :type Primitive%20Component%20Object%20Reference) (OtherBodyIndex :type Integer) (bFromSweep :type Boolean) (SweepResult :type Hit%20Result%20Structure%20%28by%20ref%29))
  ;[0 0 0] Triggers Bosses Behaviour
  (if (== OtherActor (Variables|Default|GetPlayer))
    (Utilities|FlowControl|DoOnce false
      (:Completed
        (Utilities|Time|SetTimerbyEvent (EventDispatchers|CreateEvent :!event Custom|Circle) 0.02)
        (bind _returnvalue (Game|SpawnActorfromClass "/Game/Blueprints/Bosses/BP_CircleHelper.BP_CircleHelper_C" (Transformation|GetActorTransform (Variables|Default|GetPlayer)) "Undefined" "MultiplyWithRoot" 0 0))
        (bind _output_get (Variables|Default|SetCurrent%20Circle%20Helper _returnvalue))
        (Variables|Default|SetCircle%20Helper%20Spline (Variables|/Game/Blueprints/Bosses/BP_CircleHelper.BP_CircleHelper_C|GetCircleSpline _output_get))))))

(event OnComponentBeginOverlap(DamageArea)
  (params (OverlappedComponent :type Primitive%20Component%20Object%20Reference) (OtherActor :type Actor%20Object%20Reference) (OtherComp :type Primitive%20Component%20Object%20Reference) (OtherBodyIndex :type Integer) (bFromSweep :type Boolean) (SweepResult :type Hit%20Result%20Structure%20%28by%20ref%29))
  (bind _returnvalue (Actor|GetComponentbyClass OtherActor "/Game/Blueprints/Health/BPC_Health.BPC_Health_C"))
  ;[1 1 1] If begins overlapping with player, deal damage
  (if (and (!= OtherActor self) (Utilities|IsValid _returnvalue))
    (Default|IDamage _returnvalue 5e+01)))

(event Custom|AttackCheck
  (bind _returnvalue (Math|Random|RandomBool))
  ;[0 0 0] Attack Selector
  (if (> (Transformation|GetDistanceTo (Variables|Default|GetPlayer)) (Variables|Default|GetAttackChangeRange))
    (if _returnvalue
      ;;[1 1 1] If whirlpool is used, neither it or the attack used after is selected
      (if (Variables|Default|GetUsedWhirlpool)
        (Variables|Default|SetUsedWhirlpool false)
        (CallFunction|Ram :!label _label)
        (Variables|Default|SetLastAttack "NewEnumerator3")
        (else
          (CallFunction|WhirlPool :!label _label_2)
          (Variables|Default|SetUsedWhirlpool true)
          (Variables|Default|SetLastAttack "NewEnumerator2")))
      (else
        ;;[1 1 1] Avoids using the same attack twice
        (if (Utilities|Enum|Equal(Enum) (Variables|Default|GetLastAttack) "NewEnumerator2")
          (goto _label)
          (else
            (goto _label_2)))))
    (elif _returnvalue
      (if (Utilities|Enum|Equal(Enum) (Variables|Default|GetLastAttack) "NewEnumerator1")
        (CallFunction|Leap :!label _label_3)
        (Variables|Default|SetLastAttack "NewEnumerator0")
        (else
          (CallFunction|Chomp :!label _label_4)
          (Variables|Default|SetLastAttack "NewEnumerator1")))
      (elif (Utilities|Enum|Equal(Enum) (Variables|Default|GetLastAttack) "NewEnumerator0")
        (goto _label_4)
        (else
          (goto _label_3))))))

(event Custom|Ram
  ;[0 0 0] Ram
  (Audio|Components|Audio|Stop (Variables|Default|GetCircleTL))
  (bind (_bossloc _locundership) (CallFunction|GetPositionUnderShip))
  (Variables|Default|SetRam%20Start%20Location _bossloc)
  (Variables|Default|SetRam%20Target%20Location _locundership)
  (bind _returnvalue (Utilities|Time|SetTimerbyEvent (delegate Custom|RamActive) 0.02))
  (bind _output_get (Variables|Default|SetRamHandler _returnvalue))
  (Variables|Default|SetCurrent%20Attack%20Handle _output_get))

(event Custom|Return%20to%20Circle
  ;[0 0 0] Return To Circle - When an attack finishes, the boss' transform is set to the transform of where the circle will continue.
  (Actor|DestroyActor (Variables|Default|GetCurrent%20Circle%20Helper))
  (bind _returnvalue (Game|SpawnActorfromClass "/Game/Blueprints/Bosses/BP_CircleHelper.BP_CircleHelper_C" (Transformation|GetActorTransform (Variables|Default|GetPlayer)) "Undefined" "MultiplyWithRoot" 0 0))
  (bind _output_get (Variables|Default|SetCurrent%20Circle%20Helper _returnvalue))
  (Variables|Default|SetCircle%20Helper%20Spline (Variables|/Game/Blueprints/Bosses/BP_CircleHelper.BP_CircleHelper_C|GetCircleSpline _output_get))
  (Variables|Default|SetCurrentTransform (Transformation|GetActorTransform))
  (Variables|Default|SetTargetTransform (Spline|GetTransformatDistanceAlongSpline (Variables|Default|GetCircle%20Helper%20Spline) 0.0 "World" false))
  (bind _alpha (Timeline|ReturnToCircle PlayFromStart)
    (:Update
      (Transformation|SetActorTransform (Math|Transform|MakeTransform (.location (Math|Transform|Lerp(Transform) (Variables|Default|GetCurrentTransform) (Variables|Default|GetTargetTransform) _alpha)) (Math|Rotator|FindLookatRotation (Transformation|GetActorLocation) (.location (Variables|Default|GetTargetTransform))) "1.000000,1.000000,1.000000")))
    (:Finished
      (CallFunction|Circle))))

(event Custom|Circle
  ;[0 0 0] Circle
  (Utilities|Time|SetTimerbyEvent (EventDispatchers|CreateEvent :!event Custom|AttackCheck) (Variables|Default|GetAttackCheckFrequency))
  (bind _alpha (Timeline|CircleTL PlayFromStart)
    (:Update
      (Variables|Default|SetCurrentSplineDistance (Math|Float|Lerp 0.0 (Spline|GetSplineLength (Variables|Default|GetCircle%20Helper%20Spline)) _alpha))
      (Transformation|SetActorTransform (Math|Transform|MakeTransform (.location (Spline|GetTransformatDistanceAlongSpline (Variables|Default|GetCircle%20Helper%20Spline) (Variables|Default|GetCurrentSplineDistance) "World" false)) (.rotation (Spline|GetTransformatDistanceAlongSpline (Variables|Default|GetCircle%20Helper%20Spline) (Variables|Default|GetCurrentSplineDistance) "World" false)) "1.000000,1.000000,1.000000") true))))

(event Custom|ShowOff
  (bind _showoffstart (Variables|Default|GetShowOffStart))
  (bind _showoffend (Variables|Default|GetShowOffEnd))
  (bind _whirlpoolstartrot (Variables|Default|GetWhirlPoolStartRot))
  (bind _returnvalue (Transformation|GetActorLocation _showoffstart))
  (bind _returnvalue_2 (Transformation|GetActorLocation _showoffend))
  (bind _returnvalue_3 (- _returnvalue _returnvalue_2))
  (bind _returnvalue_4 (Math|Vector|Normalize _returnvalue_3))
  (bind _returnvalue_5 (Math|Vector|VectorLength _returnvalue_3))
  (bind _returnvalue_6 (/ _returnvalue_5 2.0))
  (bind _returnvalue_7 (* _returnvalue_6 _returnvalue_4))
  (bind _returnvalue_8 (- _returnvalue _returnvalue_7))
  ;[0 0 0] Showoff
  (Variables|Default|SetShowOffStartRot (Math|Rotator|FindLookatRotation _returnvalue_8 _returnvalue))
  (bind _newtrack_0 (Timeline|T_Showoff PlayFromStart)
    (:Update
      (Transformation|SetActorLocationAndRotation (+ _returnvalue_8 (* (Math|Vector|GetForwardVector (Math|Rotator|MakeRotator (.roll _whirlpoolstartrot) (+ (* _newtrack_0 -2.7e+02) (.pitch _whirlpoolstartrot) 225.0) (.yaw _whirlpoolstartrot))) (/ (Math|Vector|VectorLength (- (Transformation|GetActorLocation (Variables|Default|GetShowOffStart)) (Transformation|GetActorLocation (Variables|Default|GetShowOffEnd)))) 2.0))) (Math|Rotator|MakeRotator 1.8e+02 (+ (* _newtrack_0 -2.7e+02) -7e+01) 0.0)))
    (:Finished
      (CallFunction|Reset))))

(event Custom|Chomp
  ;[0 0 0] Chomp
  (Audio|Components|Audio|Stop (Variables|Default|GetCircleTL))
  (bind _returnvalue (Game|SpawnActorfromClass "/Game/Blueprints/Bosses/BP_ChompHelper.BP_ChompHelper_C" (Math|Transform|MakeTransform (Transformation|GetWorldLocation (Variables|Default|GetLeapSplineStartLocation)) "0, 0, 0" "1.000000,1.000000,1.000000") "Undefined" "MultiplyWithRoot" 0 0 0))
  (bind _alpha (Timeline|Timeline PlayFromStart)
    (:Update
      (bind _output_get (Variables|Default|SetCurrentSplineDistance (Math|Float|Lerp 0.0 (Spline|GetSplineLength (Variables|/Game/Blueprints/Bosses/BP_ChompHelper.BP_ChompHelper_C|GetChompSpline1 _returnvalue)) _alpha)))
      (Transformation|SetActorTransform (Spline|GetTransformatDistanceAlongSpline (Variables|/Game/Blueprints/Bosses/BP_ChompHelper.BP_ChompHelper_C|GetChompSpline1 _returnvalue) _output_get "World" false)))
    (:Finished
      (Actor|DestroyActor _returnvalue)
      (CallFunction|ReturntoCircle))))

(event Custom|Roam)

(event Custom|WhirlPool
  ;[0 0 0] Whirlpool
  (Audio|Components|Audio|Stop (Variables|Default|GetCircleTL))
  (CallFunction|ReturntoCircle))

(event Custom|Reset
  ;[0 0 0] Reset
  (Variables|Default|SetResetStartTransform (Transformation|GetActorTransform))
  (bind _newtrack_0 (Timeline|T_Reset Play)
    (:Update
      (Transformation|SetActorTransform (Math|Transform|Lerp(Transform) (Variables|Default|GetResetStartTransform) (Math|Transform|MakeTransform (Variables|Default|GetStartLoc) "0, 0, 0" "1.000000,1.000000,1.000000") _newtrack_0)))))

(event Custom|WhirlpoolFinished
  ;[0 0 0] Attack Selector
  (if (Variables|/Game/Blueprints/Water/BP_Whirlpool.BP_Whirlpool_C|GetHasShip (Variables|Default|GetBP_Whirlpool))
    (CallFunction|Chomp)
    (Variables|Default|SetLastAttack "NewEnumerator1")
    (else
      (CallFunction|Leap)
      (Variables|Default|SetLastAttack "NewEnumerator0"))))

(event Custom|RamActive
  ;[0 0 0] Ram
  (Transformation|SetActorRotation (Math|Rotator|FindLookatRotation (Transformation|GetActorLocation) (Transformation|GetActorLocation (Variables|Default|GetPlayer))))
  (bind _alpha (Timeline|RamTL PlayFromStart)
    (:Update
      (Transformation|SetActorLocation (Math|Vector|Lerp(Vector) (Variables|Default|GetRam%20Start%20Location) (Variables|Default|GetRam%20Target%20Location) _alpha) false false))
    (:Finished
      (Utilities|Time|ClearandInvalidateTimerbyHandle (Variables|Default|GetCurrent%20Attack%20Handle))
      (CallFunction|ReturntoCircle))))

(event Custom|Leap
  ;[0 0 0] Leap
  (Audio|Components|Audio|Stop (Variables|Default|GetCircleTL))
  (bind _returnvalue (Game|SpawnActorfromClass "/Game/Blueprints/Bosses/BP_LeapHelper.BP_LeapHelper_C" (Math|Transform|MakeTransform (Transformation|GetWorldLocation (Variables|Default|GetLeapSplineStartLocation)) "0, 0, 0" "1.000000,1.000000,1.000000") "Undefined" "MultiplyWithRoot" 0 0))
  (bind _position (Class|BPIShip|IBossGetLeapPosition(Message) (Variables|Default|GetPlayer)))
  (Default|UpdateLandLocation _returnvalue _position)
  (bind _alpha (Timeline|LeapTL PlayFromStart)
    (:Update
      (bind _output_get (Variables|Default|SetCurrentSplineDistance (Math|Float|Lerp 0.0 (Spline|GetSplineLength (Variables|/Game/Blueprints/Bosses/BP_LeapHelper.BP_LeapHelper_C|GetLeapSpline _returnvalue)) _alpha)))
      (Transformation|SetActorTransform (Spline|GetTransformatDistanceAlongSpline (Variables|/Game/Blueprints/Bosses/BP_LeapHelper.BP_LeapHelper_C|GetLeapSpline _returnvalue) _output_get "World" false)))
    (:Finished
      (CallFunction|ReturntoCircle))))

(event EventBeginPlay
  ;[1 1 1] Boss initialisation
  (Variables|Default|SetPlayer (Game|Player|GetPlayerPawn 0))
  (Default|InitHealthComponent (Variables|Default|GetBPC_Health)))

(fn ConstructionScript)

(fn TransformActorAlongSpline
  (params (Distance :type Float%20%28double-precision%29) (Spline :type Spline%20Component%20Object%20Reference) (Actor :type Actor%20Object%20Reference))
  (bind _returnvalue (Spline|GetLocationatDistanceAlongSpline Spline Distance "World"))
  (Transformation|SetActorTransform Actor (Math|Transform|MakeTransform _returnvalue (Math|Rotator|FindLookatRotation _returnvalue (Spline|GetTangentatDistanceAlongSpline Spline Distance "World")) "1.000000,1.000000,1.000000")))

(fn SetSplinePointStartandEnd
  (params (Spline :type Spline%20Component%20Object%20Reference) (Start :type Vector) (End :type Vector))
  (Transformation|SetWorldTransform Spline (Math|Transform|MakeTransform Start (Math|Rotator|FindLookatRotation Start End) (Math|Conversions|ToVector(Float) (* 1.0 (Math|Vector|VectorLength (- Start End)) (Math|Vector|VectorLength (- (Spline|GetLocationatSplinePoint Spline 0 "Local") (Spline|GetLocationatSplinePoint Spline (Class|SplineComponent|GetNumberOfSplineSegments Spline) "Local")))))) false false))

(fn GetPositionUnderShip
  (bind _returnvalue (Transformation|GetActorLocation))
  (bind _player (Variables|Default|GetPlayer))
  (bind _returnvalue_2 (Transformation|GetActorLocation _player))
  (return _returnvalue (Math|Vector|MakeVector (.x _returnvalue_2) (.y _returnvalue_2) (.Z (Class|KismetMathLibrary|BreakVector3f _returnvalue)))))

(fn LerpAlongSpline
  (params (Spline :type Spline%20Component%20Object%20Reference) (Actor :type Actor%20Object%20Reference) (Speed :type Float%20%28double-precision%29))
  (bind _returnvalue (Spline|GetSplineLength Spline))
  (bind _output_get (Variables|Default|SetDistanceAlongAttack (+ (Variables|Default|GetDistanceAlongAttack) Speed)))
  (CallFunction|TransformActorAlongSpline (Math|Float|Lerp 0.0 _returnvalue (Math|Float|Clamp(Float) _output_get 0.0 _returnvalue)) Spline Actor)
  (return (== (Math|Float|Clamp(Float) _output_get 0.0 _returnvalue) _returnvalue)))

(fn SplinetoTransform
  (params (Spline :type Spline%20Component%20Object%20Reference) (SplineDistance :type Float%20%28single-precision%29))
  (bind _returnvalue (Spline|GetTransformatDistanceAlongSpline Spline SplineDistance "World" false))
  (return (Math|Transform|MakeTransform (.location _returnvalue) (.rotation _returnvalue) "1.000000,1.000000,1.000000")))