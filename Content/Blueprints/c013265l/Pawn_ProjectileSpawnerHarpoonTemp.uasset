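; Temporary harpoon projectile spawner, a child Blueprint that overrides weapon firing.
; On IFireWeapon it spawns a Projectile_Harpoon at the ProjectileSpawnReference transform, passing the player 0 pawn as owner and the AimPos target.
; A lookup in DT_ProjectilesConversion only gates the spawn, as the class is hardcoded and the enum-to-class result is unused.
; Debug prints report firing and a missing table row.
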(event EventIFireWeapon
  (params (CurrentProjectile :type Enum_Projectiles%20Enum :default "NewEnumerator0"))
  (Development|PrintString "Fired in child")
  (bind _returnvalue (Utilities|GetDataTableRow "/Game/Blueprints/Projectiles/DT_ProjectilesConversion.DT_ProjectilesConversion" "Projectile")
    (:then
      (Game|SpawnActorfromClass "/Game/Blueprints/Projectiles/Projectile_Harpoon.Projectile_Harpoon_C" (Transformation|GetWorldTransform (Variables|Default|GetProjectileSpawnReference)) "Undefined" "MultiplyWithRoot" 0 (Pawn|GetControlledPawn (Game|GetPlayerController 0)) "0.000000,0.000000,0.000000" (Variables|Default|GetAimPos) 0))
    (:RowNotFound
      (Development|PrintString "Lookup table could not find a projectile class with the requested enum value"))))

(fn ConstructionScript)