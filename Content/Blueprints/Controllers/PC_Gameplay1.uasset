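; Gameplay player controller that routes player input to the controlled ship pawn and creates the HUD.
; Enhanced Input look and move, plus legacy camera toggle and zoom bindings, are forwarded as interface messages to the pawn cached at BeginPlay.
; Weapon select input toggles the HUD's radial menu and delegates input mode switching to the HUD.
; The function named SetInputModeToUIOnly actually requests game-only mode.
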(event EventBeginPlay
  (Variables|References|SetShipPawnRef (Pawn|GetControlledPawn))
  (CallFunction|SetupMappingContext "/Game/Input/IMC_Default.IMC_Default")
  (Utilities|CreateHUD))

(event Input|EnhancedActionEvents|EnhancedInputActionIA_WeaponSelect
  (params (ActionValue :type Boolean) (ElapsedSeconds :type Float%20%28double-precision%29) (TriggeredSeconds :type Float%20%28double-precision%29) (InputAction :type Input%20Action%20Object%20Reference :default "/Game/Input/Actions/IA_WeaponSelect.IA_WeaponSelect"))
  ;[0 0 0] Weapon select radial menu
  (:Started
    (if ActionValue :!label _label
      (Utilities|SetInputModetoGameandUIOnly)
      (else
        (Utilities|SetInputModetoUIOnly)))
    (Class|BPIUI|SetWeaponSelectVisibility(Message) (Variables|References|GetHUDRef) ActionValue))
  (:Completed
    (goto _label)))

(event Input|EnhancedActionEvents|EnhancedInputActionIA_Look
  (params (ActionValue :type Vector%202D%20Structure) (ElapsedSeconds :type Float%20%28double-precision%29) (TriggeredSeconds :type Float%20%28double-precision%29) (InputAction :type Input%20Action%20Object%20Reference :default "/Game/Input/Actions/IA_Look.IA_Look"))
  (:Triggered
    (Class|BPIControllerInput|ILookInput(Message) (Variables|References|GetShipPawnRef) (.x ActionValue) (.y ActionValue))))

(event Input|EnhancedActionEvents|EnhancedInputActionIA_Move
  (params (ActionValue :type Vector%202D%20Structure) (ElapsedSeconds :type Float%20%28double-precision%29) (TriggeredSeconds :type Float%20%28double-precision%29) (InputAction :type Input%20Action%20Object%20Reference :default "/Game/Input/Actions/IA_Move.IA_Move"))
  (bind _shippawnref (Variables|References|GetShipPawnRef))
  (:Triggered
    (Class|BPIControllerInput|IMoveInputTriggered(Message) _shippawnref (.x ActionValue) (.y ActionValue)))
  (:Started
    (Class|BPIControllerInput|IMoveInputStarted(Message) _shippawnref)))

(event Input|ActionEvents|InputActionMoveCam
  (params (Key :type Key%20Structure))
  (bind _shippawnref (Variables|References|GetShipPawnRef))
  (:Pressed
    (Class|BPIControllerInput|ICameraMovementToggle(Message) _shippawnref true))
  (:Released
    (Class|BPIControllerInput|ICameraMovementToggle(Message) _shippawnref false)))

(event Input|AxisEvents|InputAxisZoom
  (params (AxisValue :type Float%20%28single-precision%29))
  (Class|BPIControllerInput|IZoomInput(Message) (Variables|References|GetShipPawnRef) AxisValue))

(fn ConstructionScript)

(fn SetupMappingContext
  (params (Context :type Input%20Mapping%20Context%20Object%20Reference))
  (bind _returnvalue (PlayerController|LocalPlayerSubsystems|GetEnhancedInputLocalPlayerSubsystem))
  (Utilities|IsValid _returnvalue
    (:Is%20Valid
      (Input|AddMappingContext _returnvalue Context 0 "(bIgnoreAllPressedKeysUntilRelease=True,bForceImmediately=False)"))))