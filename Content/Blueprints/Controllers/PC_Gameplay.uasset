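; Gameplay player controller for a ship pawn, handling input, HUD creation and foam capture setup.
; Enhanced Input look and move actions, plus a legacy Zoom axis, are forwarded to the pawn through interface messages.
; The weapon-select action toggles the HUD's radial wheel and input mode, while sector selection is an empty stub for weapon switching.
; BPFoamControllerComponent attaches its capture to the possessed pawn and starts it on BeginPlay.
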(event EventPossess
  (params (PossessedPawn :type Pawn%20Object%20Reference))
  (Default|SetCaptureAttachment (Variables|Default|GetBP_Foam_Controller_Component) PossessedPawn)
  (Development|PrintString "Set Capture Attachment Called - PC" true true "(R=0.000000,G=0.660000,B=1.000000,A=1.000000)" 5.0))

(event EventBeginPlay
  (Input|SetInputModeGameOnly self false)
  (Variables|References|SetShipPawnRef (Pawn|GetControlledPawn))
  (CallFunction|SetupMappingContext "/Game/Input/IMC_Default.IMC_Default")
  (CallFunction|CreateHUD)
  (Development|PrintString "Game Begin" true true "(R=0.995000,G=1.000000,B=0.000000,A=1.000000)" 5.0)
  (Default|InitiateFoamCapture (Variables|Default|GetBP_Foam_Controller_Component))
  (Development|PrintString "Initiate Foam Capture Called - PC" true true "(R=0.000000,G=0.660000,B=1.000000,A=1.000000)" 5.0))

(event Custom|WeaponWheelSectorSelected
  (params (Index :type Integer))
  ;[0 0 0] Sector selected on weapon wheel - ((IMPLEMENT WEAPON SWITCHING HERE))
)

(event Input|EnhancedActionEvents|EnhancedInputActionIA_WeaponSelect
  (params (ActionValue :type Boolean) (ElapsedSeconds :type Float%20%28double-precision%29) (TriggeredSeconds :type Float%20%28double-precision%29) (InputAction :type Input%20Action%20Object%20Reference :default "/Game/Input/Actions/IA_WeaponSelect.IA_WeaponSelect"))
  ;[0 0 0] Weapon select radial menu
  (:Started
    (if ActionValue :!label _label
      (Utilities|SetInputModetoGameandUIOnly)
      (else
        (Utilities|SetInputModetoUIOnly)))
    (Class|BPIUI|SetWeaponSelectVisibility(Message) (Variables|References|GetHUDRef) ActionValue))
  (:Completed
    (goto _label)))

(event Input|EnhancedActionEvents|EnhancedInputActionIA_Look
  (params (ActionValue :type Vector%202D%20Structure) (ElapsedSeconds :type Float%20%28double-precision%29) (TriggeredSeconds :type Float%20%28double-precision%29) (InputAction :type Input%20Action%20Object%20Reference :default "/Game/Input/Actions/IA_Look.IA_Look"))
  (:Triggered
    (Class|BPIControllerInput|ILookInput(Message) (Variables|References|GetShipPawnRef) (.x ActionValue) (.y ActionValue))))

(event Input|EnhancedActionEvents|EnhancedInputActionIA_Move
  (params (ActionValue :type Vector%202D%20Structure) (ElapsedSeconds :type Float%20%28double-precision%29) (TriggeredSeconds :type Float%20%28double-precision%29) (InputAction :type Input%20Action%20Object%20Reference :default "/Game/Input/Actions/IA_Move.IA_Move"))
  (bind _shippawnref (Variables|References|GetShipPawnRef))
  (:Triggered
    (Class|BPIControllerInput|IMoveInputTriggered(Message) _shippawnref (.x ActionValue) (.y ActionValue)))
  (:Started
    (Class|BPIControllerInput|IMoveInputStarted(Message) _shippawnref))
  (:Completed
    (Class|BPIControllerInput|IMoveInputStopped(Message) _shippawnref)))

(event Input|AxisEvents|InputAxisZoom
  (params (AxisValue :type Float%20%28single-precision%29))
  (Class|BPIControllerInput|IZoomInput(Message) (Variables|References|GetShipPawnRef) AxisValue))

(fn ConstructionScript)

(fn SetupMappingContext
  (params (Context :type Input%20Mapping%20Context%20Object%20Reference))
  (bind _returnvalue (PlayerController|LocalPlayerSubsystems|GetEnhancedInputLocalPlayerSubsystem))
  (Utilities|IsValid _returnvalue
    (:Is%20Valid
      (Input|AddMappingContext _returnvalue Context 0 "(bIgnoreAllPressedKeysUntilRelease=True,bForceImmediately=False)"))))

(fn CreateHUD
  (bind _returnvalue (UserInterface|CreateWidget "/Game/Blueprints/UI/HUD/UI_HUD.UI_HUD_C" self))
  (bind _output_get (Variables|References|SetHUDRef _returnvalue))
  (EventDispatchers|BindEventtoEWeaponWheelSectorSelected _output_get (EventDispatchers|CreateEvent :!event Custom|WeaponWheelSectorSelected))
  (UserInterface|Viewport|AddtoViewport _output_get 10))

(fn GetHUDReference
  (return (Variables|References|GetHUDRef)))