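; PC_MainMenu is the main menu player controller, handling Enhanced Input setup and look input.
; On BeginPlay it adds the default input mapping context to the local player's Enhanced Input subsystem, if that subsystem is valid.
; While the look action triggers, it forwards the value to UI through InputLook and prints with screen output off.
; An unconnected switch on the most recently used hardware device never runs.
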(event Input|EnhancedActionEvents|EnhancedInputActionIA_Look
  (params (ActionValue :type Vector%202D%20Structure) (ElapsedSeconds :type Float%20%28double-precision%29) (TriggeredSeconds :type Float%20%28double-precision%29) (InputAction :type Input%20Action%20Object%20Reference :default "/Game/Input/Actions/IA_Look.IA_Look"))
  (:Triggered
    (Default|InputLook (Variables|Default|GetUI) ActionValue)
    (Development|PrintString "Hello" false)))

(event EventBeginPlay
  (bind _returnvalue (PlayerController|LocalPlayerSubsystems|GetEnhancedInputLocalPlayerSubsystem))
  (Utilities|IsValid _returnvalue
    (:Is%20Valid
      (Input|AddMappingContext _returnvalue "/Game/Input/IMC_Default.IMC_Default" 0 "(bIgnoreAllPressedKeysUntilRelease=True,bForceImmediately=False)"))))

(event EventTick
  (params (DeltaSeconds :type Float%20%28single-precision%29)))

(fn ConstructionScript)