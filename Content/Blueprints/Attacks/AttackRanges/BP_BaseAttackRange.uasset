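; Base attack range actor that builds a spline-following mesh outline with the AimingRange collision profile.
; Its construction script splits the spline by SectionLength and adds a configurable spline mesh per section, with an optional material override.
; Segment tangents are clamped to the section length.
; MustBeFullLengthMeshes drops the final partial section, otherwise an extra mesh covers the remainder; the event graph is unused.
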(event EventBeginPlay)

(event Collision|EventActorBeginOverlap
  (params (OtherActor :type Actor%20Object%20Reference)))

(event EventTick
  (params (DeltaSeconds :type Float%20%28single-precision%29)))

(fn ConstructionScript
  (bind _meshscale (Variables|Default|GetMeshScale))
  (bind _meshscale_2 (Variables|Default|GetMeshScale))
  (if (Variables|Default|GetMustBeFullLengthMeshes?)
    ;[1 1 1] Ensures full length meshes only
    (for _index (range 0 (- (Math|Float|Truncate (/ (Spline|GetSplineLength (Variables|Default|GetSpline)) (Variables|Default|GetSectionLength))) 1))
      (LocalVariables|SetLoopIndex _index)
      (bind _returnvalue (AddComponent|AddSplineMeshComponent false))
      (Components|StaticMesh|SetStaticMesh _returnvalue (Variables|Default|GetSplineMesh))
      (SplineMesh|SetStartScale _returnvalue (Math|Vector2D|MakeVector2D _meshscale_2 _meshscale_2) true :!class /Script/Engine.SplineMeshComponent)
      (SplineMesh|SetEndScale _returnvalue (Math|Vector2D|MakeVector2D _meshscale _meshscale) true :!class /Script/Engine.SplineMeshComponent)
      (if (Variables|Default|GetMaterialOverride)
        (Rendering|Material|SetMaterial _returnvalue 0 (Variables|Default|GetMaterial)))
      (SplineMesh|SetForwardAxis _returnvalue (Variables|Default|GetMeshForwardAxis) true)
      (bind (_position _tangent) (CallFunction|GetStartPos/Tangent (LocalVariables|GetLoopIndex)))
      (bind (_position_2 _tangent_2) (CallFunction|GetEndPos/Tangent (LocalVariables|GetLoopIndex)))
      (SplineMesh|SetStartandEnd _returnvalue _position _tangent _position_2 _tangent_2 true :!class /Script/Engine.SplineMeshComponent)
      (Collision|SetCollisionProfileName _returnvalue "AimingRange" true :!class /Script/Engine.PrimitiveComponent))
    (else
      ;[1 1 1] Length of spline/section length = number of meshes
      (for _index_2 (range 0 (Math|Float|Truncate (/ (Spline|GetSplineLength (Variables|Default|GetSpline)) (Variables|Default|GetSectionLength))))
        (LocalVariables|SetLoopIndex _index_2)
        (bind _returnvalue_2 (AddComponent|AddSplineMeshComponent false))
        (Components|StaticMesh|SetStaticMesh _returnvalue_2 (Variables|Default|GetSplineMesh))
        (SplineMesh|SetStartScale _returnvalue_2 (Math|Vector2D|MakeVector2D _meshscale_2 _meshscale_2) true :!class /Script/Engine.SplineMeshComponent)
        (SplineMesh|SetEndScale _returnvalue_2 (Math|Vector2D|MakeVector2D _meshscale _meshscale) true :!class /Script/Engine.SplineMeshComponent)
        (if (Variables|Default|GetMaterialOverride)
          (Rendering|Material|SetMaterial _returnvalue_2 0 (Variables|Default|GetMaterial)))
        (SplineMesh|SetForwardAxis _returnvalue_2 (Variables|Default|GetMeshForwardAxis) true)
        (bind (_position_3 _tangent_3) (CallFunction|GetStartPos/Tangent (LocalVariables|GetLoopIndex)))
        (bind (_position_4 _tangent_4) (CallFunction|GetEndPos/Tangent (LocalVariables|GetLoopIndex)))
        (SplineMesh|SetStartandEnd _returnvalue_2 _position_3 _tangent_3 _position_4 _tangent_4 true :!class /Script/Engine.SplineMeshComponent)
        (Collision|SetCollisionProfileName _returnvalue_2 "AimingRange" true :!class /Script/Engine.PrimitiveComponent)))))

(fn GetStartPos/Tangent
  (params (Index :type Integer))
  (bind _sectionlength (Variables|Default|GetSectionLength))
  (bind _returnvalue (* Index _sectionlength))
  (return (Spline|GetLocationatDistanceAlongSpline (Variables|Default|GetSpline) _returnvalue "Local") (Math|Vector|ClampVectorSize (Spline|GetTangentatDistanceAlongSpline (Variables|Default|GetSpline) _returnvalue "Local") 0.0 (Variables|Default|GetSectionLength))))

(fn GetEndPos/Tangent
  (params (Index :type Integer))
  (bind _returnvalue (+ Index 1))
  (bind _sectionlength (Variables|Default|GetSectionLength))
  (bind _returnvalue_2 (* _returnvalue _sectionlength))
  (return (Spline|GetLocationatDistanceAlongSpline (Variables|Default|GetSpline) _returnvalue_2 "Local") (Math|Vector|ClampVectorSize (Spline|GetTangentatDistanceAlongSpline (Variables|Default|GetSpline) _returnvalue_2 "Local") 0.0 (Variables|Default|GetSectionLength))))