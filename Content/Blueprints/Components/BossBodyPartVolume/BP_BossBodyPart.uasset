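; BP_BossBodyPart is a box volume that represents one body part of a boss and carries its own damage multiplier.
; The construction script sizes the Box from the BoxExtent variable.
; Getter functions return the DamageMultiplier with a success flag and a reference to the part itself.
; A hit on the Box calls the Pull event, which is empty here.
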(event OnComponentHit(Box)
  (params (HitComponent :type Primitive%20Component%20Object%20Reference) (OtherActor :type Actor%20Object%20Reference) (OtherComp :type Primitive%20Component%20Object%20Reference) (NormalImpulse :type Vector :default "0, 0, 0") (Hit :type Hit%20Result%20Structure%20%28by%20ref%29))
  (CallFunction|Pull))

(event Custom|Pull)

(fn ConstructionScript
  (Components|Box|SetBoxExtent (Variables|Default|GetBox) (Variables|Default|GetBoxExtent) true))

(fn GetBossBodyPartDamageMultiplier
  (return true (Variables|Default|GetDamageMultiplier)))

(fn GetBossBodyPartReference
  (return self))