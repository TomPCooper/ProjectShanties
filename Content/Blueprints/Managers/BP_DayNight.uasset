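; Day/night manager that rotates a directional light through a cycle of sunrise, day, sunset and night.
; Tick derives sun pitch from real time and day length, converts it to clock time, and advances the state when near the next threshold.
; Transitions call CallNewTimeOfDay and drive timelines fading post-process fog and night-sky star materials.
; SetNewTime snaps materials and state without moving the sun; older timer-based logic remains disconnected.
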(event Custom|TimeIncrease)

(event Custom|StartTime)

(event Custom|Night
  (Default|CallNewTimeOfDay)
  (bind _nightfade (Timeline|NightFade PlayFromStart)
    (:Update
      (Rendering|Material|SetScalarParameterValue (Variables|Default|GetStarMaterial) "Opacity" _nightfade :!class /Script/Engine.MaterialInstanceDynamic))))

(event Custom|StopSunrise
  (bind _sunrisesunset (Timeline|Timeline ReverseFromEnd)
    (:Update
      (Rendering|Material|SetScalarParameterValue (Variables|Default|GetFogMaterial) "Fog Opacity" (Math|Float|Lerp 0.0 0.35 _sunrisesunset) :!class /Script/Engine.MaterialInstanceDynamic))))

(event Custom|NightFadeOut
  (bind _nightfade (Timeline|NightFade ReverseFromEnd)
    (:Update
      (Rendering|Material|SetScalarParameterValue (Variables|Default|GetStarMaterial) "Opacity" _nightfade :!class /Script/Engine.MaterialInstanceDynamic))))

(event Custom|Day
  (Default|CallNewTimeOfDay 2))

(event Custom|Sunrise
  (Default|CallNewTimeOfDay 1)
  (bind _sunrisesunset (Timeline|Timeline PlayFromStart)
    (:Update
      (Rendering|Material|SetScalarParameterValue (Variables|Default|GetFogMaterial) "Fog Opacity" (Math|Float|Lerp 0.0 0.35 _sunrisesunset) :!class /Script/Engine.MaterialInstanceDynamic))))

(event Custom|Sunset
  (Default|CallNewTimeOfDay 3)
  (bind _sunrisesunset (Timeline|Timeline PlayFromStart)
    (:Update
      (Rendering|Material|SetScalarParameterValue (Variables|Default|GetFogMaterial) "Fog Opacity" (Math|Float|Lerp 0.0 0.35 _sunrisesunset) :!class /Script/Engine.MaterialInstanceDynamic))))

(event Custom|SetNewTime
  (params (NewTime :type Integer))
  (bind _timesofday (Variables|Default|GetTimesOfDay))
  ;[1 1 1] Changing Time Of Day At Runtime
  (bind _output_get (Variables|Default|SetTime NewTime))
  (if (< _output_get (.Value (Utilities|Map|Find _timesofday "Sunrise")))
    ;;[1 1 1] Night
    (Rendering|Material|SetScalarParameterValue (Variables|Default|GetStarMaterial) "Opacity" 1.0 :!class /Script/Engine.MaterialInstanceDynamic)
    (Rendering|Material|SetScalarParameterValue (Variables|Default|GetFogMaterial) "Fog Opacity" 0.0 :!class /Script/Engine.MaterialInstanceDynamic)
    (Default|CallNewTimeOfDay)
    (elif (< _output_get (.Value (Utilities|Map|Find _timesofday "Day")))
      ;;[1 1 1] Sunrise
      (Rendering|Material|SetScalarParameterValue (Variables|Default|GetStarMaterial) "Opacity" 0.0 :!class /Script/Engine.MaterialInstanceDynamic)
      (Rendering|Material|SetScalarParameterValue (Variables|Default|GetFogMaterial) "Fog Opacity" 0.35 :!class /Script/Engine.MaterialInstanceDynamic)
      (Default|CallNewTimeOfDay 1)
      (elif (< _output_get (.Value (Utilities|Map|Find _timesofday "Sunset")))
        ;;[1 1 1] Day
        (Rendering|Material|SetScalarParameterValue (Variables|Default|GetStarMaterial) "Opacity" 0.0 :!class /Script/Engine.MaterialInstanceDynamic)
        (Rendering|Material|SetScalarParameterValue (Variables|Default|GetFogMaterial) "Fog Opacity" 0.0 :!class /Script/Engine.MaterialInstanceDynamic)
        (Default|CallNewTimeOfDay 2)
        (elif (< _output_get (.Value (Utilities|Map|Find _timesofday "Night")))
          ;;[1 1 1] Sunset
          (Rendering|Material|SetScalarParameterValue (Variables|Default|GetStarMaterial) "Opacity" 0.0 :!class /Script/Engine.MaterialInstanceDynamic)
          (Rendering|Material|SetScalarParameterValue (Variables|Default|GetFogMaterial) "Fog Opacity" 0.35 :!class /Script/Engine.MaterialInstanceDynamic)
          (Default|CallNewTimeOfDay 3)
          (else
            ;;[1 1 1] Night
            (Rendering|Material|SetScalarParameterValue (Variables|Default|GetStarMaterial) "Opacity" 1.0 :!class /Script/Engine.MaterialInstanceDynamic)
            (Rendering|Material|SetScalarParameterValue (Variables|Default|GetFogMaterial) "Fog Opacity" 0.0 :!class /Script/Engine.MaterialInstanceDynamic)
            (Default|CallNewTimeOfDay)))))))

(event EventTick
  (params (DeltaSeconds :type Float%20%28single-precision%29))
  (bind _returnvalue (Utilities|Time|GetRealTimeSeconds))
  (bind _returnvalue_2 (Utilities|Time|GetWorldDeltaSeconds))
  (bind _sunstartingrot (Variables|Default|GetSunStartingRot))
  (bind _fdaylengthmins (Variables|CycleSettings|GetFDayLengthMins))
  (bind _returnvalue_3 (/ 0.4 _fdaylengthmins))
  (bind (_roll _pitch _yaw) (Math|Rotator|BreakRotator _sunstartingrot))
  (bind _returnvalue_4 (* _returnvalue _returnvalue_3))
  (bind _returnvalue_5 (* _returnvalue_4 -15.0))
  (bind _returnvalue_6 (Math|Float|%(Float) _returnvalue_5 3.6e+02))
  (bind _returnvalue_7 (+ _pitch _returnvalue_6))
  (Transformation|SetActorRotation (Variables|Default|GetDirectionalLight) (Math|Rotator|MakeRotator _roll _returnvalue_7 _yaw))
  ;[1 1 1] Check if current time is near next transition state
  (bind _output_get (Variables|CycleSettings|SetFCurrentTime (Math|Float|Absolute(Float) (Math|Float|%(Float) (Math|Float|MapRangeUnclamped _returnvalue_7 0.0 -1.8e+02 (Variables|CycleSettings|GetFDayStartTime) (Variables|CycleSettings|GetFNightStartTime)) 24.0))))
  (Development|PrintString (Utilities|String|ToString(Float) _returnvalue_7) true true "(R=0.000000,G=0.660000,B=1.000000,A=1.000000)" _returnvalue_2)
  (Development|PrintString (Utilities|String|ToString(Float) _output_get) true true "(R=0.035759,G=1.000000,B=0.000000,A=1.000000)" _returnvalue_2)
  (if (Math|Float|NearlyEqual(Float) _output_get (Utilities|Select :Index (Variables|CycleSettings|GetNextTimeState) :NewEnumerator0 (Variables|CycleSettings|GetFSunriseTime) :NewEnumerator1 (Variables|CycleSettings|GetFDayStartTime) :NewEnumerator2 (Variables|CycleSettings|GetFSunsetTime) :NewEnumerator3 (Variables|CycleSettings|GetFNightStartTime)) 0.01)
    ;[1 1 1] Transition to next time state
    (switch Utilities|FlowControl|Switch|SwitchonEnum_TimeStates (Variables|CycleSettings|GetNextTimeState)
      (:NewEnumerator0
        (Development|PrintString "SUNRISE" true true "(R=1.000000,G=0.000000,B=0.889431,A=1.000000)")
        (CallFunction|Sunrise)
        (CallFunction|NightFadeOut)
        (Variables|CycleSettings|SetNextTimeState "NewEnumerator1"))
      (:NewEnumerator1
        (Development|PrintString "DAY" true true "(R=1.000000,G=0.000000,B=0.889431,A=1.000000)")
        (CallFunction|StopSunrise)
        (Variables|CycleSettings|SetNextTimeState "NewEnumerator2"))
      (:NewEnumerator2
        (Development|PrintString "SUNSET" true true "(R=1.000000,G=0.000000,B=0.889431,A=1.000000)")
        (CallFunction|Sunset)
        (Variables|CycleSettings|SetNextTimeState "NewEnumerator3"))
      (:NewEnumerator3
        (Development|PrintString "NIGHT" true true "(R=1.000000,G=0.000000,B=0.889431,A=1.000000)")
        (CallFunction|StopSunrise)
        (CallFunction|Night)
        (Variables|CycleSettings|SetNextTimeState "NewEnumerator0")))))

(event EventBeginPlay
  (bind _fcurrenttime (Variables|CycleSettings|GetFCurrentTime))
  (bind _directionallight (Variables|Default|GetDirectionalLight))
  (bind _fdaystarttime (Variables|CycleSettings|GetFDayStartTime))
  (bind _fnightstarttime (Variables|CycleSettings|GetFNightStartTime))
  (bind _shadertransitionspeed (Variables|Default|GetShaderTransitionSpeed))
  (bind _returnvalue (Transformation|GetActorRotation _directionallight))
  (bind _returnvalue_2 (Math|Float|MapRangeUnclamped _fcurrenttime _fdaystarttime _fnightstarttime 0.0 -1.8e+02))
  (bind (_roll _pitch _yaw) (Math|Rotator|BreakRotator _returnvalue))
  (bind _returnvalue_3 (Math|Rotator|MakeRotator _roll _returnvalue_2 _yaw))
  (Variables|Default|SetTime (Variables|Default|GetStartingTime))
  (Components|Timeline|SetPlayRate (Variables|Default|GetTimeline) _shadertransitionspeed)
  (Components|Timeline|SetPlayRate (Variables|Default|GetNightFade) (* _shadertransitionspeed 0.25))
  (bind _returnvalue_4 (Rendering|Material|CreateDynamicMaterialInstance (Variables|Default|GetStaticMesh) 0 "/Game/Materials/Sky/M_Procedural_Sky_Night.M_Procedural_Sky_Night" "None" :!class /Script/Engine.PrimitiveComponent))
  (Variables|Default|SetStarMaterial _returnvalue_4)
  (bind _returnvalue_5 (Rendering|Material|CreateDynamicMaterialInstance "/Game/Materials/PostProcessing/MI_Fog.MI_Fog" "None" "None" :!class /Script/Engine.KismetMaterialLibrary))
  (bind _output_get (Variables|Default|SetFogMaterial _returnvalue_5))
  (bind _output_get_2 (Variables|Default|SetFogWeightedBlendable (Utilities|Struct|MakeWeightedBlendable 1.0 _output_get)))
  (Utilities|Array|Add (Utilities|Struct|BreakWeightedBlendables (Utilities|Struct|BreakPostProcessSettings (Variables|/Script/Engine.PostProcessComponent|GetSettings (Variables|Default|GetPostProcess)))) _output_get_2)
  (CallFunction|StartTime)
  ;[1 1 1] Convert starting time to sun rotation
  (Transformation|SetActorRotation _directionallight _returnvalue_3)
  (Variables|Default|SetSunStartingRot _returnvalue_3)
  (Utilities|FlowControl|Sequence
    (:then_0
      ;[1 1 1] Set sunrise & sunset times
      (Variables|CycleSettings|SetFSunriseTime (- (Variables|CycleSettings|GetFDayStartTime) 1.0))
      (Variables|CycleSettings|SetFSunsetTime (- (Variables|CycleSettings|GetFNightStartTime) 1.0)))
    (:then_1
      (CallFunction|GetStartingNextState))))

(fn ConstructionScript
  (bind _fcurrenttime (Variables|CycleSettings|GetFCurrentTime))
  (bind _directionallight (Variables|Default|GetDirectionalLight))
  (bind _returnvalue (Transformation|GetActorRotation _directionallight))
  (bind _returnvalue_2 (Math|Float|MapRangeUnclamped _fcurrenttime 6.0 18.0 0.0 -1.8e+02))
  (bind (_roll _pitch _yaw) (Math|Rotator|BreakRotator _returnvalue))
  (Transformation|SetActorRotation _directionallight (Math|Rotator|MakeRotator _roll _returnvalue_2 _yaw))
  (Development|PrintString (Utilities|String|ToString(Float) (Math|Float|Absolute(Float) _returnvalue_2))))

(fn GetStartingNextState
  (bind (_array_element _array_index) (Utilities|Array|ForEachLoopwithBreak (Utilities|Array|MakeArray (Variables|CycleSettings|GetFSunriseTime) (Variables|CycleSettings|GetFDayStartTime) (Variables|CycleSettings|GetFSunsetTime) (Variables|CycleSettings|GetFNightStartTime)) :!label _label)
    (:LoopBody
      (if (or (< (- (Variables|CycleSettings|GetFCurrentTime) _array_element) 0.0) (>= (- (Variables|CycleSettings|GetFCurrentTime) _array_element) 12.0))
        (bind _output_get (Variables|CycleSettings|SetNextTimeState (Utilities|Select :Index _array_index :Option%200 "NewEnumerator0" :Option%201 "NewEnumerator1" :Option%202 "NewEnumerator2" :Option%203 "NewEnumerator3")))
        (Development|PrintString (Utilities|String|EnumtoString _output_get) true true "(R=1.000000,G=0.080943,B=0.000000,A=1.000000)" 1e+01)
        (goto _label Break)))))