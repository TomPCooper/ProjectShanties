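; BP_Current is a water current manager that pushes the player ship sideways with a constant impulse.
; BeginPlay caches the Pawn_ShipFinal after a short delay, and Tick applies a velocity-change impulse along negative world Y to its boat mesh while IsCurrentOn is true.
; The logic that enables the current and sets MPC_WaterParameters flow speeds is disconnected, the box overlap is empty, and the interface functions are stubs.
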(event OnComponentBeginOverlap(Box)
  (params (OverlappedComponent :type Primitive%20Component%20Object%20Reference) (OtherActor :type Actor%20Object%20Reference) (OtherComp :type Primitive%20Component%20Object%20Reference) (OtherBodyIndex :type Integer) (bFromSweep :type Boolean) (SweepResult :type Hit%20Result%20Structure%20%28by%20ref%29)))

(event EventTick
  (params (DeltaSeconds :type Float%20%28single-precision%29))
  (if (Variables|Default|GetisCurrentOn)
    (Physics|AddImpulse (Variables|/Game/Blueprints/Ship/Pawn_ShipFinal.Pawn_ShipFinal_C|GetSM_Boat (Variables|Default|GetShip)) "0.000000,-50.000000,0.000000" "None" true)))

(event EventBeginPlay
  (Utilities|FlowControl|Delay 0.2)
  (bind _returnvalue (Actor|GetActorOfClass "/Game/Blueprints/Ship/Pawn_ShipFinal.Pawn_ShipFinal_C"))
  (Variables|Default|SetShip _returnvalue))

(fn ConstructionScript)

(fn IBossGetLeapPosition
  (return "0, 0, 0"))

(fn IGetCamera
  (return 0))

(fn IGetShipMesh
  (return 0))

(fn IGetShipVelocity
  (return "0, 0, 0"))