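; BP_TaskManager shows the current task text on screen for the active quest, such as Tutorial, Megalodon, Kracken, Mo O Nui or General.
; On BeginPlay it creates a UI_Task widget for the first player controller, adds it to the viewport and shows task 0.
; UpdateQuest sets the active quest, while UpdateTask indexes that quest's task list and passes the entry to the widget through UpdateText.
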(event Custom|UpdateQuest
  (params (NewQuest :type E_Quests%20Enum :default "NewEnumerator0"))
  (Variables|Default|SetCurrentQuest NewQuest))

(event Custom|UpdateTask
  (params (NewTaskNum :type Integer))
  (switch Utilities|FlowControl|Switch|SwitchonE_Quests (Variables|Default|GetCurrentQuest)
    (:NewEnumerator0
      (CallFunction|UpdateText (Utilities|Array|Get(acopy) (Variables|Default|GetTutorialQuests) NewTaskNum)))
    (:NewEnumerator1
      (CallFunction|UpdateText (Utilities|Array|Get(acopy) (Variables|Default|GetMegalodonQuests) NewTaskNum)))
    (:NewEnumerator2
      (CallFunction|UpdateText (Utilities|Array|Get(acopy) (Variables|Default|GetKrackenQuests) NewTaskNum)))
    (:NewEnumerator3
      (CallFunction|UpdateText (Utilities|Array|Get(acopy) (Variables|Default|GetMoONuiQuests) NewTaskNum)))
    (:NewEnumerator4
      (CallFunction|UpdateText (Utilities|Array|Get(acopy) (Variables|Default|GetGeneralGameplay) NewTaskNum)))))

(event Custom|UpdateText
  (params (Quest :type String))
  (Default|UpdateText (Variables|Default|GetUI) Quest))

(event EventBeginPlay
  (bind _returnvalue (UserInterface|CreateWidget "/Game/Blueprints/UI/HUD/UI_Task.UI_Task_C" (Game|GetPlayerController 0)))
  (bind _output_get (Variables|Default|SetUI _returnvalue))
  (UserInterface|Viewport|AddtoViewport _output_get 0)
  (CallFunction|UpdateTask))

(fn ConstructionScript)