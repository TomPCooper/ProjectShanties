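; BP_KrakenSpawnCol is a trigger volume that starts the Kraken boss message when a ship enters it.
; On BeginPlay it finds and caches the BP_KrakenSpawnLoc actor in the level.
; The first box overlap by an actor implementing BPI_Ship calls IActivateBossMessage on that spawn actor, gated by a DoOnce.
; The construction script sizes the box from an extent variable.
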(event OnComponentBeginOverlap(Box)
  (params (OverlappedComponent :type Primitive%20Component%20Object%20Reference) (OtherActor :type Actor%20Object%20Reference) (OtherComp :type Primitive%20Component%20Object%20Reference) (OtherBodyIndex :type Integer) (bFromSweep :type Boolean) (SweepResult :type Hit%20Result%20Structure%20%28by%20ref%29))
  (if (Utilities|DoesObjectImplementInterface OtherActor "/Game/Blueprints/Ship/BPI_Ship.BPI_Ship_C")
    (Utilities|FlowControl|DoOnce false
      (:Completed
        (Class|BPIKraken|IActivateBoss(Message) (Variables|Default|GetKrakenSpawnRef))))))

(event EventBeginPlay
  (bind _returnvalue (Actor|GetActorOfClass "/Game/Blueprints/Bosses/Kracken/BP_KrakenSpawnLoc.BP_KrakenSpawnLoc_C"))
  (Variables|Default|SetKrakenSpawnRef _returnvalue))

(fn ConstructionScript
  (Components|Box|SetBoxExtent (Variables|Default|GetBox) (Variables|Default|GetIn%20Box%20Extent) true))