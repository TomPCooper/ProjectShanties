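; Kraken boss spike hazard that rises from the ground or water to damage ships during a spike attack.
; The ISpikeAttackMove event runs a timeline that lerps the spike upward from its current location, then snaps it back to the storage location saved at BeginPlay.
; Overlaps on DamageCol send damage through BPI_Ship, gated by a DoOnce that resets when each rise finishes.
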(event OnComponentBeginOverlap(DamageCol)
  (params (OverlappedComponent :type Primitive%20Component%20Object%20Reference) (OtherActor :type Actor%20Object%20Reference) (OtherComp :type Primitive%20Component%20Object%20Reference) (OtherBodyIndex :type Integer) (bFromSweep :type Boolean) (SweepResult :type Hit%20Result%20Structure%20%28by%20ref%29))
  (if (Utilities|DoesObjectImplementInterface OtherActor "/Game/Blueprints/Ship/BPI_Ship.BPI_Ship_C")
    (Utilities|FlowControl|DoOnce false
      (:Completed
        (Class|BPIShip|IDamageShip(Message) OtherActor 4e+01)))))

(event EventISpikeAttackMove
  (bind _output_get (Variables|Default|SetStartLocation (Transformation|GetActorLocation)))
  (Variables|Default|SetEndLocation (+ _output_get "0.000000,0.000000,700.000000"))
  (bind _alpha (Timeline|RaiseSpike PlayFromStart)
    (:Update
      (Transformation|SetActorLocation (Math|Vector|Lerp(Vector) (Variables|Default|GetStartLocation) (Variables|Default|GetEndLocation) _alpha) false false))
    (:Finished
      (Transformation|SetActorLocation (Variables|Default|GetStorageLocation) false false)
      (Utilities|FlowControl|DoOnce false) ; enters at Reset
    )))

(event EventBeginPlay
  (Variables|Default|SetStorageLocation (Transformation|GetActorLocation)))

(fn ConstructionScript)