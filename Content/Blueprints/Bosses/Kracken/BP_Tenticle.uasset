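; Kraken boss tentacle actor that builds its body procedurally along a spline in the construction script.
; When Build is on, it chains spline mesh segments of SectionLength, oriented by ForwardAxis, with tangents taken from spline direction scaled by TangentSmooth.
; A second pass adds EndMesh as another spline mesh component at the last section boundary, aligned to the spline's rotation.
; A leftover debug print fires for each body segment.
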(fn ConstructionScript
  (bind _spline (Variables|Components|GetSpline))
  (bind _spline_2 (Variables|Components|GetSpline))
  (bind _spline_3 (Variables|Components|GetSpline))
  (bind _sectionlength (Variables|Default|GetSectionLength))
  (bind _sectionlength_2 (Variables|Default|GetSectionLength))
  (bind _returnvalue (Spline|GetSplineLength _spline_2))
  (bind _returnvalue_2 (Math|Float|Division(WholeandRemainder) _returnvalue _sectionlength_2))
  (if (Variables|Default|GetBuild?)
    (for _index (range 0 (.ReturnValue (Math|Float|Division(WholeandRemainder) (Spline|GetSplineLength _spline) (Variables|Default|GetSectionLength))))
      (bind _returnvalue_3 (AddComponent|AddSplineMeshComponent false))
      (Utilities|Array|Add (Variables|Default|GetMeshes) _returnvalue_3)
      (Components|StaticMesh|SetStaticMesh _returnvalue_3 (Variables|Default|GetSplinedObject))
      (SplineMesh|SetForwardAxis _returnvalue_3 (Variables|Default|GetForwardAxis) true)
      (SplineMesh|SetStartandEnd _returnvalue_3 (Spline|GetLocationatDistanceAlongSpline _spline (* _index _sectionlength) "Local") (* (Spline|GetDirectionatDistanceAlongSpline _spline (* _index _sectionlength) "Local") (Variables|Default|GetTangentSmooth)) (Spline|GetLocationatDistanceAlongSpline _spline (+ (* _index _sectionlength) _sectionlength) "Local") (* (Spline|GetDirectionatDistanceAlongSpline _spline (+ (* _index _sectionlength) _sectionlength) "Local") (Variables|Default|GetTangentSmooth)) true :!class /Script/Engine.SplineMeshComponent)
      (Development|PrintString "Hello"))
    (for _index_2 (range 0 _returnvalue_2)
      (if (== _index_2 _returnvalue_2)
        (bind _returnvalue_4 (AddComponent|AddSplineMeshComponent false (Math|Transform|MakeTransform (Spline|GetLocationatDistanceAlongSpline _spline_3 (* _index_2 (Variables|Default|GetSectionLength)) "Local") (Spline|GetRotationatDistanceAlongSpline _spline_3 (* _index_2 (Variables|Default|GetSectionLength)) "Local"))))
        (Components|StaticMesh|SetStaticMesh _returnvalue_4 (Variables|Default|GetEndMesh))))))