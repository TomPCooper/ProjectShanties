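; Kraken boss that, once activated, spawns a whirlpool, spike and four pooled tentacles, then fights the player's ship.
; Timers drive spike and tentacle attacks, plus a consume attack when the player lines up with an unbroken pillar.
; Consume tilts the Kraken up and alters whirlpool pull, and mouth contact damages and repels the ship.
; Destroyed pillars interrupt consume and damage the boss, with timelines animating bobbing, rotation and hit reaction.
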(event OnComponentBeginOverlap(MouthCol)
  (params (OverlappedComponent :type Primitive%20Component%20Object%20Reference) (OtherActor :type Actor%20Object%20Reference) (OtherComp :type Primitive%20Component%20Object%20Reference) (OtherBodyIndex :type Integer) (bFromSweep :type Boolean) (SweepResult :type Hit%20Result%20Structure%20%28by%20ref%29))
  (if (Utilities|DoesObjectImplementInterface OtherActor "/Game/Blueprints/Ship/BPI_Ship.BPI_Ship_C")
    (Utilities|FlowControl|DoOnce false
      (:Completed
        (Class|BPIShip|IDamageShip(Message) OtherActor 8e+01)
        (Class|BPIShip|IAddImpulsetoShip(Message) OtherActor (* (Math|Vector|GetUnitDirection(Vector) (Transformation|GetWorldLocation (Variables|Default|GetMouthCol)) (Transformation|GetActorLocation OtherActor)) 2e+04))
        (CallFunction|EndConsumeAttack)
        (Utilities|Time|SetTimerbyEvent (delegate Custom|ResetMouthDamage) 2.0)
        (Development|PrintString "DAMAGING SHIP MOUTH")))))

(event Custom|SelectNextAttack
  (bind _returnvalue (Transformation|GetActorLocation))
  (bind _playerref (Variables|Default|GetPlayerRef))
  (bind _returnvalue_2 (Transformation|GetActorLocation _playerref))
  (bind _returnvalue_3 (Math|Rotator|FindLookatRotation _returnvalue _returnvalue_2))
  (bind _returnvalue_4 (Math|Float|Absolute(Float) (.yaw _returnvalue_3)))
  (if (not (or (Math|Float|InRange(Float) _returnvalue_4 0.0 45.0 false false) (Math|Float|InRange(Float) _returnvalue_4 135.0 1.8e+02 false false)))
    (CallFunction|SpikeAttack)
    (Variables|Default|SetAttackCooldown 5.5)
    (CallFunction|StartNextAttackTimer)))

(event Custom|ConsumeCooldown
  (Variables|Default|SetIsConsumeOnCooldown? false)
  (bind _returnvalue (Utilities|Time|SetTimerbyEvent (EventDispatchers|CreateEvent :!event Custom|CheckifConsume) 0.5 true))
  (Variables|Default|SetConsumeCheckHandle _returnvalue))

(event Custom|PullShipToKraken
  (Variables|/Game/Blueprints/Water/BP_Whirlpool.BP_Whirlpool_C|SetCentrePullStrength (Variables|Default|GetWhirlpoolRef) (Math|Float|Clamp(Float) (+ (Variables|Default|GetConsumePullStrength) 2.0) 2e+02 1.5e+03))
  (Class|BPIShip|IAddForcetoShip(Message) (Variables|Default|GetPlayerRef) (* (Math|Vector|GetUnitDirection(Vector) (Transformation|GetActorLocation (Variables|Default|GetPlayerRef)) (Transformation|GetWorldLocation (Variables|Default|GetPullLocation))) ""))
  (Development|PrintString (Utilities|String|ToString(Float) 0.0) false))

(event Custom|EndConsumeAttack
  ;[1 1 1] Reset consume cooldown
  (Class|BPIKraken|IUnInitPillar(Message) (Utilities|Array|Get(acopy) (Variables|Default|GetPillarRefs) (Variables|Default|GetCurrentPillarIndex)))
  (Utilities|Time|ClearandInvalidateTimerbyHandle (Variables|Default|GetPullShipHandle))
  (Variables|/Game/Blueprints/Water/BP_Whirlpool.BP_Whirlpool_C|SetCentrePullStrength (Variables|Default|GetWhirlpoolRef) 2e+02)
  (Variables|Default|SetIsConsumeOnCooldown? true)
  (CallFunction|StartConsumeCooldown)
  (CallFunction|RotateKrakenDown)
  (Variables|Default|SetAttackCooldown 4.0)
  (CallFunction|SelectNextAttack))

(event Custom|StopConsume
  (Utilities|Time|ClearandInvalidateTimerbyHandle (Variables|Default|GetPullShipHandle)))

(event Custom|RotateKrakenDown
  (bind _alpha (Timeline|RotateKraken ReverseFromEnd)
    (:Update
      (Transformation|SetRelativeRotation (Variables|Default|GetScene) (Math|Rotator|MakeRotator 0.0 (Math|Float|Lerp -4e+01 2e+01 _alpha) (.yaw (Variables|/Script/Engine.SceneComponent|GetRelativeRotation (Variables|Default|GetScene)))) false false))))

(event Custom|RotateKrakenUp
  (bind _alpha (Timeline|RotateKraken PlayFromStart)
    (:Update
      (Transformation|SetRelativeRotation (Variables|Default|GetScene) (Math|Rotator|MakeRotator 0.0 (Math|Float|Lerp -4e+01 2e+01 _alpha) (.yaw (Variables|/Script/Engine.SceneComponent|GetRelativeRotation (Variables|Default|GetScene)))) false false))))

(event Custom|ResetMouthDamage
  (Utilities|FlowControl|DoOnce false) ; enters at Reset
)

(event Custom|StartBobbing
  (bind _alpha (Timeline|BobKraken Play)
    (:Update
      (Transformation|SetRelativeLocation (Variables|Default|GetScene) (Math|Vector|Lerp(Vector) "0.000000,0.000000,-80.000000" "0.000000,0.000000,80.000000" _alpha) false false))))

(event Custom|StopBobbing
  (bind _alpha (Timeline|BobKraken Stop)
    (:Update
      (Transformation|SetRelativeLocation (Variables|Default|GetScene) (Math|Vector|Lerp(Vector) "0.000000,0.000000,-80.000000" "0.000000,0.000000,80.000000" _alpha) false false))))

(event Custom|SendTentacleOut
  (bind _returnvalue (Transformation|GetActorLocation))
  (bind _returnvalue_2 (+ _returnvalue ""))
  ;[1 1 1] Start tentacle attack
  (bind _result (Math|Integer|IncrementInt (Variables|Default|GetCurrentTentacleInt))
    (:%20%20
      (bind _output_get (Variables|Default|SetTentacleSpawnLoc (Math|Vector|MakeVector (.x _returnvalue_2) (.y _returnvalue_2) (- (.z _returnvalue_2) 3e+03))))
      (bind _output_get_2 (Variables|Default|SetCurrentTentacle (Utilities|Array|Get(acopy) (Variables|Default|GetTentacleRefs) (Math|Integer|%(Integer) _result 4))))
      (Transformation|SetActorLocationAndRotation _output_get_2 _output_get (Math|Rotator|MakeRotator 0.0 0.0 (+ 0.0 (Utilities|Select :Index (Math|Integer|%(Integer) _result 4) :Option%200 (Math|Random|RandomFloatinRange -45.0 45.0) :Option%201 (Math|Random|RandomFloatinRange 1.5e+02 1.8e+02) :Option%202 (Math|Random|RandomFloatinRange -45.0 45.0) :Option%203 (Math|Random|RandomFloatinRange -1.8e+02 -1.5e+02)))))
      (bind _alpha (Timeline|TentacleStartTimeline PlayFromStart)
        (:Update
          (Transformation|SetActorLocation (Variables|Default|GetCurrentTentacle) (Math|Vector|Lerp(Vector) (Variables|Default|GetTentacleSpawnLoc) (+ (+ (Variables|Default|GetTentacleSpawnLoc) "0.000000,0.000000,1400.000000") (* (Transformation|GetActorForwardVector (Variables|Default|GetCurrentTentacle)) 4e+02)) _alpha) false false))
        (:Finished
          (CallFunction|SendTentacleForward))))))

(event Custom|StartNextAttackTimer
  (bind _returnvalue (Utilities|Time|SetTimerbyEvent (delegate Custom|SelectNextAttack) (Variables|Default|GetAttackCooldown)))
  (Variables|Default|SetAttackSelectHandle _returnvalue)
  (bind _returnvalue_2 (Utilities|Time|SetTimerbyEvent (EventDispatchers|CreateEvent :!event Custom|SendTentacleOut) 2.2 true))
  (Variables|Default|SetTentacleTimer _returnvalue_2))

(event Custom|SpikeAttack
  (bind _playerref (Variables|Default|GetPlayerRef))
  (bind _playerref_2 (Variables|Default|GetPlayerRef))
  (bind _returnvalue (Transformation|GetActorLocation _playerref))
  (bind _returnvalue_2 (Transformation|GetActorLocation _playerref_2))
  ;[1 1 1] Start spike attack
  (Transformation|SetActorLocation (Variables|Default|GetSpikeRef) (Math|Vector|MakeVector (.x _returnvalue) (.y _returnvalue) -6e+02) false false)
  (Timeline|SpikeStartTime PlayFromStart
    (:Update
      (Transformation|SetActorLocation (Variables|Default|GetSpikeRef) (Math|Vector|MakeVector (.x _returnvalue_2) (.y _returnvalue_2) -6e+02) false false))
    (:Finished
      (CallFunction|SendSpikeUpwards)
      (Development|PrintString "Spike attack!" true true "(R=1.000000,G=0.078311,B=0.000000,A=1.000000)"))))

(event Custom|CheckifConsume
  (if (not (Variables|Default|GetIsConsumeOnCooldown?))
    (Development|PrintString "checking consume" true true "(R=1.000000,G=0.159335,B=0.000000,A=1.000000)" 5.0)
    (bind (_array_element _array_index) (Utilities|Array|ForEachLoopwithBreak (Variables|Default|GetUnBrokenPillarAngles) :!label _label)
      (:LoopBody
        (Development|PrintString (Utilities|String|ToString(Float) _array_element) false)
        (if (Math|Float|NearlyEqual(Float) (.yaw (Math|Rotator|FindLookatRotation (Transformation|GetActorLocation) (Transformation|GetActorLocation (Variables|Default|GetPlayerRef)))) _array_element 15.0)
          (bind _output_get (Variables|Default|SetCurrentPillarIndex _array_index))
          (CallFunction|ConsumeAttack _array_element)
          (Class|BPIKraken|IInitPillar(Message) (Utilities|Array|Get(acopy) (Variables|Default|GetPillarRefs) _output_get) _output_get)
          (Utilities|Time|ClearandInvalidateTimerbyHandle (Variables|Default|GetConsumeCheckHandle))
          (Variables|Default|SetIsConsumeOnCooldown? true)
          (Development|PrintString "Started consume!" true true "(R=0.000000,G=1.000000,B=0.093073,A=1.000000)")
          (goto _label Break))))))

(event Custom|ConsumeAttack
  (params (AttackAngle :type Float%20%28double-precision%29))
  (bind _returnvalue (Utilities|Time|SetTimerbyEvent (delegate Custom|PullShipToKraken) (Utilities|Time|GetWorldDeltaSeconds) true))
  (Variables|Default|SetPullShipHandle _returnvalue)
  (CallFunction|RotateKrakenUp)
  (Utilities|Time|ClearandInvalidateTimerbyHandle (Variables|Default|GetAttackSelectHandle))
  (Utilities|Time|ClearandInvalidateTimerbyHandle (Variables|Default|GetTentacleTimer)))

(event Custom|SendSpikeUpwards
  ;[1 1 1] Start spike attack
  (Class|BPIKraken|ISpikeAttackMove(Message) (Variables|Default|GetSpikeRef)))

(event Custom|SendTentacleForward
  ;[1 1 1] Start tentacle attack
  (Class|BPIKraken|IStartTentacle(Message) (Variables|Default|GetCurrentTentacle))
  (Development|PrintString "tentacle attack!" true true "(R=1.000000,G=0.078311,B=0.000000,A=1.000000)"))

(event Custom|StartConsumeCooldown
  (Utilities|Time|SetTimerbyEvent (delegate Custom|ConsumeCooldown) (Variables|Default|GetConsumeCooldownTime)))

(event EventBeginPlay)

(event EventIPillarDestroyed
  (params (PillarIndex :type Integer))
  (bind _scene (Variables|Default|GetScene))
  (bind _head (Variables|Default|GetHead))
  (bind _returnvalue (Transformation|GetWorldLocation _head))
  (CallFunction|StopConsume)
  (Utilities|Array|RemoveIndex (Variables|Default|GetPillarRefs) PillarIndex)
  (Utilities|Array|RemoveIndex (Variables|Default|GetUnBrokenPillarAngles) (Variables|Default|GetCurrentPillarIndex))
  (CallFunction|StopBobbing)
  (Variables|Default|SetStartRelLoc (Variables|/Script/Engine.SceneComponent|GetRelativeLocation _scene))
  (Utilities|FlowControl|Delay 2.8)
  (Variables|Default|SetStartRelRot (Variables|/Script/Engine.SceneComponent|GetRelativeRotation _scene))
  (Utilities|FlowControl|Sequence
    (:then_0
      (Audio|PlaySoundatLocation "/Game/c013265l/Audio/Kraken/Pillars/krakenhitgrowl.krakenhitgrowl" _returnvalue "0, 0, 0" 5.0 1.0 0.0 "/Game/c013265l/Audio/Kraken/Pillars/SA_BreathKraken.SA_BreathKraken" 0 0 0))
    (:then_1
      (Audio|PlaySoundatLocation "/Game/c013265l/Audio/Kraken/Pillars/ColumnFall1.ColumnFall1" _returnvalue "0, 0, 0" 0.8 1.0 0.0 0 0 0 0)
      (Class|BPIHealth|IDamage(Message) (Variables|Default|GetBPC_Health) 1e+02)
      (bind _alpha (Timeline|KrakenHitByPillar PlayFromStart)
        (:Update
          (Transformation|SetRelativeLocationAndRotation (Variables|Default|GetScene) (Math|Vector|Lerp(Vector) (Variables|Default|GetStartRelLoc) "0.000000,-50.000000,-400.000000" _alpha) (Math|Rotator|Lerp(Rotator) (Variables|Default|GetStartRelRot) "20.000000,0.000000,0.000000" 0.0) false false))
        (:Finished
          (CallFunction|EndConsumeAttack)
          (Development|PrintString "Pillar gone" true true "(R=1.000000,G=0.317743,B=0.000000,A=1.000000)")
          (if (Utilities|Array|IsEmpty (Variables|Default|GetUnBrokenPillarAngles))
            (Development|PrintString "DEADDDDD" true true "(R=1.000000,G=0.008681,B=0.000000,A=1.000000)")
            (else
              (CallFunction|StartBobbing))))))))

(event EventIActivateBoss
  (bind _returnvalue (Transformation|GetActorTransform))
  (bind _returnvalue_2 (Transformation|GetActorTransform))
  (bind _returnvalue_3 (Transformation|GetActorTransform))
  (Variables|Default|SetPlayerRef (Game|Player|GetPlayerPawn 0))
  (bind _returnvalue_4 (Game|SpawnActorfromClass "/Game/Blueprints/Water/BP_Whirlpool.BP_Whirlpool_C" (Math|Transform|MakeTransform (Math|Vector|MakeVector (.x (.location _returnvalue_3)) (.y (.location _returnvalue_3)) 0.0) (.rotation _returnvalue_3) (.scale _returnvalue_3)) "Undefined" "MultiplyWithRoot" 0 5.0 5.0 5e+02 1e+03 "100.000000,100.000000,2.000000" 0))
  (Variables|Default|SetWhirlpoolRef _returnvalue_4)
  (bind _returnvalue_5 (Game|SpawnActorfromClass "/Game/Blueprints/Bosses/Kracken/BP_Spike.BP_Spike_C" (Math|Transform|MakeTransform (- (.location _returnvalue) "0.000000,0.000000,20000.000000") (.rotation _returnvalue) (.scale _returnvalue)) "Undefined" "MultiplyWithRoot" 0 0))
  (Variables|Default|SetSpikeRef _returnvalue_5)
  (for _index (range 0 3)
    (bind _returnvalue_6 (Game|SpawnActorfromClass "/Game/Blueprints/Bosses/Kracken/BP_TentacleStatic.BP_TentacleStatic_C" (Math|Transform|MakeTransform (- (.location _returnvalue_2) "0.000000,0.000000,20000.000000") (.rotation _returnvalue_2) (.scale _returnvalue_2)) "Undefined" "MultiplyWithRoot" 0 0))
    (Utilities|Array|Add (Variables|Default|GetTentacleRefs) _returnvalue_6))
  (bind _outactors (Actor|GetAllActorsOfClass "/Game/Blueprints/Bosses/Kracken/BP_Pillar.BP_Pillar_C"))
  (bind _output_get (Variables|Default|SetPillarRefs _outactors))
  (for _array_element _output_get
    (Utilities|Array|Add (Variables|Default|GetUnBrokenPillarAngles) (.yaw (Math|Rotator|FindLookatRotation (Transformation|GetActorLocation) (Transformation|GetActorLocation _array_element))))
    (Utilities|FlowControl|Sequence
      (:then_0
        (bind _alpha (Timeline|BobKraken Play)
          (:Update
            (Transformation|SetRelativeLocation (Variables|Default|GetScene) (Math|Vector|Lerp(Vector) "0.000000,0.000000,-80.000000" "0.000000,0.000000,80.000000" _alpha) false false))))
      (:then_1
        (CallFunction|StartNextAttackTimer))
      (:then_2
        (CallFunction|StartConsumeCooldown))
      (:then_3
        (bind _returnvalue_7 (Audio|SpawnSoundatLocation "/Game/c013265l/Audio/Kraken/Pillars/SC_Breath.SC_Breath" (Transformation|GetWorldLocation (Variables|Default|GetHead)) "0, 0, 0" 0.8 1.0 0.0 "/Game/c013265l/Audio/Kraken/Pillars/SA_BreathKraken.SA_BreathKraken" 0))
        (Variables|Default|SetBreathSound _returnvalue_7)))))

(event EventTick
  (params (DeltaSeconds :type Float%20%28single-precision%29)))

(fn ConstructionScript)