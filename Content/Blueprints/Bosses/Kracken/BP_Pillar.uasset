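; Collapsible pillar for the Kraken boss fight that the boss is notified about when it is pulled down.
; Interface calls supply the Kraken reference and arm or disarm the pillar, toggling capsule queries and playing or reversing a slight lean.
; When pulled while armed, it reports its index to the Kraken, topples further from the leaning rotation, then sinks and destroys itself, all timeline-driven.
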(event Custom|ReverseInitialAngle
  (bind _startrot (Variables|Default|GetStartRot))
  (bind (_roll _pitch _yaw) (Math|Rotator|BreakRotator _startrot))
  (bind (_direction _alpha) (Timeline|Timeline Reverse)
    (:Update
      (Transformation|SetActorRotation (Math|Rotator|Lerp(Rotator) _startrot (Math|Rotator|MakeRotator _roll (- _pitch 1e+01) _yaw) _alpha)))
    (:Finished
      (switch Utilities|FlowControl|Switch|SwitchonETimelineDirection _direction
        (:Forward
          (Variables|Default|SetStartRotCollapse (Transformation|GetActorRotation)))))))

(event EventIActorPulled
  (bind _startrotcollapse (Variables|Default|GetStartRotCollapse))
  (bind (_roll _pitch _yaw) (Math|Rotator|BreakRotator _startrotcollapse))
  (if (Variables|Default|GetCanBePulled?)
    (Audio|PlaySoundatLocation "/Game/c013265l/Audio/Kraken/Pillars/ColumnFall1.ColumnFall1" (Transformation|GetActorLocation (Variables|Default|GetKrakenRef)) "0, 0, 0" 1.0 1.0 0.1 0 0 0 0)
    (Class|BPIKraken|IPillarDestroyed(Message) (Variables|Default|GetKrakenRef) (Variables|Default|GetPillarIndex))
    (bind _alpha (Timeline|Rotate PlayFromStart)
      (:Update
        (Transformation|SetActorRotation (Math|Rotator|Lerp(Rotator) _startrotcollapse (Math|Rotator|MakeRotator _roll (- _pitch 45.0) _yaw) _alpha)))
      (:Finished
        (Variables|Default|SetStartLoc (Transformation|GetActorLocation))
        (bind _alpha_2 (Timeline|RemovePillar Play)
          (:Update
            (Transformation|SetActorLocation (Math|Vector|Lerp(Vector) (Variables|Default|GetStartLoc) (- (Variables|Default|GetStartLoc) "0.000000,0.000000,3000.000000") _alpha_2) false false))
          (:Finished
            (Actor|DestroyActor)))))))

(event EventIInitPillar
  (params (Index :type Integer))
  (bind _startrot (Variables|Default|GetStartRot))
  (bind (_roll _pitch _yaw) (Math|Rotator|BreakRotator _startrot))
  (Variables|Default|SetCanBePulled? true)
  (Audio|PlaySoundatLocation "/Game/c013265l/Audio/Kraken/Pillars/Pillarcollapsestart_mixdown.Pillarcollapsestart_mixdown" (Transformation|GetActorLocation) "0, 0, 0" 1.0 1.0 0.0 0 0 0 0)
  (bind _output_get (Variables|Default|SetPillarIndex Index))
  (Collision|SetCollisionEnabled (Variables|Default|GetCapsule) "QueryOnly")
  (bind (_direction _alpha) (Timeline|Timeline Play)
    (:Update
      (Transformation|SetActorRotation (Math|Rotator|Lerp(Rotator) _startrot (Math|Rotator|MakeRotator _roll (- _pitch 1e+01) _yaw) _alpha)))
    (:Finished
      (switch Utilities|FlowControl|Switch|SwitchonETimelineDirection _direction
        (:Forward
          (Variables|Default|SetStartRotCollapse (Transformation|GetActorRotation)))))))

(event EventIStartPillarCollapse
  (Rendering|Material|SetMaterial (Variables|Default|GetPillarMesh) 0 "/Game/Meshes/Foliage/Cactus/01_-_Default.01_-_Default"))

(event EventBeginPlay
  (Variables|Default|SetStartRot (Transformation|GetActorRotation))
  (Collision|SetCollisionEnabled (Variables|Default|GetCapsule) "NoCollision"))

(event EventIUnInitPillar
  (Variables|Default|SetCanBePulled? false)
  (Collision|SetCollisionEnabled (Variables|Default|GetCapsule) "NoCollision")
  (CallFunction|ReverseInitialAngle))

(event EventIActivateBoss
  (params (KrakenRef :type Actor%20Object%20Reference))
  (Variables|Default|SetKrakenRef KrakenRef))

(fn ConstructionScript
  (Components|StaticMesh|SetStaticMesh (Variables|Default|GetPillarMesh) (Variables|Default|GetPillarMeshTarget)))

(fn IGetMeshReference
  (return 0))