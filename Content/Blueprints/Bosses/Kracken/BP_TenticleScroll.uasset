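; Kraken boss tentacle actor that animates a repeated mesh scrolling along a spline.
; BeginPlay creates spline mesh components from SplinedObject according to spline length and SectionLength, then starts a Timeline with play rate inverse to MovementSpeed.
; Each update slides every segment forward by up to spline length over mesh count, with tangents scaled by TangentSmooth.
; The Timeline restarts on finish, looping this roughly one-section shift like a conveyor.
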(event Custom|PlayTimeline
  (bind _sectionlength (Variables|Default|GetSectionLength))
  (bind _spline (Variables|Default|GetSpline))
  (bind _newtrack_0 (Timeline|Timeline PlayFromStart)
    (:Update
      (for _index (range 0 (.ReturnValue (Math|Float|Division(WholeandRemainder) (Spline|GetSplineLength (Variables|Default|GetSpline)) (Variables|Default|GetSectionLength))))
        (SplineMesh|SetStartandEnd (Utilities|Array|Get(acopy) (Variables|Default|GetMeshes) _index) (Spline|GetLocationatDistanceAlongSpline _spline (+ (* _index _sectionlength) (Math|Float|Lerp 0.0 (/ (Spline|GetDistanceAlongSplineatSplinePoint (Variables|Default|GetSpline) (- (Spline|GetNumberOfSplinePoints (Variables|Default|GetSpline)) 1)) (Utilities|Array|Length (Variables|Default|GetMeshes))) _newtrack_0)) "Local") (* (Spline|GetDirectionatDistanceAlongSpline _spline (+ (* _index _sectionlength) (Math|Float|Lerp 0.0 (/ (Spline|GetDistanceAlongSplineatSplinePoint (Variables|Default|GetSpline) (- (Spline|GetNumberOfSplinePoints (Variables|Default|GetSpline)) 1)) (Utilities|Array|Length (Variables|Default|GetMeshes))) _newtrack_0)) "Local") (Variables|Default|GetTangentSmooth)) (Spline|GetLocationatDistanceAlongSpline _spline (+ (+ (* _index _sectionlength) (Math|Float|Lerp 0.0 (/ (Spline|GetDistanceAlongSplineatSplinePoint (Variables|Default|GetSpline) (- (Spline|GetNumberOfSplinePoints (Variables|Default|GetSpline)) 1)) (Utilities|Array|Length (Variables|Default|GetMeshes))) _newtrack_0)) _sectionlength) "Local") (* (Spline|GetDirectionatDistanceAlongSpline _spline (+ (+ (* _index _sectionlength) (Math|Float|Lerp 0.0 (/ (Spline|GetDistanceAlongSplineatSplinePoint (Variables|Default|GetSpline) (- (Spline|GetNumberOfSplinePoints (Variables|Default|GetSpline)) 1)) (Utilities|Array|Length (Variables|Default|GetMeshes))) _newtrack_0)) _sectionlength) "Local") (Variables|Default|GetTangentSmooth)) true :!class /Script/Engine.SplineMeshComponent)))
    (:Finished
      (CallFunction|PlayTimeline))))

(event EventBeginPlay
  (for _index (range 0 (.ReturnValue (Math|Float|Division(WholeandRemainder) (Spline|GetSplineLength (Variables|Default|GetSpline)) (Variables|Default|GetSectionLength))))
    (bind _returnvalue (AddComponent|AddSplineMeshComponent false))
    (Components|StaticMesh|SetStaticMesh _returnvalue (Variables|Default|GetSplinedObject))
    (SplineMesh|SetForwardAxis _returnvalue (Variables|Default|GetForwardAxis) true)
    (Utilities|Array|Add (Variables|Default|GetMeshes) _returnvalue))
  (Components|Timeline|SetPlayRate (Variables|Default|GetTimeline) (/ 1.0 (Variables|Default|GetMovementSpeed)))
  (CallFunction|PlayTimeline))

(fn ConstructionScript)