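; Kraken boss tentacle hazard that sweeps across the play space and damages ships.
; BeginPlay saves its storage location and plays a timeline that subtly stretches the mesh vertically.
; IStartTentacle drives chained timelines that move it forward, sink it, then snap it back to storage.
; Front and rear hit colliders share a DoOnce that damages one BPI_Ship actor, resetting only after the return to storage.
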(event OnComponentBeginOverlap(HitColFront)
  (params (OverlappedComponent :type Primitive%20Component%20Object%20Reference) (OtherActor :type Actor%20Object%20Reference) (OtherComp :type Primitive%20Component%20Object%20Reference) (OtherBodyIndex :type Integer) (bFromSweep :type Boolean) (SweepResult :type Hit%20Result%20Structure%20%28by%20ref%29))
  (Variables|Default|SetHitActor OtherActor)
  (if (Utilities|DoesObjectImplementInterface (Variables|Default|GetHitActor) "/Game/Blueprints/Ship/BPI_Ship.BPI_Ship_C")
    (Utilities|FlowControl|DoOnce false
      (:Completed
        (Class|BPIShip|IDamageShip(Message) (Variables|Default|GetHitActor) 4e+01)
        (Variables|Default|SetHitActor 0)
        (Development|PrintString "Damging ship tebtacle")))))

(event OnComponentBeginOverlap(HitColRear)
  (params (OverlappedComponent :type Primitive%20Component%20Object%20Reference) (OtherActor :type Actor%20Object%20Reference) (OtherComp :type Primitive%20Component%20Object%20Reference) (OtherBodyIndex :type Integer) (bFromSweep :type Boolean) (SweepResult :type Hit%20Result%20Structure%20%28by%20ref%29))
  (Variables|Default|SetHitActor OtherActor)
  (if (Utilities|DoesObjectImplementInterface (Variables|Default|GetHitActor) "/Game/Blueprints/Ship/BPI_Ship.BPI_Ship_C")
    (Utilities|FlowControl|DoOnce false
      (:Completed
        (Class|BPIShip|IDamageShip(Message) (Variables|Default|GetHitActor) 4e+01)
        (Variables|Default|SetHitActor 0)
        (Development|PrintString "Damging ship tebtacle")))))

(event EventIStartTentacle
  (bind _output_get (Variables|Default|SetStartingLocation (Transformation|GetActorLocation)))
  (Variables|Default|SetEndLocation (+ _output_get (* (Transformation|GetActorForwardVector) 5e+03)))
  (bind _alpha (Timeline|MoveTentacleTimeline PlayFromStart)
    (:Update
      (Transformation|SetActorLocation (Math|Vector|Lerp(Vector) (Variables|Default|GetStartingLocation) (Variables|Default|GetEndLocation) _alpha) false false))
    (:Finished
      (bind _output_get_2 (Variables|Default|SetFinalLocation (Transformation|GetActorLocation)))
      (bind _alpha_2 (Timeline|TentacleToStorage PlayFromStart)
        (:Update
          (Transformation|SetActorLocation (Math|Vector|Lerp(Vector) _output_get_2 (+ _output_get_2 (+ (* (Transformation|GetActorUpVector) 2e+02) "0.000000,0.000000,-2000.000000")) _alpha_2) false false))
        (:Finished
          (Transformation|SetActorLocation (Variables|Default|GetStorageLocation) false false)
          (Utilities|FlowControl|DoOnce false) ; enters at Reset
        )))))

(event EventBeginPlay
  (Variables|Default|SetStorageLocation (Transformation|GetActorLocation))
  (bind _alpha (Timeline|StretchTentacle Play)
    (:Update
      (Transformation|SetWorldScale3D (Variables|Default|GetTentacle) (Math|Vector|MakeVector 1.0 1.0 (Math|Float|Lerp 0.95 1.0 _alpha))))))

(fn ConstructionScript)