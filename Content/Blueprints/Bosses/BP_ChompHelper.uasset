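; BP_ChompHelper is a helper actor for the boss chomp attack, marking the chomp target and dealing its damage.
; On spawn it turns toward the player's leap position and exposes an event to move the target.
; The boss entering its trigger spheres fires a one-time sphere-trace bite and a timeline-scaled shockwave mesh.
; The active wave damages the player once through the ship damage interface, and the actor destroys itself when expansion finishes.
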(event OnComponentBeginOverlap(WaveActivateSphere)
  (params (OverlappedComponent :type Primitive%20Component%20Object%20Reference) (OtherActor :type Actor%20Object%20Reference) (OtherComp :type Primitive%20Component%20Object%20Reference) (OtherBodyIndex :type Integer) (bFromSweep :type Boolean) (SweepResult :type Hit%20Result%20Structure%20%28by%20ref%29))
  (bind _start_wave_scale (Variables|Default|GetStart%20Wave%20Scale))
  ;[0 0 0] Increase Wave Scale Over Time
  (if (== OtherActor (Variables|Default|GetBoss))
    (Utilities|FlowControl|DoOnce false
      (:Completed
        (Rendering|SetVisibility (Variables|Default|GetDamagingWaveMesh) true false)
        (Variables|Default|SetActivated true)
        (bind _alpha (Timeline|Increase%20Wave%20Scale PlayFromStart)
          (:Update
            (Transformation|SetRelativeScale3D (Variables|Default|GetDamagingWaveMesh) (Math|Vector|Lerp(Vector) _start_wave_scale (+ _start_wave_scale "10.000000,10.000000,10.000000") _alpha)))
          (:Finished
            (Actor|DestroyActor)))))))

(event OnComponentBeginOverlap(DamageSphere)
  (params (OverlappedComponent :type Primitive%20Component%20Object%20Reference) (OtherActor :type Actor%20Object%20Reference) (OtherComp :type Primitive%20Component%20Object%20Reference) (OtherBodyIndex :type Integer) (bFromSweep :type Boolean) (SweepResult :type Hit%20Result%20Structure%20%28by%20ref%29))
  ;[0 0 0] Wave Damage
  (if (and (== OtherActor (Variables|Default|GetPlayer)) (Variables|Default|GetActivated))
    (Utilities|FlowControl|DoOnce false
      (:Completed
        (Class|BPIShip|IDamageShip(Message) (Variables|Default|GetPlayer) 2e+01)
        (Development|PrintString (Utilities|String|Append "Wave Damage: " (Utilities|String|ToString(Float) 2e+01)))))))

(event OnComponentBeginOverlap(ChompDamageSphere)
  (params (OverlappedComponent :type Primitive%20Component%20Object%20Reference) (OtherActor :type Actor%20Object%20Reference) (OtherComp :type Primitive%20Component%20Object%20Reference) (OtherBodyIndex :type Integer) (bFromSweep :type Boolean) (SweepResult :type Hit%20Result%20Structure%20%28by%20ref%29))
  (bind _chomp_damage_sphere (Variables|Default|GetChomp%20Damage%20Sphere))
  (bind _returnvalue (Transformation|GetWorldLocation _chomp_damage_sphere))
  ;[0 0 0] Chomp Damage
  (if (== OtherActor (Variables|Default|GetBoss))
    (Utilities|FlowControl|DoOnce false
      (:Completed
        (bind _outhits (Collision|MultiSphereTraceByChannel _returnvalue _returnvalue 3e+02 "TraceTypeQuery1" false (Utilities|Array|MakeArray (Variables|Default|GetBoss)) "None"))
        (for _array_element _outhits
          (Class|BPIShip|IDamageShip(Message) (.HitActor (Collision|BreakHitResult _array_element)) 3e+01)
          (Development|PrintString (Utilities|String|Append "Chomp Damage: " (Utilities|String|ToString(Float) 3e+01))))))))

(event Custom|Update%20Chomp%20Location
  (params (Location :type Vector%20%28by%20ref%29))
  (Transformation|SetWorldLocation (Variables|Default|GetChomp%20Target%20Location) Location false false))

(event EventBeginPlay
  (bind _returnvalue (Transformation|GetActorLocation))
  (Variables|Default|SetPlayer (Game|Player|GetPlayerPawn 0))
  (bind _returnvalue_2 (Actor|GetActorOfClass "/Game/Blueprints/Bosses/MoONUI/CH_BaseBoss.CH_BaseBoss_C"))
  (Variables|Default|SetBoss _returnvalue_2)
  (bind _position (Class|BPIShip|IBossGetLeapPosition(Message) (Variables|Default|GetPlayer)))
  (Transformation|SetActorTransform (Math|Transform|MakeTransform _returnvalue (Math|Rotator|FindLookatRotation _returnvalue _position) "1.000000,1.000000,1.000000"))
  (Variables|Default|SetStart%20Wave%20Scale (Variables|/Script/Engine.SceneComponent|GetRelativeScale3D (Variables|Default|GetDamagingWaveMesh))))

(event EventTick
  (params (DeltaSeconds :type Float%20%28single-precision%29)))

(fn ConstructionScript)