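; Base boss for a ship-versus-sea-creature fight, using timelines to drive its movement and attacks on Pawn_ShipNew.
; The player's first overlap with WhirlpoolRange starts a chain: move into position, spawn BP_Whirlpool, circle it, then dive and chomp upward at the player's sampled location.
; ShowOff arcs the boss between two markers, then Reset lerps it toward StartLoc.
; Ram and Roam are empty, Activation_Range triggers nothing, and the AttackCheck timer is unwired.
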(event OnComponentBeginOverlap(Activation_Range)
  (params (OverlappedComponent :type Primitive%20Component%20Object%20Reference) (OtherActor :type Actor%20Object%20Reference) (OtherComp :type Primitive%20Component%20Object%20Reference) (OtherBodyIndex :type Integer) (bFromSweep :type Boolean) (SweepResult :type Hit%20Result%20Structure%20%28by%20ref%29))
  (if (== OtherActor (Variables|Default|GetPlayer))
    (Utilities|FlowControl|DoOnce false)))

(event OnComponentBeginOverlap(WhirlpoolRange)
  (params (OverlappedComponent :type Primitive%20Component%20Object%20Reference) (OtherActor :type Actor%20Object%20Reference) (OtherComp :type Primitive%20Component%20Object%20Reference) (OtherBodyIndex :type Integer) (bFromSweep :type Boolean) (SweepResult :type Hit%20Result%20Structure%20%28by%20ref%29))
  (if (== OtherActor (Variables|Default|GetPlayer))
    (Utilities|FlowControl|DoOnce false
      (:Completed
        (CallFunction|WhirlPool)))))

(event Custom|AttackCheck
  (if (Collision|IsOverlappingActor (Variables|Default|GetWhirlpoolRange) (Variables|Default|GetPlayer) :!class /Script/Engine.PrimitiveComponent)
    (CallFunction|WhirlPool)))

(event Custom|Ram)

(event Custom|ShowOff
  (bind _showoffstart (Variables|Default|GetShowOffStart))
  (bind _showoffend (Variables|Default|GetShowOffEnd))
  (bind _whirlpoolstartrot (Variables|Default|GetWhirlPoolStartRot))
  (bind _returnvalue (Transformation|GetActorLocation _showoffstart))
  (bind _returnvalue_2 (Transformation|GetActorLocation _showoffend))
  (bind _returnvalue_3 (- _returnvalue _returnvalue_2))
  (bind _returnvalue_4 (Math|Vector|Normalize _returnvalue_3))
  (bind _returnvalue_5 (Math|Vector|VectorLength _returnvalue_3))
  (bind _returnvalue_6 (/ _returnvalue_5 2.0))
  (bind _returnvalue_7 (* _returnvalue_6 _returnvalue_4))
  (bind _returnvalue_8 (- _returnvalue _returnvalue_7))
  (Variables|Default|SetShowOffStartRot (Math|Rotator|FindLookatRotation _returnvalue_8 _returnvalue))
  (bind _newtrack_0 (Timeline|T_Showoff PlayFromStart)
    (:Update
      (Transformation|SetActorLocationAndRotation (+ _returnvalue_8 (* (Math|Vector|GetForwardVector (Math|Rotator|MakeRotator (.roll _whirlpoolstartrot) (+ (* _newtrack_0 -2.7e+02) (.pitch _whirlpoolstartrot) 225.0) (.yaw _whirlpoolstartrot))) (/ (Math|Vector|VectorLength (- (Transformation|GetActorLocation (Variables|Default|GetShowOffStart)) (Transformation|GetActorLocation (Variables|Default|GetShowOffEnd)))) 2.0))) (Math|Rotator|MakeRotator 1.8e+02 (+ (* _newtrack_0 -2.7e+02) -7e+01) 0.0)))
    (:Finished
      (CallFunction|Reset))))

(event Custom|Chomp
  (bind _chompaimlocation (Variables|Default|GetChompAimLocation))
  (bind _chompaimlocation_2 (Variables|Default|GetChompAimLocation))
  (bind _chompaimlocation_3 (Variables|Default|GetChompAimLocation))
  (Variables|Default|SetLocationAtAttackStart (Transformation|GetActorLocation))
  (bind _newtrack_0 (Timeline|T_ChompPrep PlayFromStart)
    (:Update
      (Transformation|SetActorLocation (Math|Vector|Lerp(Vector) (Variables|Default|GetLocationAtAttackStart) (Math|Vector|MakeVector (.x _chompaimlocation_2) (.y _chompaimlocation_2) (- (.z _chompaimlocation_2) 1e+04)) _newtrack_0) false false))
    (:Finished
      (bind _newtrack_0_2 (Timeline|T_Chomp PlayFromStart)
        (:Update
          (Transformation|SetActorLocationAndRotation (Math|Vector|Lerp(Vector) (Math|Vector|MakeVector (.x _chompaimlocation) (.y _chompaimlocation) (- (.z _chompaimlocation) 5e+03)) (Math|Vector|MakeVector (.x _chompaimlocation_3) (.y _chompaimlocation_3) (+ (.z _chompaimlocation_3) 1e+04)) _newtrack_0_2) "-90.000000,0.000000,0.000000"))))))

(event Custom|Roam)

(event Custom|WhirlPool
  (Variables|Default|SetWhirlPoolCentre (Transformation|GetActorLocation (Variables|Default|GetPlayer)))
  (Variables|Default|SetLocationAtAttackStart (Transformation|GetActorLocation))
  (Variables|Default|SetWhirlpoolStartLoc (+ (Variables|Default|GetWhirlPoolCentre) (* (Math|Vector|GetForwardVector (Math|Rotator|MakeRotator (.roll (Variables|Default|GetWhirlPoolStartRot)) (.pitch (Variables|Default|GetWhirlPoolStartRot)) (+ (.yaw (Variables|Default|GetWhirlPoolStartRot)) 0.0 0.0))) (Math|Vector|VectorLength (- (Variables|/Script/Engine.SphereComponent|GetSphereRadius (Variables|Default|GetWhirlpoolRange)) 1e+04)))))
  (bind _newtrack_0 (Timeline|T_PrepWhirlpool PlayFromStart)
    (:Update
      (Transformation|SetActorLocation (Math|Vector|Lerp(Vector) (Variables|Default|GetLocationAtAttackStart) (Variables|Default|GetWhirlpoolStartLoc) _newtrack_0) false false))
    (:Finished
      (Utilities|FlowControl|Sequence
        (:then_0
          (bind _returnvalue (Game|SpawnActorfromClass "/Game/Blueprints/Water/BP_Whirlpool.BP_Whirlpool_C" (Math|Transform|MakeTransform (Math|Vector|MakeVector (.x (Variables|Default|GetWhirlPoolCentre)) (.y (Variables|Default|GetWhirlPoolCentre)) 0.0) "0, 0, 0" "1.000000,1.000000,1.000000") "Undefined" "MultiplyWithRoot" 0 0))
          (Variables|Default|SetBP_Whirlpool _returnvalue))
        (:then_1
          (Variables|Default|SetWhirlPoolStartRot (Math|Rotator|FindLookatRotation (Variables|Default|GetWhirlpoolStartLoc) (Variables|Default|GetWhirlPoolCentre)))
          (bind _newtrack_0_2 (Timeline|T_Whirlpool PlayFromStart)
            (:Update
              (Transformation|SetActorLocationAndRotation (+ (Variables|Default|GetWhirlPoolCentre) (* (Math|Vector|GetForwardVector (Math|Rotator|MakeRotator (.roll (Variables|Default|GetWhirlPoolStartRot)) (.pitch (Variables|Default|GetWhirlPoolStartRot)) (+ (.yaw (Variables|Default|GetWhirlPoolStartRot)) (* _newtrack_0_2 -3.6e+02) 9e+01))) (Math|Vector|VectorLength (- (Variables|/Script/Engine.SphereComponent|GetSphereRadius (Variables|Default|GetWhirlpoolRange)) 1e+04)))) (Math|Rotator|MakeRotator 0.0 0.0 (* _newtrack_0_2 -3.6e+02))))
            (:Finished
              (Variables|Default|SetChompAimLocation (Transformation|GetActorLocation (Variables|Default|GetPlayer)))
              (CallFunction|Chomp))))))))

(event Custom|Reset
  (Variables|Default|SetResetStartTransform (Transformation|GetActorTransform))
  (bind _newtrack_0 (Timeline|T_Reset Play)
    (:Update
      (Transformation|SetActorTransform (Math|Transform|Lerp(Transform) (Variables|Default|GetResetStartTransform) (Math|Transform|MakeTransform (Variables|Default|GetStartLoc) "0, 0, 0" "1.000000,1.000000,1.000000") _newtrack_0)))))

(event EventBeginPlay
  (bind _returnvalue (Actor|GetActorOfClass "/Game/Blueprints/t014172k/Pawn_ShipNew.Pawn_ShipNew_C"))
  (Variables|Default|SetPlayer _returnvalue))

(event Collision|EventActorBeginOverlap
  (params (OtherActor :type Actor%20Object%20Reference)))

(event EventTick
  (params (DeltaSeconds :type Float%20%28single-precision%29)))

(fn ConstructionScript)