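; BP_CircleHelper_Small is a boss-fight helper actor that follows the player and carries a circle spline.
; On BeginPlay it finds the boss (CH_BaseBoss, falling back to Pawn_BaseBoss) and turns once to face it, flattened to yaw by using the boss's height.
; Each Tick it sweeps to the player's location, then sweeps CircleSpline to the Sphere component's world position.
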(event EventBeginPlay
  (bind _returnvalue (Transformation|GetActorLocation))
  (Variables|Default|SetPlayer (Game|Player|GetPlayerPawn 0))
  (bind _returnvalue_2 (Actor|GetActorOfClass "/Game/Blueprints/Bosses/MoONUI/CH_BaseBoss.CH_BaseBoss_C"))
  (bind _output_get (Variables|Default|SetBoss _returnvalue_2))
  (Utilities|IsValid _output_get
    (:Is%20Valid
      _)
    (:Is%20Not%20Valid
      (bind _returnvalue_3 (Actor|GetActorOfClass "/Game/Blueprints/Bosses/MoONUI/Pawn_BaseBoss.Pawn_BaseBoss_C"))
      (Variables|Default|SetBoss _returnvalue_3)))
  (Transformation|SetActorRotation (Math|Rotator|FindLookatRotation (Math|Vector|MakeVector (.x _returnvalue) (.y _returnvalue) (.z (Transformation|GetActorLocation (Variables|Default|GetBoss)))) (Transformation|GetActorLocation (Variables|Default|GetBoss)))))

(event EventTick
  (params (DeltaSeconds :type Float%20%28single-precision%29))
  (Transformation|SetActorLocation (Transformation|GetActorLocation (Variables|Default|GetPlayer)) true false)
  (Transformation|SetWorldLocation (Variables|Default|GetCircleSpline) (Transformation|GetWorldLocation (Variables|Default|GetSphere)) true false))

(fn ConstructionScript)