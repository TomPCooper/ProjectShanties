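; BP_MoONuiScale is a scale body part of the MoONui boss that can be pulled loose and float on water.
; The construction script applies the configured mesh and multiplies its scale by the actor's scale.
; Pull enables water-float ticking, turns on hull physics with damping, and launches it upward with randomized sideways and spin impulses.
; It also reports itself as the hit actor and supplies a damage multiplier.
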(event EventPull
  (bind _floathull (Variables|Default|GetFloatHull))
  (Components|Tick|SetComponentTickEnabled (Variables|Default|GetBPC_WaterFloat) true)
  (Physics|SetSimulatePhysics _floathull true)
  (Collision|SetCollisionProfileName _floathull "PhysicsActor" true :!class /Script/Engine.PrimitiveComponent)
  (Collision|SetCollisionObjectType _floathull "ECC_GameTraceChannel1")
  (Class|PrimitiveComponent|SetAngularDamping _floathull 0.4)
  (Class|PrimitiveComponent|SetLinearDamping _floathull 0.4)
  (Physics|AddImpulse _floathull (Math|Vector|MakeVector (Math|Random|RandomFloatinRange -5e+03 5e+03) (Math|Random|RandomFloatinRange -5e+03 5e+03) 1e+04) "None" false)
  (Class|PrimitiveComponent|AddAngularImpulseinDegrees _floathull (Math|Vector|MakeVector (Math|Random|RandomFloatinRange 0.0 1e+02) (Math|Random|RandomFloatinRange 0.0 1e+02) (Math|Random|RandomFloatinRange 0.0 1e+02)) "None" true))

(fn ConstructionScript
  (bind _scalesmesh (Variables|Default|GetScaleSmesh))
  (|CallParentFunction)
  (Components|StaticMesh|SetStaticMesh _scalesmesh (Variables|Default|GetScaleMesh))
  (Transformation|SetWorldScale3D _scalesmesh (* (Variables|Default|GetMeshScale) (Transformation|GetActorScale3D))))

(fn GetBossBodyPartDamageMultiplier
  (return true (Variables|Default|GetDamageMultiplier)))

(fn GetActorHit
  (return self))