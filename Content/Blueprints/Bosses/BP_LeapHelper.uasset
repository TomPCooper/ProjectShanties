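; Helper actor for the boss leap attack, holding the leap spline and the damaging shockwave at the landing spot.
; On BeginPlay it finds the ship and boss and turns toward the ship's BossLeapLocation.
; UpdateLandLocation moves a spline point, the trigger sphere and the wave mesh to the landing location.
; When the boss enters the trigger, a timeline grows the wave, which can damage the ship once, then the actor destroys itself.
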(event OnComponentBeginOverlap(DamageSphere)
  (params (OverlappedComponent :type Primitive%20Component%20Object%20Reference) (OtherActor :type Actor%20Object%20Reference) (OtherComp :type Primitive%20Component%20Object%20Reference) (OtherBodyIndex :type Integer) (bFromSweep :type Boolean) (SweepResult :type Hit%20Result%20Structure%20%28by%20ref%29))
  ;[0 0 0] Wave Damage
  (if (and (== OtherActor (Variables|Default|GetPlayer)) (Variables|Default|GetActivated))
    (Utilities|FlowControl|DoOnce false
      (:Completed
        (bind _returnvalue (Game|Damage|ApplyDamage (Variables|Default|GetPlayer) 3e+01 0 (Variables|Default|GetBoss)))
        (Development|PrintString (Utilities|String|Append "Damage: " (Utilities|String|ToString(Float) _returnvalue)))))))

(event OnComponentBeginOverlap(ActivateSphere)
  (params (OverlappedComponent :type Primitive%20Component%20Object%20Reference) (OtherActor :type Actor%20Object%20Reference) (OtherComp :type Primitive%20Component%20Object%20Reference) (OtherBodyIndex :type Integer) (bFromSweep :type Boolean) (SweepResult :type Hit%20Result%20Structure%20%28by%20ref%29))
  (bind _start_wave_scale (Variables|Default|GetStart%20Wave%20Scale))
  ;[0 0 0] Increase Wave Scale Over Time
  (if (== OtherActor (Variables|Default|GetBoss))
    (Utilities|FlowControl|DoOnce false
      (:Completed
        (Rendering|SetVisibility (Variables|Default|GetDamagingWaveMesh) true false)
        (Variables|Default|SetActivated true)
        (bind _alpha (Timeline|Timeline PlayFromStart)
          (:Update
            (Transformation|SetRelativeScale3D (Variables|Default|GetDamagingWaveMesh) (Math|Vector|Lerp(Vector) _start_wave_scale (+ _start_wave_scale "5.000000,5.000000,5.000000") _alpha)))
          (:Finished
            (Actor|DestroyActor)))))))

(event Custom|Update%20Land%20Location
  (params (Location :type Vector%20%28by%20ref%29))
  ;[0 0 0] Changes the land location to in front of the ship.
  (Spline|SetLocationatSplinePoint (Variables|Default|GetLeapSpline) 4 Location "World" true)
  (Transformation|SetWorldLocation (Variables|Default|GetActivate%20Sphere) Location false false)
  (Transformation|SetWorldLocation (Variables|Default|GetDamagingWaveMesh) Location false false))

(event EventBeginPlay
  (bind _returnvalue (Transformation|GetActorLocation))
  (bind _returnvalue_2 (Actor|GetActorOfClass "/Game/Blueprints/t014172k/Pawn_ShipNew.Pawn_ShipNew_C"))
  (Variables|Default|SetPlayer _returnvalue_2)
  (bind _returnvalue_3 (Actor|GetActorOfClass "/Game/Blueprints/Bosses/MoONUI/CH_BaseBoss.CH_BaseBoss_C"))
  (Variables|Default|SetBoss _returnvalue_3)
  (Transformation|SetActorTransform (Math|Transform|MakeTransform _returnvalue (Math|Rotator|FindLookatRotation _returnvalue (Transformation|GetWorldLocation (Variables|/Game/Blueprints/t014172k/Pawn_ShipNew.Pawn_ShipNew_C|GetBoss%20Leap%20Location (Variables|Default|GetPlayer)))) "1.000000,1.000000,1.000000"))
  (Variables|Default|SetStart%20Wave%20Scale (Variables|/Script/Engine.SceneComponent|GetRelativeScale3D (Variables|Default|GetDamagingWaveMesh))))

(fn ConstructionScript)