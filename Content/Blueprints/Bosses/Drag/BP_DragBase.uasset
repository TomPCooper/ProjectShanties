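; Base actor for a floating bounty in the boss folder that the player's ship can tow.
; The construction script applies the configured mesh and float hull box extent, and BeginPlay forces a water-float submerged check and creates the tow prompt widget.
; Overlap by a SHIP_MAIN component toggles the prompt and sets or clears the ship's interactable.
; Interacting messages the player pawn to attach the tow and destroys the prompt area.
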(event OnComponentBeginOverlap(ShipPromptArea)
  (params (OverlappedComponent :type Primitive%20Component%20Object%20Reference) (OtherActor :type Actor%20Object%20Reference) (OtherComp :type Primitive%20Component%20Object%20Reference) (OtherBodyIndex :type Integer) (bFromSweep :type Boolean) (SweepResult :type Hit%20Result%20Structure%20%28by%20ref%29))
  (if (Components|ComponentHasTag OtherComp "SHIP_MAIN")
    (UserInterface|Viewport|AddtoViewport (Variables|Default|GetInteractionWidget) 0)
    (Class|BPIShip|IInteractable(Message) OtherActor self)))

(event OnComponentEndOverlap(ShipPromptArea)
  (params (OverlappedComponent :type Primitive%20Component%20Object%20Reference) (OtherActor :type Actor%20Object%20Reference) (OtherComp :type Primitive%20Component%20Object%20Reference) (OtherBodyIndex :type Integer))
  (if (Components|ComponentHasTag OtherComp "SHIP_MAIN")
    (Widget|RemovefromParent (Variables|Default|GetInteractionWidget))
    (Class|BPIShip|IInteractable(Message) OtherActor)))

(event EventBeginPlay
  (Default|ForceSubmergedCheck (Variables|Default|GetBPC_WaterFloat))
  (bind _returnvalue (UserInterface|CreateWidget "/Game/Blueprints/UI/Interaction/WBP_Interaction.WBP_Interaction_C" (Game|GetPlayerController 0)))
  (bind _output_get (Variables|Default|SetInteractionWidget _returnvalue))
  (Default|UpdateText _output_get "e" "tow bounty"))

(event EventInteract
  (Class|BPIShip|IAttachTow(Message) (Game|Player|GetPlayerPawn 0) self)
  (Components|DestroyComponent (Variables|Default|GetShipPromptArea)))

(fn ConstructionScript
  (Variables|/Script/Engine.SkeletalMeshComponent|SetSkeletalMeshAsset (Variables|Default|GetSkeletalMesh) (Variables|Default|GetMesh))
  (Components|Box|SetBoxExtent (Variables|Default|GetFloatHull) (Variables|Default|GetBox%20Extent) true))