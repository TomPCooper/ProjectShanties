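; Health component that tracks its owner's HP and answers damage, heal and death events.
; Standard damage is reduced by resistance, clamped and triggers death at zero, destroying the owner and child components' owners.
; Direct damage bypasses resistance and passes up through parent components, without clamping or a death check.
; Healing is unclamped, and damage milestones are a print-only TODO.
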(event EventBeginPlay
  (Variables|Default|SetCurrentHealth (Variables|Default|GetHealthMax)))

(event EventTick
  (params (DeltaSeconds :type Float%20%28single-precision%29)))

(event EventIDamage
  (params (Damage :type Float%20%28double-precision%29))
  ;[1 1 1] Apply damage
  (bind _output_get (Variables|Default|SetCurrentHealth (Math|Float|Clamp(Float) (- (Variables|Default|GetCurrentHealth) (- Damage (* Damage (Variables|Default|GetDamageResistance)))) 0.0 (Variables|Default|GetHealthMax))))
  (Development|PrintString (Class|KismetStringLibrary|BuildStringDouble "" "Health: " _output_get))
  (if (<= _output_get 0.0)
    (CallFunction|IDeath)))

(event EventIDamageMilestone
  (params (HealthPercentage :type Float%20%28double-precision%29))
  ;[1 1 1] TODO: Damage milestones
  (Development|PrintString (Class|KismetStringLibrary|BuildStringDouble "" "DAMAGE MILESTONE: " HealthPercentage "%")))

(event EventIDeath
  ;[1 1 1] Destroy self and children on death
  (Development|PrintString "HC DEATH")
  (for _array_element (Variables|Default|GetChildHealthComponents)
    (Actor|DestroyActor (Components|GetOwner _array_element)))
  (Actor|DestroyActor (Components|GetOwner)))

(event EventIHeal
  (params (HealAmount :type Float%20%28double-precision%29))
  ;[1 1 1] Damage healing
  (Variables|Default|SetCurrentHealth (+ (Variables|Default|GetCurrentHealth) HealAmount))
  (Development|PrintString (Class|KismetStringLibrary|BuildStringDouble (Class|KismetStringLibrary|BuildStringDouble "" "Healed " HealAmount " HP (Total: ") "" (Variables|Default|GetCurrentHealth) ")")))

(event EventIDamageDirect
  (params (Damage :type Float%20%28double-precision%29))
  (bind _parenthealthcomponent (Variables|Default|GetParentHealthComponent))
  ;[1 1 1] Damage direct
  (Variables|Default|SetCurrentHealth (- (Variables|Default|GetCurrentHealth) Damage))
  (Utilities|IsValid _parenthealthcomponent
    (:Is%20Valid
      (Default|IDamageDirect _parenthealthcomponent Damage))))