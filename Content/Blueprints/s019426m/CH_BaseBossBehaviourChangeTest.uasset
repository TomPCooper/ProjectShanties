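; Test sea-boss Blueprint that targets Pawn_ShipNew, prototyping attack behaviour and selection.
; AttackCheck picks attacks by distance, randomness and attack history, though Leap, Chomp and ReturnToCircle are empty stubs and activation triggers nothing.
; WhirlPool uses timelines to spawn BP_Whirlpool and orbit it before calling Chomp; ShowOff arcs between markers, then resets.
; Ram stretches a spline beneath the ship, stepped by a non-looping timer.
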(event OnComponentBeginOverlap(Activation_Range)
  (params (OverlappedComponent :type Primitive%20Component%20Object%20Reference) (OtherActor :type Actor%20Object%20Reference) (OtherComp :type Primitive%20Component%20Object%20Reference) (OtherBodyIndex :type Integer) (bFromSweep :type Boolean) (SweepResult :type Hit%20Result%20Structure%20%28by%20ref%29))
  (if (== OtherActor (Variables|Default|GetPlayer))
    (Utilities|FlowControl|DoOnce false)))

(event OnComponentBeginOverlap(WhirlpoolRange)
  (params (OverlappedComponent :type Primitive%20Component%20Object%20Reference) (OtherActor :type Actor%20Object%20Reference) (OtherComp :type Primitive%20Component%20Object%20Reference) (OtherBodyIndex :type Integer) (bFromSweep :type Boolean) (SweepResult :type Hit%20Result%20Structure%20%28by%20ref%29)))

(event Custom|AttackCheck
  (bind _returnvalue (Math|Random|RandomBool))
  ;[1 1 1] Attack Selector
  (if (<= (Math|Vector|VectorLength (- (Transformation|GetActorLocation) (Transformation|GetActorLocation (Variables|Default|GetPlayer)))) 1e+03)
    (if _returnvalue
      ;;[1 1 1] If whirlpool is used, neither it or the attack used after is selected
      (if (Variables|Default|GetUsedWhirlpool)
        (Variables|Default|SetUsedWhirlpool false)
        (CallFunction|Ram :!label _label)
        (Variables|Default|SetLastAttack "NewEnumerator3")
        (else
          (CallFunction|WhirlPool :!label _label_2)
          (Variables|Default|SetUsedWhirlpool true)))
      (else
        ;;[1 1 1] Avoids using the same attack twice
        (if (Utilities|Enum|Equal(Enum) (Variables|Default|GetLastAttack) "NewEnumerator3")
          (goto _label)
          (else
            (goto _label_2)))))
    (elif _returnvalue
      (if (Utilities|Enum|Equal(Enum) (Variables|Default|GetLastAttack) "NewEnumerator1")
        (CallFunction|Chomp :!label _label_3)
        (Variables|Default|SetLastAttack "NewEnumerator1")
        (else
          (CallFunction|Leap :!label _label_4)
          (Variables|Default|SetLastAttack "NewEnumerator0")))
      (elif (Utilities|Enum|Equal(Enum) (Variables|Default|GetLastAttack) "NewEnumerator0")
        (goto _label_4)
        (else
          (goto _label_3))))))

(event Custom|Ram
  ;[1 1 1] Ram
  (bind (_bossloc _locundership) (CallFunction|GetPositionUnderShip))
  (CallFunction|SetSplinePointStartandEnd (Variables|Default|GetRamSpline) _bossloc _locundership)
  (Variables|Default|SetDistanceAlongAttack 0.0)
  (bind _returnvalue (Utilities|Time|SetTimerbyEvent (delegate Custom|RamActive) 0.02))
  (bind _output_get (Variables|Default|SetRamHandler _returnvalue))
  (Variables|Default|SetCurrent%20Attack%20Handle _output_get))

(event Custom|ReturnToCircle)

(event Custom|Circle%20Active)

(event Custom|ShowOff
  (bind _showoffstart (Variables|Default|GetShowOffStart))
  (bind _showoffend (Variables|Default|GetShowOffEnd))
  (bind _whirlpoolstartrot (Variables|Default|GetWhirlPoolStartRot))
  (bind _returnvalue (Transformation|GetActorLocation _showoffstart))
  (bind _returnvalue_2 (Transformation|GetActorLocation _showoffend))
  (bind _returnvalue_3 (- _returnvalue _returnvalue_2))
  (bind _returnvalue_4 (Math|Vector|Normalize _returnvalue_3))
  (bind _returnvalue_5 (Math|Vector|VectorLength _returnvalue_3))
  (bind _returnvalue_6 (/ _returnvalue_5 2.0))
  (bind _returnvalue_7 (* _returnvalue_6 _returnvalue_4))
  (bind _returnvalue_8 (- _returnvalue _returnvalue_7))
  (Variables|Default|SetShowOffStartRot (Math|Rotator|FindLookatRotation _returnvalue_8 _returnvalue))
  (bind _newtrack_0 (Timeline|T_Showoff PlayFromStart)
    (:Update
      (Transformation|SetActorLocationAndRotation (+ _returnvalue_8 (* (Math|Vector|GetForwardVector (Math|Rotator|MakeRotator (.roll _whirlpoolstartrot) (+ (* _newtrack_0 -2.7e+02) (.pitch _whirlpoolstartrot) 225.0) (.yaw _whirlpoolstartrot))) (/ (Math|Vector|VectorLength (- (Transformation|GetActorLocation (Variables|Default|GetShowOffStart)) (Transformation|GetActorLocation (Variables|Default|GetShowOffEnd)))) 2.0))) (Math|Rotator|MakeRotator 1.8e+02 (+ (* _newtrack_0 -2.7e+02) -7e+01) 0.0)))
    (:Finished
      (CallFunction|Reset))))

(event Custom|Chomp)

(event Custom|Roam)

(event Custom|WhirlPool
  (Variables|Default|SetWhirlPoolCentre (Transformation|GetActorLocation (Variables|Default|GetPlayer)))
  (Variables|Default|SetLocationAtAttackStart (Transformation|GetActorLocation))
  (Variables|Default|SetWhirlpoolStartLoc (+ (Variables|Default|GetWhirlPoolCentre) (* (Math|Vector|GetForwardVector (Math|Rotator|MakeRotator (.roll (Variables|Default|GetWhirlPoolStartRot)) (.pitch (Variables|Default|GetWhirlPoolStartRot)) (+ (.yaw (Variables|Default|GetWhirlPoolStartRot)) 0.0 0.0))) (Math|Vector|VectorLength (- (Variables|/Script/Engine.SphereComponent|GetSphereRadius (Variables|Default|GetWhirlpoolRange)) 1e+04)))))
  (bind _newtrack_0 (Timeline|T_PrepWhirlpool PlayFromStart)
    (:Update
      (Transformation|SetActorLocation (Math|Vector|Lerp(Vector) (Variables|Default|GetLocationAtAttackStart) (Variables|Default|GetWhirlpoolStartLoc) _newtrack_0) false false))
    (:Finished
      (Utilities|FlowControl|Sequence
        (:then_0
          (bind _returnvalue (Game|SpawnActorfromClass "/Game/Blueprints/Water/BP_Whirlpool.BP_Whirlpool_C" (Math|Transform|MakeTransform (Math|Vector|MakeVector (.x (Variables|Default|GetWhirlPoolCentre)) (.y (Variables|Default|GetWhirlPoolCentre)) 0.0) "0, 0, 0" "1.000000,1.000000,1.000000") "Undefined" "MultiplyWithRoot" 0 0))
          (Variables|Default|SetBP_Whirlpool _returnvalue))
        (:then_1
          (Variables|Default|SetWhirlPoolStartRot (Math|Rotator|FindLookatRotation (Variables|Default|GetWhirlpoolStartLoc) (Variables|Default|GetWhirlPoolCentre)))
          (bind _newtrack_0_2 (Timeline|T_Whirlpool PlayFromStart)
            (:Update
              (Transformation|SetActorLocationAndRotation (+ (Variables|Default|GetWhirlPoolCentre) (* (Math|Vector|GetForwardVector (Math|Rotator|MakeRotator (.roll (Variables|Default|GetWhirlPoolStartRot)) (.pitch (Variables|Default|GetWhirlPoolStartRot)) (+ (.yaw (Variables|Default|GetWhirlPoolStartRot)) (* _newtrack_0_2 -3.6e+02) 9e+01))) (Math|Vector|VectorLength (- (Variables|/Script/Engine.SphereComponent|GetSphereRadius (Variables|Default|GetWhirlpoolRange)) 1e+04)))) (Math|Rotator|MakeRotator 0.0 0.0 (* _newtrack_0_2 -3.6e+02))))
            (:Finished
              (Variables|Default|SetChompAimLocation (Transformation|GetActorLocation (Variables|Default|GetPlayer)))
              (CallFunction|Chomp))))))))

(event Custom|Reset
  (Variables|Default|SetResetStartTransform (Transformation|GetActorTransform))
  (bind _newtrack_0 (Timeline|T_Reset Play)
    (:Update
      (Transformation|SetActorTransform (Math|Transform|Lerp(Transform) (Variables|Default|GetResetStartTransform) (Math|Transform|MakeTransform (Variables|Default|GetStartLoc) "0, 0, 0" "1.000000,1.000000,1.000000") _newtrack_0)))))

(event Custom|WhirlpoolFinished
  ;[1 1 1] Attack Selector
  (if (Variables|/Game/Blueprints/Water/BP_Whirlpool.BP_Whirlpool_C|GetHasShip (Variables|Default|GetBP_Whirlpool))
    (CallFunction|Chomp)
    (Variables|Default|SetLastAttack "NewEnumerator1")
    (else
      (CallFunction|Leap)
      (Variables|Default|SetLastAttack "NewEnumerator0"))))

(event Custom|RamActive
  ;[1 1 1] Ram
  (bind _finished_ (CallFunction|LerpAlongSpline (Variables|Default|GetRamSpline) self (Variables|Default|GetSpeed)))
  (if _finished_
    (Utilities|Time|ClearandInvalidateTimerbyHandle (Variables|Default|GetCurrent%20Attack%20Handle))
    (CallFunction|ReturntoCircle)))

(event Custom|Leap)

(event EventBeginPlay
  (bind _returnvalue (Actor|GetActorOfClass "/Game/Blueprints/t014172k/Pawn_ShipNew.Pawn_ShipNew_C"))
  (Variables|Default|SetPlayer _returnvalue))

(fn ConstructionScript)

(fn TransformActorAlongSpline
  (params (Distance :type Float%20%28double-precision%29) (Spline :type Spline%20Component%20Object%20Reference) (Actor :type Actor%20Object%20Reference))
  (bind _returnvalue (Spline|GetLocationatDistanceAlongSpline Spline Distance "World"))
  (Transformation|SetActorTransform Actor (Math|Transform|MakeTransform _returnvalue (Math|Rotator|FindLookatRotation _returnvalue (Spline|GetTangentatDistanceAlongSpline Spline Distance "World")) "1.000000,1.000000,1.000000")))

(fn SetSplinePointStartandEnd
  (params (Spline :type Spline%20Component%20Object%20Reference) (Start :type Vector) (End :type Vector))
  (Transformation|SetWorldTransform Spline (Math|Transform|MakeTransform Start (Math|Rotator|FindLookatRotation Start End) (Math|Conversions|ToVector(Float) (* 1.0 (Math|Vector|VectorLength (- Start End)) (Math|Vector|VectorLength (- (Spline|GetLocationatSplinePoint Spline 0 "Local") (Spline|GetLocationatSplinePoint Spline (Class|SplineComponent|GetNumberOfSplineSegments Spline) "Local")))))) false false))

(fn GetPositionUnderShip
  (bind _returnvalue (Transformation|GetActorLocation))
  (bind _player (Variables|Default|GetPlayer))
  (bind _returnvalue_2 (Transformation|GetActorLocation _player))
  (return _returnvalue (Math|Vector|MakeVector (.x _returnvalue_2) (.y _returnvalue_2) (.Z (Class|KismetMathLibrary|BreakVector3f _returnvalue)))))

(fn LerpAlongSpline
  (params (Spline :type Spline%20Component%20Object%20Reference) (Actor :type Actor%20Object%20Reference) (Speed :type Float%20%28double-precision%29))
  (bind _returnvalue (Spline|GetSplineLength Spline))
  (bind _output_get (Variables|Default|SetDistanceAlongAttack (+ (Variables|Default|GetDistanceAlongAttack) Speed)))
  (CallFunction|TransformActorAlongSpline (Math|Float|Lerp 0.0 _returnvalue (Math|Float|Clamp(Float) _output_get 0.0 _returnvalue)) Spline Actor)
  (return (== (Math|Float|Clamp(Float) _output_get 0.0 _returnvalue) _returnvalue)))