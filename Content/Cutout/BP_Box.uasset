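; Box actor that publishes its Cube component's transform to the MPC_Box_Data Material Parameter Collection, apparently to define an oriented cutout volume for materials.
; It writes world location, scale as bounds, and forward, right and up vectors as the box axes.
; The same writes run in the Construction Script and on BeginPlay, with no per-frame update.
; All instances share one collection, so the last write wins.
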(event EventBeginPlay
  (bind _cube (Variables|Default|GetCube))
  (Rendering|Material|SetVectorParameterValue "/Game/Cutout/MPC_Box_Data.MPC_Box_Data" "Location" (Math|Conversions|ToLinearColor(Vector) (Transformation|GetWorldLocation _cube)) :!class /Script/Engine.KismetMaterialLibrary)
  (Rendering|Material|SetVectorParameterValue "/Game/Cutout/MPC_Box_Data.MPC_Box_Data" "Bounds" (Math|Conversions|ToLinearColor(Vector) (Transformation|GetWorldScale _cube)) :!class /Script/Engine.KismetMaterialLibrary)
  (Rendering|Material|SetVectorParameterValue "/Game/Cutout/MPC_Box_Data.MPC_Box_Data" "x" (Math|Conversions|ToLinearColor(Vector) (Math|Vector|GetForwardVector _cube)) :!class /Script/Engine.KismetMaterialLibrary)
  (Rendering|Material|SetVectorParameterValue "/Game/Cutout/MPC_Box_Data.MPC_Box_Data" "y" (Math|Conversions|ToLinearColor(Vector) (Math|Vector|GetRightVector _cube)) :!class /Script/Engine.KismetMaterialLibrary)
  (Rendering|Material|SetVectorParameterValue "/Game/Cutout/MPC_Box_Data.MPC_Box_Data" "z" (Math|Conversions|ToLinearColor(Vector) (Math|Vector|GetUpVector _cube)) :!class /Script/Engine.KismetMaterialLibrary))

(event Collision|EventActorBeginOverlap
  (params (OtherActor :type Actor%20Object%20Reference)))

(fn ConstructionScript
  (bind _cube (Variables|Default|GetCube))
  (Rendering|Material|SetVectorParameterValue "/Game/Cutout/MPC_Box_Data.MPC_Box_Data" "Location" (Math|Conversions|ToLinearColor(Vector) (Transformation|GetWorldLocation _cube)) :!class /Script/Engine.KismetMaterialLibrary)
  (Rendering|Material|SetVectorParameterValue "/Game/Cutout/MPC_Box_Data.MPC_Box_Data" "Bounds" (Math|Conversions|ToLinearColor(Vector) (Transformation|GetWorldScale _cube)) :!class /Script/Engine.KismetMaterialLibrary)
  (Rendering|Material|SetVectorParameterValue "/Game/Cutout/MPC_Box_Data.MPC_Box_Data" "x" (Math|Conversions|ToLinearColor(Vector) (Math|Vector|GetForwardVector _cube)) :!class /Script/Engine.KismetMaterialLibrary)
  (Rendering|Material|SetVectorParameterValue "/Game/Cutout/MPC_Box_Data.MPC_Box_Data" "y" (Math|Conversions|ToLinearColor(Vector) (Math|Vector|GetRightVector _cube)) :!class /Script/Engine.KismetMaterialLibrary)
  (Rendering|Material|SetVectorParameterValue "/Game/Cutout/MPC_Box_Data.MPC_Box_Data" "z" (Math|Conversions|ToLinearColor(Vector) (Math|Vector|GetUpVector _cube)) :!class /Script/Engine.KismetMaterialLibrary))